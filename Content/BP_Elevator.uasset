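; Elevator actor that stages the game's intro ride with camera fade, audio and a level sequence, or simply unlocks if the intro is off.
; Panning materials fake motion until the sequence ends or X skips it.
; Arrival then stops the panning, shows timed tutorial widgets and lerps the offset floor to its original position via a height-scaled timeline.
; When the timeline finishes, it unlocks the child-actor door and enables the button.
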(event EventTick
  (params (DeltaSeconds :type Float%20%28single-precision%29))
  (if (Variables|Default|GetIsArriving)
    (Utilities|FlowControl|DoOnce false
      (:Completed
        (Rendering|Material|SetScalarParameterValueonMaterials (Variables|Default|GetPanner) "SpeedY" 0.0)
        (Components|Timeline|SetPlayRate (Variables|Default|GetArriveTimeline) (/ 1.0 (Variables|Default|GetRiseHeightMeters)))
        (bind _arrivefloattrack (Timeline|ArriveTimeline Play)
          (:Update
            (Transformation|SetWorldLocation (Variables|Default|GetElevatorFloor) (Math|Vector|Lerp(Vector) (Variables|Default|GetElevatorStart) (Variables|Default|GetElevatorStop) _arrivefloattrack) false false))
          (:Finished
            (CallFunction|UnlockDoor)
            (Class|FMODBlueprintStatics|EventInstanceStop (stale EventBeginPlay _returnvalue_2) false)))))))

(event EventBeginPlay
  (bind _fadeduration (Variables|Default|GetFadeDuration))
  (bind _elevatorfloor (Variables|Default|GetElevatorFloor))
  (bind _sequences (Variables|Default|GetSequences))
  (bind _sequenceindex (Variables|Default|GetSequenceIndex))
  (bind _returnvalue (Transformation|GetWorldLocation _elevatorfloor))
  (bind _output (Utilities|Array|Get(acopy) _sequences _sequenceindex))
  (bind _sequenceplayer (Variables|/Script/LevelSequence.LevelSequenceActor|GetSequencePlayer _output))
  (if (Variables|Default|GetDoIntro)
    (if (Variables|Default|GetPlayMusic)
      (bind _returnvalue_2 (Class|FMODBlueprintStatics|PlayEvent2D "/Game/FMOD/Events/Music/Environment/Hiss.Hiss")))
    (Variables|Default|SetElevatorStop _returnvalue)
    (Transformation|AddWorldOffset _elevatorfloor (Math|Vector|MakeVector 0.0 0.0 (* (Variables|Default|GetRiseHeightMeters) 1e+02)) false false)
    (Variables|Default|SetElevatorStart _returnvalue)
    (bind _returnvalue_3 (Class|FMODBlueprintStatics|PlayEventAttached "/Game/FMOD/Events/SFX/Interaction_SFX/Elevator/Elevator_ride_interior.Elevator_ride_interior" (Variables|/Script/Engine.Character|GetCapsuleComponent (Game|GetPlayerCharacter 0)) "None" "0, 0, 0" "KeepRelativeOffset"))
    (CameraFades|StartCameraFade :self (Game|GetPlayerCameraManager 0) :FromAlpha 1.4 :Duration _fadeduration)
    (Utilities|FlowControl|Delay _fadeduration)
    (Input|EnableInput (Game|GetPlayerController 0))
    (Sequencer|Player|Play _sequenceplayer :!class /Script/MovieScene.MovieSceneSequencePlayer)
    (Utilities|FlowControl|Delay (Class|TimeManagementBlueprintLibrary|ToSeconds(QualifiedFrameTime) (Media|MediaPlayer|GetDuration _sequenceplayer)))
    (Utilities|FlowControl|DoOnce false
      (:Completed
        (Class|FMODAudioComponent|SetParameter _returnvalue_3 "Is Stopping" 1.0)
        (Variables|Default|SetIsArriving true)
        (Variables|Default|SetDoIntro false)
        (Utilities|FlowControl|Delay 5.0)
        (bind _returnvalue_4 (UserInterface|CreateWidget "/Game/Blueprints/Source/LevelBlueprints/Widgets/Tips/MoveTipsWidgetAnimated.MoveTipsWidgetAnimated_C" (Game|GetPlayerController 0)))
        (UserInterface|Viewport|AddtoViewport _returnvalue_4 0)
        (Utilities|FlowControl|Delay 5.0)
        (bind _returnvalue_5 (UserInterface|CreateWidget "/Game/Blueprints/Source/LevelBlueprints/Widgets/Tips/InteractTipsWidgetAnimated.InteractTipsWidgetAnimated_C" (Game|GetPlayerController 0)))
        (UserInterface|Viewport|AddtoViewport _returnvalue_5 0)
        (Utilities|FlowControl|Delay 5.0)
        (bind _returnvalue_6 (UserInterface|CreateWidget "/Game/Blueprints/Source/LevelBlueprints/Widgets/Tips/ZoomTipsWidgetAnimated.ZoomTipsWidgetAnimated_C" (Game|GetPlayerController 0)))
        (UserInterface|Viewport|AddtoViewport _returnvalue_6 0)))
    (else
      (CallFunction|UnlockDoor))))

(event Input|KeyboardEvents|X
  (params (Key :type Key%20Structure :default "None"))
  (bind _sequences (Variables|Default|GetSequences))
  (bind _sequenceindex (Variables|Default|GetSequenceIndex))
  (bind _output (Utilities|Array|Get(acopy) _sequences _sequenceindex))
  (bind _sequenceplayer (Variables|/Script/LevelSequence.LevelSequenceActor|GetSequencePlayer _output))
  (:Pressed
    (if (Variables|Default|GetDoIntro)
      (Class|MovieSceneSequencePlayer|JumptoFrame _sequenceplayer (Utilities|Struct|MakeFrameTime (Utilities|Struct|MakeFrameNumber (- (Class|MovieSceneSequencePlayer|GetFrameDuration _sequenceplayer) 1)) 0.0))
      (Utilities|FlowControl|DoOnce false
        (:Completed
          (Class|FMODAudioComponent|SetParameter (stale EventBeginPlay _returnvalue_3) "Is Stopping" 1.0)
          (Variables|Default|SetIsArriving true)
          (Variables|Default|SetDoIntro false)
          (Utilities|FlowControl|Delay 5.0)
          (bind _returnvalue (UserInterface|CreateWidget "/Game/Blueprints/Source/LevelBlueprints/Widgets/Tips/MoveTipsWidgetAnimated.MoveTipsWidgetAnimated_C" (Game|GetPlayerController 0)))
          (UserInterface|Viewport|AddtoViewport _returnvalue 0)
          (Utilities|FlowControl|Delay 5.0)
          (bind _returnvalue_2 (UserInterface|CreateWidget "/Game/Blueprints/Source/LevelBlueprints/Widgets/Tips/InteractTipsWidgetAnimated.InteractTipsWidgetAnimated_C" (Game|GetPlayerController 0)))
          (UserInterface|Viewport|AddtoViewport _returnvalue_2 0)
          (Utilities|FlowControl|Delay 5.0)
          (bind _returnvalue_3 (UserInterface|CreateWidget "/Game/Blueprints/Source/LevelBlueprints/Widgets/Tips/ZoomTipsWidgetAnimated.ZoomTipsWidgetAnimated_C" (Game|GetPlayerController 0)))
          (UserInterface|Viewport|AddtoViewport _returnvalue_3 0))))))

(fn ConstructionScript)

(fn UnlockDoor
  (Utilities|FlowControl|Sequence
    (:then_0
      (bind _asbp_elevator_door (Utilities|Casting|CastToBP_ElevatorDoor (Variables|/Script/Engine.ChildActorComponent|GetChildActor (Variables|Default|GetBP_ElevatorDoor))))
      (Variables|/Game/Blueprints/Source/Interaction/BP_InteractableDoor.BP_InteractableDoor_C|SetLocked _asbp_elevator_door false)
      (Rendering|SetVisibility (Variables|Default|GetPanner) false false))
    (:then_1
      (bind _asbp_elevator_button (Utilities|Casting|CastToBP_ElevatorButton (Variables|/Script/Engine.ChildActorComponent|GetChildActor (Variables|Default|GetBP_ElevatorButton))))
      (Variables|/Game/Blueprints/Source/Interaction/BP_ElevatorButton.BP_ElevatorButton_C|SetEnabled _asbp_elevator_button true))))