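; BP_MachineComponent is an actor that represents a machine component and visualizes its link to another component referenced by Comp.
; An EditorTick event calls DrawLine, which, when Comp is valid, draws a thick red debug arrow between the two components' root locations, each offset by its ReferencePoint.
; The construction script adds a child actor component; no gameplay logic runs on BeginPlay or Tick.
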(event EventBeginPlay)

(event Collision|EventActorBeginOverlap
  (params (OtherActor :type Actor%20Object%20Reference)))

(event EventTick
  (params (DeltaSeconds :type Float%20%28single-precision%29)))

(event EventEditorTick
  (CallFunction|DrawLine))

(fn ConstructionScript
  (AddComponent|AddChildActorComponent false))

(fn DrawLine
  (bind _comp (Variables|Default|GetComp))
  (if (Utilities|IsValid (Variables|Default|GetComp))
    (Rendering|Debug|DrawDebugArrow (+ (Transformation|GetWorldLocation (Variables|Default|GetDefaultSceneRoot)) (Variables|Default|GetReferencePoint)) (+ (Transformation|GetWorldLocation (Variables|BP_MachineComponent_C|GetDefaultSceneRoot _comp)) (Variables|BP_MachineComponent_C|GetReferencePoint _comp)) 1e+03 "(R=1.000000,G=0.009182,B=0.000000,A=1.000000)" 0.0 7.0)))