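; BP_FloorGas is an effect actor that builds a layered floor gas volume out of stacked mesh slices.
; On BeginPlay it records the Plane's world Z as the base, then adds static mesh components at even vertical steps derived from VolumeHeight and SliceNumber.
; The Plane and each slice get a dynamic material instance fed that base Z and VolumeHeight, so the material knows the volume's vertical range.
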(event EventBeginPlay
  (bind _plane (Variables|Default|GetPlane))
  (bind _returnvalue (Transformation|GetWorldLocation _plane))
  (bind _returnvalue_2 (Rendering|Material|CreateDynamicMaterialInstance _plane 0 (Rendering|Material|GetMaterial (Variables|Default|GetPlane) 0) "None" :!class /Script/Engine.PrimitiveComponent))
  (Variables|Default|SetSeedHeight (.z _returnvalue))
  (Rendering|Material|SetScalarParameterValue _returnvalue_2 "MinFromBP" (.z _returnvalue) :!class /Script/Engine.MaterialInstanceDynamic)
  (Rendering|Material|SetScalarParameterValue _returnvalue_2 "MaxFromBP" (Variables|Default|GetVolumeHeight) :!class /Script/Engine.MaterialInstanceDynamic)
  (for _index (range 0 (Variables|Default|GetSliceNumber))
    (bind _returnvalue_3 (AddComponent|AddStaticMeshComponent false (Math|Transform|MakeTransform (Math|Vector|MakeVector 0.0 0.0 (Variables|Default|GetPreviousLayer)) "0, 0, 0" "1,1,1")))
    (Variables|Default|SetPreviousLayer (+ (Variables|Default|GetPreviousLayer) (/ (Variables|Default|GetVolumeHeight) (Math|Conversions|ToFloat(Integer) (Variables|Default|GetSliceNumber)))))
    (bind _returnvalue_4 (Rendering|Material|CreateDynamicMaterialInstance _returnvalue_3 0 (Rendering|Material|GetMaterial _returnvalue_3 0) "None" :!class /Script/Engine.PrimitiveComponent))
    (Rendering|Material|SetScalarParameterValue _returnvalue_4 "MinFromBP" (Variables|Default|GetSeedHeight) :!class /Script/Engine.MaterialInstanceDynamic)
    (Rendering|Material|SetScalarParameterValue _returnvalue_4 "MaxFromBP" (Variables|Default|GetVolumeHeight) :!class /Script/Engine.MaterialInstanceDynamic)))

(fn ConstructionScript)