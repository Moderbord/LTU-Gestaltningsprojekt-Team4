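; BP_Camera is a surveillance-style camera actor that feeds a live image to a coupled monitor in the world.
; On BeginPlay it creates a square canvas render target at the configured resolution, assigns it to its scene capture and hands it to the monitor as a screen texture.
; When limited framerate is enabled, a looping timer triggers manual captures at that rate, replacing per-frame and on-movement capture.
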(event Custom|setFramerate
  (bind _cameracapture (Variables|Default|GetCameraCapture))
  ;[1 1 1] Camera framerate
  (if (Variables|Default|GetLimitedFramerate)
    (Utilities|Time|SetTimerbyEvent (delegate Custom|CameraUpdate) (/ 1.0 (Variables|Default|GetFramerate)) true)
    (Variables|/Script/Engine.SceneCaptureComponent|SetbCaptureEveryFrame _cameracapture false)
    (Variables|/Script/Engine.SceneCaptureComponent|SetbCaptureOnMovement _cameracapture false)))

(event Custom|CameraUpdate
  ;[1 1 1] Camera framerate
  (Rendering|SceneCapture|CaptureScene (Variables|Default|GetCameraCapture) :!class /Script/Engine.SceneCaptureComponent2D))

(event EventBeginPlay
  (bind _cameraresolution (Variables|Default|GetCameraResolution))
  ;[1 1 1] Create and send image feed
  (bind _returnvalue (CanvasRenderTarget2D|CreateCanvasRenderTarget2D "/Script/Engine.CanvasRenderTarget2D" _cameraresolution _cameraresolution))
  (bind _output_get (Variables|/Script/Engine.SceneCaptureComponent2D|SetTextureTarget (Variables|Default|GetCameraCapture) _returnvalue))
  (Default|AssignScreenTexture (Variables|Default|GetCoupledMonitor) _output_get)
  (CallFunction|SetFramerate))

(fn ConstructionScript)