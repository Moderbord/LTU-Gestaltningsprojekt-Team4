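; Base spline actor that tiles a configurable mesh along its spline as deformed spline mesh segments, built in the construction script.
; Count derives section length from the actor's X scale times 100 and fits whole sections into the spline length.
; Section samples local positions and tangents at each segment's ends, clamping tangents to section length.
; SetVariables applies mesh, material, forward axis and optional collision to each added component.
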(event EventBeginPlay)

(event Collision|EventActorBeginOverlap
  (params (OtherActor :type Actor%20Object%20Reference)))

(event EventTick
  (params (DeltaSeconds :type Float%20%28single-precision%29)))

(fn ConstructionScript
  (bind _returnvalue (CallFunction|Count))
  (for _index (range 0 _returnvalue)
    (bind _returnvalue_2 (AddComponent|AddSplineMeshComponent false))
    (bind _outputpin (CallFunction|SetVariables _returnvalue_2))
    (bind (_startposition _starttangent _endposition _endtangent) (CallFunction|Section _index))
    (SplineMesh|SetStartandEnd _outputpin _startposition _starttangent _endposition _endtangent true :!class /Script/Engine.SplineMeshComponent)))

(fn SetVariables
  (params (Component :type Spline%20Mesh%20Component%20Object%20Reference))
  (Components|StaticMesh|SetStaticMesh Component (Variables|Surface|GetSurfaceMesh))
  (Rendering|Material|SetMaterial Component 0 (Variables|Surface|GetSurfaceMaterial))
  (SplineMesh|SetForwardAxis Component (Variables|Default|GetForwardAxis) true)
  (Collision|SetCollisionEnabled Component (select (Variables|Collision|GetCollision) "QueryAndPhysics" "NoCollision"))
  (return Component))

(fn Section
  (params (Index :type Integer))
  (bind _returnvalue (+ Index 1))
  (bind _spline (Variables|Default|GetSpline))
  (bind _spline_2 (Variables|Default|GetSpline))
  (bind _sectionlenght (Variables|Default|GetSectionLenght))
  (bind _sectionlenght_2 (Variables|Default|GetSectionLenght))
  (bind _returnvalue_2 (* _returnvalue _sectionlenght))
  (bind _returnvalue_3 (* Index _sectionlenght))
  (return (Spline|GetLocationatDistanceAlongSpline _spline_2 _returnvalue_3 "Local") (Math|Vector|ClampVectorSize (Spline|GetTangentatDistanceAlongSpline _spline_2 _returnvalue_3 "Local") 0.0 _sectionlenght_2) (Spline|GetLocationatDistanceAlongSpline _spline _returnvalue_2 "Local") (Math|Vector|ClampVectorSize (Spline|GetTangentatDistanceAlongSpline _spline _returnvalue_2 "Local") 0.0 _sectionlenght_2)))

(fn Count
  (Variables|Default|SetSectionLenght (* (.x (Transformation|GetActorScale3D)) 1e+02))
  (return (- (Math|Float|Truncate (/ (Spline|GetSplineLength (Variables|Default|GetSpline)) (Variables|Default|GetSectionLenght))) 1)))