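; Interactable wall button that toggles between pressed and released and outlines itself while hovered.
; Interaction flips the Pressed state, ignored while the push timeline is running, then plays or reverses that timeline to slide the button mesh.
; When the timeline finishes, it plays an attached on or off sound event and broadcasts the new state through OnButtonChanged.
; BeginPlay runs the same path to apply the initial state.
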(event EventOnHover
  (params (CursorOver :type Boolean))
  (CallFunction|SetComponentOutline (Variables|Default|GetButton) CursorOver "NewEnumerator0"))

(event EventOnBeginInteract
  (params (Caller :type Actor%20Object%20Reference))
  (bind _button (Variables|Default|GetButton))
  (if (not (Audio|Components|Audio|IsPlaying (Variables|Default|GetPushTimeLine)))
    (bind _output_get (Variables|Default|SetPressed (not (Variables|Default|GetPressed))))
    (if _output_get
      (bind _floattrack (Timeline|PushTimeLine Play)
        (:Update
          (Transformation|SetRelativeLocation _button (Math|Vector|Lerp(Vector) "0, 0,3.000000" "0, 0, 0" _floattrack) false false))
        (:Finished
          (Class|FMODBlueprintStatics|PlayEventAttached (select _output_get (Variables|Default|GetButtonOn) (Variables|Default|GetButtonOff)) _button "None" "0, 0, 0" "KeepRelativeOffset")
          (Default|CallOnButtonChanged _output_get)))
      (else
        (Timeline|PushTimeLine Reverse)))))

(event EventBeginPlay
  (bind _button (Variables|Default|GetButton))
  (if (stale EventOnBeginInteract _output_get)
    (bind _floattrack (Timeline|PushTimeLine Play)
      (:Update
        (Transformation|SetRelativeLocation _button (Math|Vector|Lerp(Vector) "0, 0,3.000000" "0, 0, 0" _floattrack) false false))
      (:Finished
        (Class|FMODBlueprintStatics|PlayEventAttached (select (stale EventOnBeginInteract _output_get) (Variables|Default|GetButtonOn) (Variables|Default|GetButtonOff)) _button "None" "0, 0, 0" "KeepRelativeOffset")
        (Default|CallOnButtonChanged (stale EventOnBeginInteract _output_get))))
    (else
      (Timeline|PushTimeLine Reverse))))

(fn ConstructionScript)