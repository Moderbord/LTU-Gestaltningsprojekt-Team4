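; BP_Fuse is an interactable fuse for the fusebox whose hover outline color reflects whether the fuse is working.
; Beginning interaction plays an attached grab sound and turns on physics simulation.
; Component hits play a drop sound at the impact point, with volume mapped from linear velocity that a delayed Tick samples periodically.
; A DoOnce with a short random-delay reset throttles repeated impact sounds.
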(event OnComponentHit(Fuse)
  (params (HitComponent :type Primitive%20Component%20Object%20Reference) (OtherActor :type Actor%20Object%20Reference) (OtherComp :type Primitive%20Component%20Object%20Reference) (NormalImpulse :type Vector :default "0, 0, 0") (Hit :type Hit%20Result%20Structure%20%28by%20ref%29))
  ;[1 1 1] Sound
  (Utilities|FlowControl|Sequence
    (:then_0
      (Utilities|FlowControl|DoOnce false :!label _label
        (:Completed
          (bind _returnvalue (Class|FMODBlueprintStatics|PlayEventatLocation "/Game/FMOD/Events/SFX/Interaction_SFX/Fuse_Box/Fuse_Box_Drop.Fuse_Box_Drop" (Math|Conversions|ToTransform(Vector) (.Location (Collision|BreakHitResult Hit)))))
          (Class|FMODBlueprintStatics|EventInstanceSetVolume _returnvalue (Math|Float|MapRangeClamped (Math|Vector|VectorLength (stale EventTick _returnvalue)) 1.7e+02 0.0 1.0 0.0)))))
    (:then_1
      (Utilities|FlowControl|Delay (Math|Random|RandomFloatinRange 0.2 0.4))
      (goto _label Reset))))

(event EventOnHover
  (params (CursorOver :type Boolean))
  (CallFunction|SetOutline self CursorOver (Utilities|Enum|ByteToEnumEOutlineColors (Math|Conversions|ToByte(Integer) (not (Variables|Default|GetFuseWorking))))))

(event EventTick
  (params (DeltaSeconds :type Float%20%28single-precision%29))
  ;[1 1 1] Sound
  (Utilities|FlowControl|Delay 0.1)
  (bind _returnvalue (Physics|GetPhysicsLinearVelocity (Variables|Default|GetFuse) "None")))

(event EventOnBeginInteract
  (params (Caller :type Actor%20Object%20Reference))
  (Class|FMODBlueprintStatics|PlayEventAttached "/Game/FMOD/Events/Character/Grab.Grab" (Variables|Default|GetFuse) "None" "0, 0, 0" "KeepRelativeOffset")
  (CallFunction|SetSimPhysics true))

(fn ConstructionScript)

(fn SetSimPhysics
  (params (SimulatePhysics :type Boolean))
  (Physics|SetSimulatePhysics (Variables|Default|GetFuse) SimulatePhysics))