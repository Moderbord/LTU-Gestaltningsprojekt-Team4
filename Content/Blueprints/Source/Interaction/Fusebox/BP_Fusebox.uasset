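; Fusebox actor that holds a replaceable fuse and reports its powered state through OnFuseChanged and a Probe query.
; Overlapping a working fuse consumes it and spawns a locked replacement in the socket; removing the held fuse trips the box.
; A power failure breaks the fuse and adds a particle effect, which a new fuse clears.
; A dynamic material switches the indicator light between green and red.
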(event EventBeginPlay
  (bind _returnvalue (Rendering|Material|CreateDynamicMaterialInstance (Variables|Default|GetFuseBox) 0 "/Game/Materials/Source_Materials/Corridor/FuseBox.FuseBox" "None" :!class /Script/Engine.PrimitiveComponent))
  (Variables|Default|SetMaterial _returnvalue)
  (if (Variables|Default|GetFuseIn)
    (CallFunction|InsertFuse)
    (else
      (CallFunction|TripFuse))))

(event Collision|EventActorBeginOverlap
  (params (OtherActor :type Actor%20Object%20Reference))
  (if (not (Variables|Default|GetFuseIn))
    (bind _asbp_fuse (Utilities|Casting|CastToBP_Fuse OtherActor))
    (if (Variables|/Game/Blueprints/Source/Interaction/Fusebox/BP_Fuse.BP_Fuse_C|GetFuseWorking _asbp_fuse)
      (Actor|DestroyActor _asbp_fuse)
      ;[1 1 1] Sound
      (Class|FMODBlueprintStatics|PlayEventAttached "/Game/FMOD/Events/SFX/Interaction_SFX/Fuse_Box/Fuse_Box_Replace.Fuse_Box_Replace" (Variables|Default|GetFuseBox) "None" "0, 0, 0" "KeepRelativeOffset")
      (CallFunction|InsertFuse)
      (if (Utilities|IsValid (Variables|Default|GetParticleSystem))
        (Components|DestroyComponent (Variables|Default|GetParticleSystem))))))

(event EventOnPowerFailureEvent
  (Variables|Default|SetFuseIn false)
  (CallFunction|TripFuse)
  (bind _returnvalue (AddComponent|AddParticleSystemComponent false (Variables|Default|GetParticleSystemPos)))
  (Variables|Default|SetParticleSystem _returnvalue))

(event Collision|EventActorEndOverlap
  (params (OtherActor :type Actor%20Object%20Reference))
  (if (== OtherActor (Variables|Default|GetFuse))
    (Variables|Default|SetFuseIn false)
    (Variables|Default|SetFuse 0)
    ;[1 1 1] Sound
    (Class|FMODBlueprintStatics|PlayEventAttached "/Game/FMOD/Events/SFX/Interaction_SFX/Fuse_Box/Fuse_Box_Remove.Fuse_Box_Remove" (Variables|Default|GetFuseBox) "None" "0, 0, 0" "KeepRelativeOffset")
    (CallFunction|TripFuse)))

(fn ConstructionScript)

(fn GetFuse
  (bind _fuse (Variables|Default|GetFuse))
  (Utilities|IsValid _fuse
    (:Is%20Valid
      (return (Variables|/Game/Blueprints/Source/Interaction/Fusebox/BP_Fuse.BP_Fuse_C|GetFuseWorking _fuse)))
    (:Is%20Not%20Valid
      (return false))))

(fn TripFuse
  (bind _fuse (Variables|Default|GetFuse))
  (Default|CallOnFuseChanged false)
  (Rendering|Material|SetVectorParameterValue (Variables|Default|GetMaterial) "LightColor" "(R=1.000000,G=0.000000,B=0.032086,A=1.000000)" :!class /Script/Engine.MaterialInstanceDynamic)
  (Utilities|IsValid _fuse
    (:Is%20Valid
      (Variables|/Game/Blueprints/Source/Interaction/Fusebox/BP_Fuse.BP_Fuse_C|SetFuseWorking _fuse false)
      (Rendering|Material|SetMaterial (Variables|/Game/Blueprints/Source/Interaction/Fusebox/BP_Fuse.BP_Fuse_C|GetFuse _fuse) 0 "/Game/Materials/Source_Materials/Corridor/BrokenFuse.BrokenFuse"))))

(fn InsertFuse
  (Default|CallOnFuseChanged true)
  (bind _returnvalue (Game|SpawnActorfromClass "/Game/Blueprints/Source/Interaction/Fusebox/BP_Fuse.BP_Fuse_C" (Transformation|GetWorldTransform (Variables|Default|GetFuseLocation)) "AlwaysSpawn" 0 0))
  (bind _output_get (Variables|Default|SetFuse _returnvalue))
  (Default|SetSimPhysics _output_get false)
  (Variables|Default|SetFuseIn true)
  (Rendering|Material|SetVectorParameterValue (Variables|Default|GetMaterial) "LightColor" "(R=0.117745,G=0.911458,B=0.000000,A=1.000000)" :!class /Script/Engine.MaterialInstanceDynamic))

(fn Probe
  (params (Key :type Signal%20Key%20Structure))
  (bind _working (CallFunction|GetFuse))
  (return (Math|Conversions|ToFloat(Boolean) (and _working (Utilities|Enum|Equal(Enum) (.type Key) "NewEnumerator12")))))