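; Interactable radio prop that the player can switch on and off.
; Each interaction flips IsPlaying, plays a matching button on or off audio event attached to the radio mesh, and starts or stops the Radio component.
; Hover events toggle an outline on the actor while the cursor is over it.
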(event EventBeginPlay)

(event EventOnBeginInteract
  (params (Caller :type Actor%20Object%20Reference))
  (bind _sm_radio (Variables|Default|GetSM_Radio))
  (bind _radio (Variables|Default|GetRadio))
  (bind _output_get (Variables|Default|SetIsPlaying (not (Variables|Default|GetIsPlaying))))
  (if _output_get
    (Class|FMODBlueprintStatics|PlayEventAttached "/Game/FMOD/Events/SFX/Interaction_SFX/Buttons/Button5_on.Button5_on" _sm_radio "None" "0, 0, 0" "KeepRelativeOffset")
    (Class|FMODAudioComponent|Play _radio)
    (else
      (Class|FMODBlueprintStatics|PlayEventAttached "/Game/FMOD/Events/SFX/Interaction_SFX/Buttons/Button5_off.Button5_off" _sm_radio "None" "0, 0, 0" "KeepRelativeOffset")
      (Class|FMODAudioComponent|Stop _radio))))

(event EventOnHover
  (params (CursorOver :type Boolean))
  (CallFunction|SetOutline self CursorOver "NewEnumerator0"))

(fn ConstructionScript)