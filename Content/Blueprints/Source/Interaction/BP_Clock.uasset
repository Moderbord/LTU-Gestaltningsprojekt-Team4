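; BP_Clock is an animated clock that rotates its second, minute and hour hands and plays ticking audio.
; On BeginPlay, AddSeconds applies TimeOffsetInSeconds as the starting time, then each Tick feeds it DeltaSeconds.
; AddSeconds turns each hand's offset component by a fixed pitch rate per second.
; A FlipFlop alternates Tick and Tock sounds on every Tick event; an event-based looping-sound setup is left unconnected.
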(event EventTick
  (params (DeltaSeconds :type Float%20%28single-precision%29))
  (CallFunction|AddSeconds DeltaSeconds)
  (Utilities|FlowControl|FlipFlop
    (:A
      (Class|FMODAudioComponent|Play (Variables|Default|GetTick)))
    (:B
      (Class|FMODAudioComponent|Play (Variables|Default|GetTock)))))

(event EventBeginPlay
  (CallFunction|AddSeconds (Variables|Default|GetTimeOffsetInSeconds)))

(fn ConstructionScript)

(fn AddSeconds
  (params (Seconds :type Float%20%28single-precision%29))
  (Transformation|AddLocalRotation (Variables|Default|GetSecondOffset) (Math|Rotator|MakeRotator 0.0 (* Seconds -6.0) 0.0) false false)
  (Transformation|AddLocalRotation (Variables|Default|GetMinuteOffset) (Math|Rotator|MakeRotator 0.0 (* Seconds -0.1) 0.0) false false)
  (Transformation|AddLocalRotation (Variables|Default|GetHourOffset) (Math|Rotator|MakeRotator 0.0 (* Seconds -0.0017) 0.0) false false))