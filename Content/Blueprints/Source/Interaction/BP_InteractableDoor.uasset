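; BP_InteractableDoor is an interactable door actor that swings open or closed when its Interact event fires.
; A DoorAnimation timeline drives the yaw of the RotationAxis component, with a Direction flag flipping the swing's sign.
; Interact plays the timeline unless the door is fully open, in which case it reverses it.
; Actor collision is disabled during the motion and restored when the timeline finishes.
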(event EventBeginPlay)

(event Collision|EventActorBeginOverlap
  (params (OtherActor :type Actor%20Object%20Reference)))

(event EventTick
  (params (DeltaSeconds :type Float%20%28single-precision%29)))

(event EventInteract
  (params (Caller :type Actor%20Object%20Reference))
  (Collision|SetActorEnableCollision false)
  (if (< (stale _dooropen) 1.0)
    (bind _dooropen (Timeline|DoorAnimation Play)
      (:Update
        (Transformation|SetRelativeRotation (Variables|Default|GetRotationAxis) (Math|Rotator|MakeRotator 0.0 9e+01 (* _dooropen (Math|Float|SelectFloat 1.0 -1.0 (Variables|Default|GetDirection)))) false false))
      (:Finished
        (Collision|SetActorEnableCollision true)))
    (else
      (Timeline|DoorAnimation Reverse))))

(fn ConstructionScript)