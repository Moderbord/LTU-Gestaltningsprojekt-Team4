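; BP_ElevatorButton is an interactable elevator button that ends the game by loading the EndCredits level, guarded by a two-press confirmation.
; Hover toggles an outline whose color reflects whether the button is enabled.
; When enabled, a first press arms AllowLeave and shows the ElevatorCheckAnimated widget for SafetyDelay, then removes it and disarms.
; A second press within that window opens the credits.
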(event EventOnHover
  (params (CursorOver :type Boolean))
  (CallFunction|SetOutline self CursorOver (Utilities|Enum|ByteToEnumEOutlineColors (Math|Conversions|ToByte(Integer) (not (Variables|Default|GetEnabled))))))

(event EventOnBeginInteract
  (params (Caller :type Actor%20Object%20Reference))
  (if (Variables|Default|GetEnabled)
    (if (Variables|Default|GetAllowLeave)
      (Game|OpenLevel(byName) "EndCredits")
      (else
        (Variables|Default|SetAllowLeave true)
        (bind _returnvalue (UserInterface|CreateWidget "/Game/Blueprints/Source/LevelBlueprints/Widgets/Tips/ElevatorCheckAnimated.ElevatorCheckAnimated_C" (Game|GetPlayerController 0)))
        (UserInterface|Viewport|AddtoViewport _returnvalue 0)
        (Utilities|FlowControl|Delay (Variables|Default|GetSafetyDelay))
        (Widget|RemovefromParent _returnvalue)
        (Variables|Default|SetAllowLeave false)))))

(fn ConstructionScript)