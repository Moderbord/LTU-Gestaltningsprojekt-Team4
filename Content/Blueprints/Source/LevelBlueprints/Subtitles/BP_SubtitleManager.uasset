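; BP_SubtitleManager is an actor that shows narration subtitles on screen, one line at a time.
; On BeginPlay it creates a subtitles widget, adds it to the viewport and clears it.
; ShowNextLine, also exposed through ShowNextLineFunc, reads a row from the supplied data table by index, displays its text and advances the counter.
; A first-line flag resets the counter, and ClearSubtitles blanks the display.
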(event Custom|ClearSubtitles
  (Default|DisplayLine (Variables|Default|GetSubtitlesWidgetRef)))

(event Custom|ShowNextLine
  (params (FirstLine :type Boolean) (NarrationList :type Data%20Table%20Object%20Reference))
  (Variables|Default|SetCurrentNarrationList NarrationList)
  (if FirstLine
    (Variables|Default|SetCurrentRow 0)
    (bind _outrownames (DataTable|GetDataTableRowNames (Variables|Default|GetCurrentNarrationList)))
    (bind _returnvalue (Utilities|GetDataTableRow (Variables|Default|GetCurrentNarrationList) (Utilities|Array|Get(acopy) _outrownames (Variables|Default|GetCurrentRow)))
      (:then
        (Default|DisplayLine (Variables|Default|GetSubtitlesWidgetRef) (.LineToShow (Utilities|Struct|BreakSubtitleStruct _returnvalue)))
        (Variables|Default|SetCurrentRow (+ (Variables|Default|GetCurrentRow) 1))))
    (else
      (bind _outrownames_2 (DataTable|GetDataTableRowNames (Variables|Default|GetCurrentNarrationList)))
      (bind _returnvalue_2 (Utilities|GetDataTableRow (Variables|Default|GetCurrentNarrationList) (Utilities|Array|Get(acopy) _outrownames_2 (Variables|Default|GetCurrentRow)))
        (:then
          (Default|DisplayLine (Variables|Default|GetSubtitlesWidgetRef) (.LineToShow (Utilities|Struct|BreakSubtitleStruct _returnvalue_2)))
          (Variables|Default|SetCurrentRow (+ (Variables|Default|GetCurrentRow) 1)))))))

(event EventBeginPlay
  (bind _returnvalue (UserInterface|CreateWidget "/Game/Blueprints/Source/LevelBlueprints/Subtitles/SubtitlesWidget.SubtitlesWidget_C"))
  (bind _output_get (Variables|Default|SetSubtitlesWidgetRef _returnvalue))
  (UserInterface|Viewport|AddtoViewport _output_get 0)
  (CallFunction|ClearSubtitles))

(fn ConstructionScript)

(fn ShowNextLineFunc
  (params (FirstLine :type Boolean) (NarrationList :type Data%20Table%20Object%20Reference))
  (CallFunction|ShowNextLine FirstLine NarrationList))