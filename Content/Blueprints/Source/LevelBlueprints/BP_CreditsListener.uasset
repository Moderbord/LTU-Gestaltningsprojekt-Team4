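; BP_CreditsListener is a level actor that unlocks leaving by elevator when its Listener component raises an alert.
; On BeginPlay it binds to the Listener's state change and caches the BP_ElevatorButton and BP_SoundController actors by class lookup.
; A true alert state overrides the sound controller's event with SuccessEvent and sets AllowLeave on the elevator button.
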(event Custom|OnStateChanged
  (params (AlertState :type Boolean) (SignalValue :type Float%20%28single-precision%29))
  (if AlertState
    (Default|OverrideEvent (Variables|Default|GetSoundController) (Variables|Default|GetSuccessEvent))
    (Variables|/Game/Blueprints/Source/Interaction/BP_ElevatorButton.BP_ElevatorButton_C|SetAllowLeave (Variables|Default|GetElevatorButton) true)))

(event EventBeginPlay
  (EventDispatchers|BindEventtoOnStateChange (Variables|Default|GetListener) (delegate Custom|OnStateChanged))
  (Utilities|FlowControl|Sequence
    (:then_0
      (bind _returnvalue (Actor|GetActorOfClass "/Game/Blueprints/Source/Interaction/BP_ElevatorButton.BP_ElevatorButton_C"))
      (Variables|Default|SetElevatorButton _returnvalue))
    (:then_1
      (bind _returnvalue_2 (Actor|GetActorOfClass "/Game/Blueprints/Source/EventController/BP_SoundController.BP_SoundController_C"))
      (Variables|Default|SetSoundController _returnvalue_2))))

(fn ConstructionScript)