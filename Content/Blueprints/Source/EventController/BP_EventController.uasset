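; Event controller that turns machine alerts and accumulated chaos into game events for BPI_EventListener actors.
; Alert changes update per-signal counters, which start or cancel delayed timers against configured thresholds.
; LaunchEvent maps the signal to an event like power failure, broadcasts it and records listeners for CompleteEvent to notify.
; Per-panel chaos sums into interval-based stages, broadcast only while no event is active; widgets display both tallies.
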(event Custom|CustomEvent
  (params (Signal :type Signal%20Key%20Structure) (AlertState :type Boolean))
  (Events|OnAlertStateChange Signal AlertState))

(event EventBeginPlay
  (EventDispatchers|BindEventtoOnCPAlertStateChange (delegate Custom|CustomEvent)))

(event Collision|EventActorBeginOverlap
  (params (OtherActor :type Actor%20Object%20Reference)))

(event EventTick
  (params (DeltaSeconds :type Float%20%28single-precision%29)))

(event EventLaunchEvent
  (params (signal :type Integer))
  (bind _returnvalue (Math|Conversions|ToByte(Integer) signal))
  (bind _returnvalue_2 (Utilities|Enum|ByteToEnumEPassiveSignals _returnvalue))
  (Development|PrintString (Utilities|String|Append (Utilities|String|EnumtoString _returnvalue_2) " event triggered!") true true "(R=1.000000,G=0.000000,B=0.051918,A=1.000000)" 3.0)
  (Events|DispatchEvent _returnvalue_2)
  (Timers|ClearTimers))

(fn ConstructionScript)

(fn AddtoCurrentEvent
  (params (Actor :type Actor%20Object%20Reference) (Force :type Boolean))
  (bind _asbp_mcbase (Utilities|Casting|CastToBP_MCBase Actor)
    (:then
      (if (or (Variables|/Game/Blueprints/Source/MachineComponents/Base/BP_MCBase.BP_MCBase_C|GetRunning _asbp_mcbase) Force)
        (Utilities|Array|Add (Variables|Events|GetEventListeners) Actor)))
    (:CastFailed
      (Utilities|Array|Add (Variables|Events|GetEventListeners) Actor) ; Actor not MC and should be added
    )))

(fn ClearAlertMap
  (Utilities|Map|Clear (Variables|Events|GetAlertCounterMap)))

(fn ClearOtherTimers
  (params (Exception :type EPassiveSignals%20Enum :default "NewEnumerator2"))
  (bind _keys (Utilities|Map|Keys (Variables|Events|GetTimerHandles)))
  (for _array_element _keys
    (if (Utilities|Enum|NotEqual(Enum) _array_element Exception)
      (Timers|ClearTimer _array_element))))

(fn ClearTimer
  (params (Signal :type EPassiveSignals%20Enum :default "NewEnumerator2"))
  (Utilities|Time|ClearandInvalidateTimerbyHandle (.Value (Utilities|Map|Find (Variables|Events|GetTimerHandles) Signal)))
  (bind _returnvalue (Utilities|Map|Remove (Variables|Events|GetTimerHandles) Signal))
  (if _returnvalue
    (Development|PrintString (Utilities|String|Append "Removed timer: " (Utilities|String|EnumtoString Signal)) true true "(R=0.000000,G=0.660000,B=1.000000,A=1.000000)" 3.0)))

(fn ClearTimers
  (bind _keys (Utilities|Map|Keys (Variables|Events|GetTimerHandles)))
  (for _array_element _keys
    (Timers|ClearTimer _array_element)))

(fn PauseTimers
  (bind _values (Utilities|Map|Values (Variables|Events|GetTimerHandles)))
  (for _array_element _values
    (Utilities|Time|PauseTimerbyHandle _array_element)))

(fn CompleteEvent
  (bind _eventlisteners (Variables|Events|GetEventListeners))
  (for _array_element _eventlisteners
    (Class|BPIEventListener|OnEventComplete(Message) _array_element))
  (Utilities|Array|Clear _eventlisteners)
  (Variables|Events|SetCurrentEvent "NewEnumerator0")
  (Variables|Events|SetEventIsActive false))

(fn CountAlerts
  (bind _keys (Utilities|Map|Keys (Variables|Events|GetAlertCounterMap)))
  (for _array_element _keys
    (bind _output_get (LocalVariables|SetCurrAlert (.type _array_element)))
    (bind _alert_threshold (Events|GetAlertThreshold _output_get))
    (if (>= (.Value (Utilities|Map|Find (Variables|Events|GetAlertCounterMap) (Utilities|Struct|MakeSignalKey _output_get "NewEnumerator5"))) _alert_threshold) ; Threshold reached
      (Timers|NewEventTimer (LocalVariables|GetCurrAlert))
      (else
        (Timers|ClearTimer (LocalVariables|GetCurrAlert))))))

(fn DispatchEvent
  (params (Signal :type EPassiveSignals%20Enum :default "NewEnumerator2"))
  (Utilities|FlowControl|Sequence
    (:then_0
      (switch Utilities|FlowControl|Switch|SwitchonEPassiveSignals Signal
        (:NewEnumerator0
          (Variables|Events|SetCurrentEvent "NewEnumerator2"))
        (:NewEnumerator9
          (Variables|Events|SetCurrentEvent "NewEnumerator4"))))
    (:then_1
      (bind _outactors (Actor|GetAllActorswithInterface "/Game/Blueprints/Source/EventController/BPI_EventListener.BPI_EventListener_C"))
      (for _array_element _outactors
        (Utilities|FlowControl|Sequence
          (:then_0
            (Events|AddtoCurrentEvent _array_element false))
          (:then_1
            (Events|EventCall (Variables|Events|GetCurrentEvent) _array_element))))
      (Variables|Events|SetEventIsActive true))))

(fn EventCall
  (params (Event :type EHavocEvents%20Enum :default "NewEnumerator0") (Actor :type Actor%20Object%20Reference))
  (switch Utilities|FlowControl|Switch|SwitchonEHavocEvents Event
    (:NewEnumerator1
      (Class|BPIEventListener|OnGenericEvent(Message) Actor))
    (:NewEnumerator2
      (Class|BPIEventListener|OnPowerFailureEvent(Message) Actor))
    (:NewEnumerator3
      (Class|BPIEventListener|OnShortCircuitEvent(Message) Actor))
    (:NewEnumerator4
      (Class|BPIEventListener|OnHighPressureEvent(Message) Actor))))

(fn GetAlertThreshold
  (params (Key :type EPassiveSignals%20Enum%20%28by%20ref%29 :default "NewEnumerator2"))
  (return (.alertthreshold (.Value (Utilities|Map|Find (Variables|Events|GetAlertConditonsMap) Key)))))

(fn GetEventDelay
  (params (Key :type EPassiveSignals%20Enum%20%28by%20ref%29 :default "NewEnumerator2"))
  (return (.eventdelay (.Value (Utilities|Map|Find (Variables|Events|GetAlertConditonsMap) Key)))))

(fn AddtoChaosMap
  (params (PanelComponent :type BP%20CP%20Element%20Base%20Object%20Reference) (Chaos :type Float%20%28single-precision%29))
  (Utilities|Map|Add (Variables|Events|GetChaosMap) PanelComponent Chaos)
  (Widgets|UpdateChaosWidget)
  (Chaos|EvalChaosStage))

(fn GetChaosStage
  (params (ChaosValue :type Float%20%28single-precision%29))
  (if (<= ChaosValue 0.0)
    (return -1)
    (else
      (bind (_array_element _array_index) (Utilities|Array|ForEachLoopwithBreak (Variables|Events|GetChaosIntervals) :!label _label)
        (:LoopBody
          (if (>= ChaosValue _array_element)
            (LocalVariables|SetIndex _array_index)
            (else
              (goto _label Break))))
        (:Completed
          (return (LocalVariables|GetIndex)))))))

(fn EvalChaosStage
  (bind _out (Chaos|GetTotalChaos))
  (if (!= _out (Variables|Events|GetLastChaos)) ; Update value if changed
    (bind _output_get (Variables|Events|SetLastChaos _out))
    (bind _newstage (Chaos|GetChaosStage _output_get))
    (if (and (!= _newstage (Variables|Events|GetChaosStage)) (not (Variables|Events|GetEventIsActive)))
      (Variables|Events|SetChaosStage _newstage)
      (bind _outactors (Actor|GetAllActorswithInterface "/Game/Blueprints/Source/EventController/BPI_EventListener.BPI_EventListener_C"))
      (for _array_element _outactors
        (Class|BPIEventListener|OnChaosStageChange(Message) _array_element (Variables|Events|GetChaosStage))))))

(fn GetTotalChaos
  (bind _values (Utilities|Map|Values (Variables|Events|GetChaosMap)))
  (for _array_element _values
    (LocalVariables|SetChaosAmount (+ (LocalVariables|GetChaosAmount) _array_element)))
  (return (LocalVariables|GetChaosAmount)))

(fn OnAlertStateChange
  (params (Signal :type Signal%20Key%20Structure) (State :type Boolean))
  (bind _alertcountermap (Variables|Events|GetAlertCounterMap))
  (bind _signalkey (Utilities|Struct|MakeSignalKey (.type Signal) "NewEnumerator5"))
  (Utilities|FlowControl|Sequence
    (:then_0
      (if State ; Add/Reduce
        (LocalVariables|SetDiff 1.0)
        (else
          (LocalVariables|SetDiff -1.0))))
    (:then_1
      (Utilities|Map|Add _alertcountermap _signalkey (+ (.Value (Utilities|Map|Find _alertcountermap _signalkey)) (LocalVariables|GetDiff)))
      (Development|PrintString (Utilities|String|Append "AlertStateChange: (" (Utilities|String|EnumtoString (.type Signal)) ", " (Utilities|String|EnumtoString (.data Signal)) ") " (Utilities|String|ToString(Float) (LocalVariables|GetDiff))) false true "(R=1.000000,G=0.000000,B=0.857058,A=1.000000)" 5.0)
      (Events|CountAlerts)
      (Widgets|UpdateAlertWidget))))

(fn UpdateAlertWidget
  (bind _asbp_mcpanel_widget (Utilities|Casting|CastToBP_MCPanelWidget (UserInterface|GetUserWidgetObject (Variables|Default|GetAlertTracker))))
  (Default|UpdatePanel _asbp_mcpanel_widget (Variables|Events|GetAlertCounterMap)))

(fn UpdateChaosWidget
  (bind _out (Chaos|GetTotalChaos))
  (Utilities|Map|Add (Variables|Events|GetChaosCounter) (Utilities|Struct|MakeSignalKey "NewEnumerator8" "NewEnumerator5") _out)
  (bind _asbp_mcpanel_widget (Utilities|Casting|CastToBP_MCPanelWidget (UserInterface|GetUserWidgetObject (Variables|Default|GetChaosMeter))))
  (Default|UpdatePanel _asbp_mcpanel_widget (Variables|Events|GetChaosCounter)))

(fn ResumeTimers
  (bind _values (Utilities|Map|Values (Variables|Events|GetTimerHandles)))
  (for _array_element _values
    (Utilities|Time|UnpauseTimerbyHandle _array_element)))

(fn NewEventTimer
  (params (Event :type EPassiveSignals%20Enum :default "NewEnumerator2"))
  (if (Math|Boolean|NORBoolean (.ReturnValue (Utilities|Map|Find (Variables|Events|GetTimerHandles) Event)) (Variables|Events|GetEventIsActive))
    (bind _event_delay (Events|GetEventDelay Event))
    (bind _returnvalue (Class|CustomTimerActor|CreateTimer (Math|Conversions|ToInteger(Byte) Event) _event_delay))
    (Utilities|Map|Add (Variables|Events|GetTimerHandles) Event _returnvalue)
    (Development|PrintString (Utilities|String|Append "Created timer: " (Utilities|String|EnumtoString Event)) true true "(R=0.000000,G=0.791958,B=1.000000,A=1.000000)" 5.0)))