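; BP_CameraShaker is an event-controller actor that plays a world camera shake whenever OnAnyEvent fires.
; The shake uses the configured type, outer radius and falloff, with its epicenter at the Radius sphere component's location.
; The construction script sizes that sphere from ShakeRadius and moves it to the referenced machine's root when MachineReference is valid.
; ShakeRadius only sets the sphere, while the shake's range comes from the separate OuterRadius.
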(event EventOnAnyEvent
  (params (Event :type EHavocEvents%20Enum :default "NewEnumerator0"))
  (CallFunction|Shake))

(fn ConstructionScript
  (bind _machinereference (Variables|Default|GetMachineReference))
  (Components|Sphere|SetSphereRadius (Variables|Default|GetRadius) (Variables|Default|GetShakeRadius) true)
  (if (Utilities|IsValid _machinereference)
    (Transformation|SetWorldLocation (Variables|Default|GetRadius) (Transformation|GetWorldLocation (Variables|/Game/Blueprints/Source/MachineComponents/Base/BP_MCBase.BP_MCBase_C|GetDefaultSceneRoot _machinereference)) false false)))

(fn Shake
  (Camera|PlayWorldCameraShake (Variables|Default|GetShakeType) (Transformation|GetWorldLocation (Variables|Default|GetRadius)) 0.0 (LocalVariables|GetOuterRadius) (Variables|Default|GetFalloff)))