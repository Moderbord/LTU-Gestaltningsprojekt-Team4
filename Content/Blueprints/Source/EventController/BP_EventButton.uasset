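; BP_EventButton is an alert indicator that watches a component's passive signal and reports chaos to the EventController.
; Each Tick compares the signal against the minimum threshold, optionally reversed, and shows the indicator light while alerting.
; Alerting contributors report their ChaosPool, scaled by signal position between the thresholds unless these are nearly equal; otherwise they report zero.
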(event EventBeginPlay
  (Rendering|SetVisibility (Variables|Default|GetIndicatorLight) false false))

(event EventTick
  (params (DeltaSeconds :type Float%20%28single-precision%29))
  (bind (_value _alert) (CallFunction|EvalSignal))
  (bind _output_get (Variables|Signaling|SetState _alert))
  (if _output_get
    (Rendering|SetVisibility (Variables|Default|GetIndicatorLight) true false)
    (CallFunction|OnStateChange (Variables|Signaling|GetState) _value)
    (else
      (Rendering|SetVisibility (Variables|Default|GetIndicatorLight) false false)
      (CallFunction|OnStateChange (Variables|Signaling|GetState) 0.0))))

(fn ConstructionScript)

(fn GetChaos
  (params (Current :type Float%20%28single-precision%29))
  (if (Math|Float|NearlyEqual(Float) (Variables|Signaling|GetSignalMaxThreshold) (Variables|Signaling|GetSignalMinThreshold) 0.01)
    (return (Variables|Chaos|GetChaosPool))
    (else
      (bind _out (CallFunction|ChaosPoolWeight Current))
      (return _out))))

(fn ChaosPoolWeight
  (params (Amount :type Float%20%28single-precision%29))
  (return (* (Math|Float|Clamp(Float) (/ (Math|Float|Absolute(Float) (- Amount (Variables|Signaling|GetSignalMinThreshold))) (Math|Float|Absolute(Float) (- (Variables|Signaling|GetSignalMaxThreshold) (Variables|Signaling|GetSignalMinThreshold))))) (Variables|Chaos|GetChaosPool))))

(fn EvalSignal
  (bind _passive (Variables|Default|GetPassive))
  (bind _component (Variables|Default|GetComponent))
  (bind _out_signals (Variables|/Game/Blueprints/Source/MachineComponents/Base/BP_MCBase.BP_MCBase_C|GetOut%20Signals _component))
  (bind _value (Utilities|Map|Find _out_signals _passive))
  (if (Variables|Signaling|GetReverseThresholdCheck)
    (return _value (< _value (Variables|Signaling|GetSignalMinThreshold)))
    (else
      (return _value (> _value (Variables|Signaling|GetSignalMinThreshold))))))

(fn OnStateChange
  (params (State :type Boolean) (Value :type Float%20%28single-precision%29))
  (if (and State (Variables|Chaos|GetChaosContributor))
    (bind _out (CallFunction|GetChaos Value))
    (Default|AddtoChaosMap (Variables|Signaling|GetEventController) self _out)
    (else
      (Default|AddtoChaosMap (Variables|Signaling|GetEventController) self 0.0))))