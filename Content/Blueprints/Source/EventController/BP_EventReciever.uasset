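; BP_EventReciever is an actor that visualizes game events by recoloring its Cube mesh, with a distinct color for generic, power failure, high pressure and short circuit events.
; Each event handler creates a new dynamic instance of the EventColor material on the cube and sets its BaseColor parameter.
; Chaos stage changes only print the new stage to the screen, and the file does not bind or dispatch the events itself.
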(event EventBeginPlay)

(event Collision|EventActorBeginOverlap
  (params (OtherActor :type Actor%20Object%20Reference)))

(event EventTick
  (params (DeltaSeconds :type Float%20%28single-precision%29)))

(event EventOnPowerFailureEvent
  (bind _returnvalue (Rendering|Material|CreateDynamicMaterialInstance (Variables|Default|GetCube) 0 "/Game/Blueprints/Source/EventController/EventColor.EventColor" "None" :!class /Script/Engine.PrimitiveComponent))
  (Rendering|Material|SetVectorParameterValue _returnvalue "BaseColor" "(R=1.000000,G=0.844624,B=0.000000,A=1.000000)" :!class /Script/Engine.MaterialInstanceDynamic))

(event EventOnGenericEvent
  (bind _returnvalue (Rendering|Material|CreateDynamicMaterialInstance (Variables|Default|GetCube) 0 "/Game/Blueprints/Source/EventController/EventColor.EventColor" "None" :!class /Script/Engine.PrimitiveComponent))
  (Rendering|Material|SetVectorParameterValue _returnvalue "BaseColor" "(R=1.000000,G=0.997690,B=0.962442,A=1.000000)" :!class /Script/Engine.MaterialInstanceDynamic))

(event EventOnHighPressureEvent
  (bind _returnvalue (Rendering|Material|CreateDynamicMaterialInstance (Variables|Default|GetCube) 0 "/Game/Blueprints/Source/EventController/EventColor.EventColor" "None" :!class /Script/Engine.PrimitiveComponent))
  (Rendering|Material|SetVectorParameterValue _returnvalue "BaseColor" "(R=0.000000,G=0.186898,B=1.000000,A=1.000000)" :!class /Script/Engine.MaterialInstanceDynamic))

(event EventOnShortCircuitEvent
  (bind _returnvalue (Rendering|Material|CreateDynamicMaterialInstance (Variables|Default|GetCube) 0 "/Game/Blueprints/Source/EventController/EventColor.EventColor" "None" :!class /Script/Engine.PrimitiveComponent))
  (Rendering|Material|SetVectorParameterValue _returnvalue "BaseColor" "(R=1.000000,G=0.000000,B=0.817070,A=1.000000)" :!class /Script/Engine.MaterialInstanceDynamic))

(event EventOnChaosStageChange
  (params (Stage :type Integer))
  (Development|PrintString (Utilities|String|ToString(Integer) Stage) true true "(R=1.000000,G=0.931425,B=0.000000,A=1.000000)"))

(fn ConstructionScript)