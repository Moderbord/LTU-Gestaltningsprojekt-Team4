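; Sound controller actor that drives the chaos soundscape through FMOD from the game's chaos state.
; A stage change starts the 2D chaos event if none is playing and toggles the global "Chaos" parameter.
; ChaosHandling, run on a throttled tick and on stage changes, feeds BP_EventController's total chaos into the instance's level parameter and fades volume up to full at 25.
; Puzzle success and failure sound nodes are unconnected.
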(event EventBeginPlay
  (Actor|Tick|SetActorTickInterval (Variables|Default|GetTickIntervall))
  (bind _returnvalue (Actor|GetActorOfClass "/Game/Blueprints/Source/EventController/BP_EventController.BP_EventController_C"))
  (Variables|Default|SetEventController _returnvalue))

(event Collision|EventActorBeginOverlap
  (params (OtherActor :type Actor%20Object%20Reference)))

(event EventTick
  (params (DeltaSeconds :type Float%20%28single-precision%29))
  (CallFunction|ChaosHandling))

(event EventOnChaosStageChange
  (params (Stage :type Integer))
  (Utilities|FlowControl|Sequence
    (:then_0
      (if (>= Stage 0)
        (Utilities|FlowControl|Sequence
          (:then_0
            (bind _returnvalue (Class|FMODBlueprintStatics|EventInstanceIsValid (Variables|Default|GetChaosInstance)))
            (if (not _returnvalue)
              (bind _returnvalue_2 (Class|FMODBlueprintStatics|PlayEvent2D (Variables|Default|GetChaosEvent)))
              (Variables|Default|SetChaosInstance _returnvalue_2)))
          (:then_1
            (Class|FMODBlueprintStatics|SetGlobalParameterbyName "Chaos" 1.0)))
        (else
          (Class|FMODBlueprintStatics|SetGlobalParameterbyName "Chaos" 0.0))))
    (:then_1
      (CallFunction|ChaosHandling))))

(fn ConstructionScript)

(fn ChaosHandling
  (bind _chaosinstance (Variables|Default|GetChaosInstance))
  (bind _out (Default|GetTotalChaos (Variables|Default|GetEventController)))
  (bind _returnvalue (Class|FMODBlueprintStatics|EventInstanceIsValid _chaosinstance))
  (if _returnvalue
    (Class|FMODBlueprintStatics|EventInstanceSetParameter _chaosinstance "Chaos_level" _out)
    (if (>= _out 25.0)
      (Class|FMODBlueprintStatics|EventInstanceSetVolume _chaosinstance 1.0)
      (else
        (Class|FMODBlueprintStatics|EventInstanceSetVolume _chaosinstance (* _out 0.04))))))