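; First-person player character that interacts with objects, drags physics props and toggles a flashlight once the Interact event grants it.
; InteractMode toggles a cursor mode that freezes camera rotation.
; Fire line-traces from camera or cursor, sending hit actors interact and impact-offset messages.
; Grabbed physics components follow the view through a PhysicsHandle, or the deprojected mouse via per-tick SetRelativeLocation in cursor mode, at their grab distance.
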(event EventBeginPlay
  ;[1 1 1] Flashlight
  (Rendering|ToggleVisibility (Variables|Default|GetSpotLight) false)
  ;[1 1 1] Enable input
  (Input|EnableInput (Game|GetPlayerController 0)))

(event EventTick
  (params (DeltaSeconds :type Float%20%28single-precision%29))
  (bind _returnvalue (Game|GetPlayerController 0))
  (bind (_worldlocation _worlddirection) (Game|Player|ConvertMouseLocationToWorldSpace _returnvalue))
  ;[1 1 1] Transform component
  (if (Variables|Default|GetInteractiveMode)
    (Pawn|SetControlRotation _returnvalue (Variables|Default|GetInteractModeCameraRotation))
    (if (Utilities|IsValid (Variables|Default|GetGrabbedComponent))
      (if (Physics|IsSimulatingPhysics (Variables|Default|GetGrabbedComponent) "None")
        (Transformation|SetRelativeLocation (Variables|Default|GetGrabbedComponent) (+ _worldlocation (* _worlddirection (- (Variables|Default|GetOriginalDistanceToObject) 1e+01))) false false)))))

(event EventInteract
  (params (Caller :type Actor%20Object%20Reference))
  ;[1 1 1] Flashlight
  (Variables|Default|SetHasFlashlight true))

(event Input|ActionEvents|InputActionFlashlight
  (params (Key :type Key%20Structure :default "None"))
  ;[1 1 1] Flashlight
  (:Pressed
    (if (Variables|Default|GetHasFlashlight)
      (Utilities|FlowControl|FlipFlop
        (:A
          _)
        (:B
          _))
      (Rendering|ToggleVisibility (Variables|Default|GetSpotLight) false))))

(event Input|ActionEvents|InputActionInteractMode
  (params (Key :type Key%20Structure :default "None"))
  (bind _returnvalue (Game|GetPlayerController 0))
  ;[1 1 1] Set Interactive mode
  (:Pressed
    (bind _isa (Utilities|FlowControl|FlipFlop)
      (:A
        (Input|SetInputModeGameandUI _returnvalue 0 "DoNotLock" false)
        (Variables|Default|SetInteractModeCameraRotation (Pawn|GetControlRotation _returnvalue :!class /Script/Engine.Controller)))
      (:B
        (Input|SetInputModeGameOnly _returnvalue)
        (Physics|Components|PhysicsHandle|ReleaseComponent (Variables|Default|GetPhysicsHandle))))
    (bind _output_get (Variables|/Script/Engine.PlayerController|SetbShowMouseCursor _returnvalue _isa))
    (Variables|Default|SetInteractiveMode _output_get)))

(event Input|ActionEvents|InputActionFire
  (params (Key :type Key%20Structure :default "None"))
  (bind _returnvalue (Game|GetPlayerController 0))
  (bind _firstpersoncamera (Variables|Default|GetFirstPersonCamera))
  (bind _physicshandle (Variables|Default|GetPhysicsHandle))
  (bind _interactivemode (Variables|Default|GetInteractiveMode))
  (bind _interactivemode_2 (Variables|Default|GetInteractiveMode))
  (bind _returnvalue_2 (Transformation|GetWorldLocation _firstpersoncamera))
  (bind (_worldlocation _worlddirection) (Game|Player|ConvertMouseLocationToWorldSpace _returnvalue))
  ;[1 1 1] Handle button press
  (:Pressed
    (if _interactivemode_2
      ;[1 1 1] Grab component interactive mode
      (if _interactivemode
        (bind (_outhit _returnvalue_3) (Collision|LineTraceByChannel _worldlocation (+ (* _worlddirection 3e+02) _worldlocation) "TraceTypeQuery1" true 0 "ForDuration"))
        (if _returnvalue_3
          (Class|ComponentInterface|Interact(Message) (.HitActor (Collision|BreakHitResult _outhit)) self)
          (Utilities|IsValid (.HitActor (Collision|BreakHitResult _outhit))
            (:Is%20Valid
              (if (== (Variables|/Script/Engine.SceneComponent|GetMobility (.HitComponent (Collision|BreakHitResult _outhit))) (Utilities|Enum|LiteralenumEComponentMobility "Movable"))
                (Class|ComponentInterface|AxisValuesEvent(Message) (.HitActor (Collision|BreakHitResult _outhit)) (Math|Vector|MakeVector (- (.x (.ImpactPoint (Collision|BreakHitResult _outhit))) (.x (Transformation|GetWorldLocation (.HitComponent (Collision|BreakHitResult _outhit))))) (- (.y (.ImpactPoint (Collision|BreakHitResult _outhit))) (.y (Transformation|GetWorldLocation (.HitComponent (Collision|BreakHitResult _outhit))))) (- (.z (.ImpactPoint (Collision|BreakHitResult _outhit))) (.z (Transformation|GetWorldLocation (.HitComponent (Collision|BreakHitResult _outhit)))))))
                (if (Physics|IsSimulatingPhysics (.HitComponent (Collision|BreakHitResult _outhit)) "None")
                  (Variables|Default|SetOriginalDistanceToObject (.Distance (Collision|BreakHitResult _outhit)))
                  (Variables|Default|SetGrabbedActor (.HitActor (Collision|BreakHitResult _outhit)))
                  (Variables|Default|SetGrabbedComponent (.HitComponent (Collision|BreakHitResult _outhit)))))))))
      (else
        ;[1 1 1] Grab component without interactive mode
        (bind (_outhit_2 _returnvalue_4) (Collision|LineTraceByChannel _returnvalue_2 (+ (* (Math|Vector|GetForwardVector _firstpersoncamera) 3e+02) _returnvalue_2) "TraceTypeQuery1" false 0 "ForDuration"))
        (Variables|Default|SetOriginalDistanceToObject (.Distance (Collision|BreakHitResult _outhit_2)))
        (if _returnvalue_4
          (Class|ComponentInterface|Interact(Message) (.HitActor (Collision|BreakHitResult _outhit_2)) self)
          (Utilities|IsValid (.HitActor (Collision|BreakHitResult _outhit_2))
            (:Is%20Valid
              (Class|ComponentInterface|AxisValuesEvent(Message) (.HitActor (Collision|BreakHitResult _outhit_2)) (Math|Vector|MakeVector (- (.x (.ImpactPoint (Collision|BreakHitResult _outhit_2))) (.x (Transformation|GetWorldLocation (.HitComponent (Collision|BreakHitResult _outhit_2))))) (- (.y (.ImpactPoint (Collision|BreakHitResult _outhit_2))) (.y (Transformation|GetWorldLocation (.HitComponent (Collision|BreakHitResult _outhit_2))))) (- (.z (.ImpactPoint (Collision|BreakHitResult _outhit_2))) (.z (Transformation|GetWorldLocation (.HitComponent (Collision|BreakHitResult _outhit_2)))))))
              (if (Physics|IsSimulatingPhysics (.HitComponent (Collision|BreakHitResult _outhit_2)) "None")
                (Physics|Components|PhysicsHandle|GrabComponentatLocationwithRotation _physicshandle (.HitComponent (Collision|BreakHitResult _outhit_2)) "None" (.Location (Collision|BreakHitResult _outhit_2)) (Variables|/Script/Engine.SceneComponent|GetRelativeRotation (.HitComponent (Collision|BreakHitResult _outhit_2))))
                (Class|PhysicsHandleComponent|SetAngularDamping _physicshandle 1e+03))))))))
  (:Released
    (if _interactivemode_2
      (if _interactivemode
        (Variables|Default|SetGrabbedComponent 0)
        (Variables|Default|SetGrabbedActor 0)
        (Physics|Components|PhysicsHandle|ReleaseComponent (Variables|Default|GetPhysicsHandle)))
      (else
        (Physics|Components|PhysicsHandle|ReleaseComponent (Variables|Default|GetPhysicsHandle))))))

(event Input|AxisEvents|InputAxisTurn
  (params (AxisValue :type Float%20%28single-precision%29))
  (bind _firstpersoncamera (Variables|Default|GetFirstPersonCamera))
  ;[1 1 1] Rotate object depending on mouse input
  (Pawn|Input|AddControllerYawInput AxisValue)
  (if (not (Variables|Default|GetInteractiveMode))
    (Physics|Components|PhysicsHandle|SetTargetLocation (Variables|Default|GetPhysicsHandle) (+ (* (Math|Vector|GetForwardVector _firstpersoncamera) (- (Variables|Default|GetOriginalDistanceToObject) 1e+01)) (Transformation|GetWorldLocation _firstpersoncamera)))))

(event Input|AxisEvents|InputAxisLookUp
  (params (AxisValue :type Float%20%28single-precision%29))
  (bind _firstpersoncamera (Variables|Default|GetFirstPersonCamera))
  ;[1 1 1] Rotate object depending on mouse input
  (Pawn|Input|AddControllerPitchInput AxisValue)
  (if (not (Variables|Default|GetInteractiveMode))
    (Physics|Components|PhysicsHandle|SetTargetLocation (Variables|Default|GetPhysicsHandle) (+ (* (Math|Vector|GetForwardVector _firstpersoncamera) (- (Variables|Default|GetOriginalDistanceToObject) 1e+01)) (Transformation|GetWorldLocation _firstpersoncamera)))))

(fn ConstructionScript)