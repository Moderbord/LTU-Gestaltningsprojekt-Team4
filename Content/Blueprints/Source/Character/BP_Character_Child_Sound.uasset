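; Character child Blueprint that drives FMOD footstep audio from movement speed and floor surface.
; Each tick it sets the global WalkingSpeed parameter from velocity and the Material parameter from a downward trace's physical surface (tile, stone, metal or default).
; A Footsteps macro then uses a Delay, shortened as speed rises, to pace Footsteps and Running events, both played attached to the capsule without any minimum-speed check.
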(event EventBeginPlay
  (|CallParentFunction) ; This node is disabled and will not be called.\nDrag off pins to build functionality.
)

(event Collision|EventActorBeginOverlap
  (params (OtherActor :type Actor%20Object%20Reference)))

(event EventTick
  (params (DeltaSeconds :type Float%20%28single-precision%29))
  (|CallParentFunction DeltaSeconds)
  (CallFunction|GetMovementSpeed)
  (CallFunction|GetMaterial)
  (Utilities|Footsteps))

(fn ConstructionScript
  (|CallParentFunction))

(fn GetMovementSpeed
  (Variables|Default|SetWalkingSpeed (Math|Float|Absolute(Float) (Math|Vector|VectorLength (Variables|/Script/Engine.MovementComponent|GetVelocity (Pawn|GetMovementComponent)))))
  (Class|FMODBlueprintStatics|SetGlobalParameterbyName "WalkingSpeed" (Variables|Default|GetWalkingSpeed)))

(fn GetMaterial
  (bind _capsulecomponent (Variables|Default|GetCapsuleComponent))
  (bind _returnvalue (Transformation|GetWorldLocation _capsulecomponent))
  (bind _outhit (Collision|LineTraceByChannel (Transformation|GetWorldLocation _capsulecomponent) (Math|Vector|MakeVector (.x _returnvalue) (.y _returnvalue) (- (.z _returnvalue) 1.2e+02)) "TraceTypeQuery1" true 0 "None"))
  (switch Utilities|FlowControl|Switch|SwitchonEPhysicalSurface (Variables|/Script/Engine.PhysicalMaterial|GetSurfaceType (.PhysMat (Collision|BreakHitResult _outhit)))
    (:SurfaceType_Default
      (Variables|Default|SetMaterial 3.0))
    (:SurfaceType1
      (Variables|Default|SetMaterial 0.0))
    (:SurfaceType2
      (Variables|Default|SetMaterial 1.0))
    (:SurfaceType3
      (Variables|Default|SetMaterial 2.0)))
  (Class|FMODBlueprintStatics|SetGlobalParameterbyName "Material" (Variables|Default|GetMaterial)))