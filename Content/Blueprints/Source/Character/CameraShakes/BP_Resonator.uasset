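; BP_Resonator is an actor that shakes cameras around it while it is being overlapped.
; Begin and end overlap events toggle a flag without filtering by actor, so any actor leaving clears it.
; While the flag is set, Tick plays a world camera shake every frame from the root's location, using the configured class, radius and falloff.
; The construction script sizes the Radius sphere to the shake's outer radius.
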(event Collision|EventActorBeginOverlap
  (params (OtherActor :type Actor%20Object%20Reference))
  (Variables|Default|SetShake true))

(event EventTick
  (params (DeltaSeconds :type Float%20%28single-precision%29))
  (if (Variables|Default|GetShake)
    (Camera|PlayWorldCameraShake (Variables|Default|GetShakeClass) (Transformation|GetWorldLocation (Variables|Default|GetDefaultSceneRoot)) 0.0 (Variables|Default|GetShakeRadius) (Variables|Default|GetShakeFalloff))))

(event Collision|EventActorEndOverlap
  (params (OtherActor :type Actor%20Object%20Reference))
  (Variables|Default|SetShake false))

(fn ConstructionScript
  (Components|Sphere|SetSphereRadius (Variables|Default|GetRadius) (Variables|Default|GetShakeRadius) true))