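; First-person player character with sprint, smooth FOV zoom, pause menu, and a flashlight and notebook unlocked by pickups.
; DoTrace raycasts from the camera, or from the cursor in toggled interactive mode, driving hover and interaction events.
; Physics objects are dragged by PhysicsHandle or by cursor-driven relocation.
; Non-simulating hits become the AnalogueActor, which receives mouse input instead of the camera.
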(event EventTick
  (params (DeltaSeconds :type Float%20%28single-precision%29))
  (bind _returnvalue (Game|GetPlayerController 0))
  (bind _grabbedcomponent (Variables|Default|GetGrabbedComponent))
  (bind (_worldlocation _worlddirection) (Game|Player|ConvertMouseLocationToWorldSpace _returnvalue))
  (Utilities|FlowControl|Sequence
    (:then_0
      ;[1 1 1] Transform component
      (if (Variables|Default|GetIsInteracting)
        (Class|ComponentInterface|OnInteractStep(Message) (Variables|Default|GetAnalogueActor))
        (if (Variables|Default|GetInteractiveMode)
          (if (Utilities|IsValid _grabbedcomponent)
            (if (Physics|IsSimulatingPhysics _grabbedcomponent "None")
              (Transformation|SetRelativeLocation _grabbedcomponent (+ _worldlocation (* _worlddirection (- (Variables|Default|GetOriginalDistanceToObject) 1e+01))) false false))))))
    (:then_1
      ;[1 1 1] Do OnHover event
      (bind (_success _hitresult) (CallFunction|DoTrace (Variables|Default|GetInteractiveMode)))
      (if _success
        (if (!= (Variables|Rendering|GetCurrentHover) (.HitActor (Collision|BreakHitResult _hitresult)))
          (Utilities|FlowControl|Sequence
            (:then_0
              (Utilities|IsValid (Variables|Rendering|GetCurrentHover) :!label _label
                (:Is%20Valid
                  (bind _ascomponent_interface (Utilities|Casting|CastToComponentInterface (Variables|Rendering|GetCurrentHover)))
                  (Variables|Rendering|SetCurrentHover 0)
                  (Default|OnHover _ascomponent_interface false))))
            (:then_1
              (bind _ascomponent_interface_2 (Utilities|Casting|CastToComponentInterface (.HitActor (Collision|BreakHitResult _hitresult))))
              (Variables|Rendering|SetCurrentHover (.HitActor (Collision|BreakHitResult _hitresult)))
              (Default|OnHover _ascomponent_interface_2 true))))
        (else
          (goto _label))))
    (:then_2
      ;[1 1 1] Smooth zoom
      (bind _output_get (Variables|Rendering|SetZoomDelta (Math|Interpolation|FInterpTo (Variables|Rendering|GetZoomDelta) (Math|Float|SelectFloat (Variables|Rendering|GetFOVZoom) (Variables|Rendering|GetFOVStandard) (Variables|Rendering|GetIsZoomed)) DeltaSeconds (Variables|Default|GetZoomSpeed))))
      (Camera|SetFieldOfView (Variables|Default|GetFirstPersonCamera) _output_get))))

(event EventOnBeginInteract
  (params (Caller :type Actor%20Object%20Reference))
  ;[1 1 1] Flashlight
  (Utilities|Casting|CastToBP_Flashlight Caller
    (:then
      (Variables|Default|SetHasFlashlight true)
      (bind _returnvalue (UserInterface|CreateWidget "/Game/Blueprints/Source/LevelBlueprints/Widgets/Tips/FlashlightTipsWidgetAnimated.FlashlightTipsWidgetAnimated_C" (Game|GetPlayerController 0)))
      (UserInterface|Viewport|AddtoViewport _returnvalue 0)
      (Utilities|FlowControl|Delay (Variables|Default|GetTipsDuration))
      (Widget|RemovefromParent _returnvalue))
    (:CastFailed
      ;[1 1 1] Notebook
      (Utilities|Casting|CastToBP_Notebook Caller)
      (Variables|Default|SetHasNotebook true)
      (bind _returnvalue_2 (UserInterface|CreateWidget "/Game/Blueprints/Source/Interaction/Book/NotebookWidget.NotebookWidget_C" (Game|GetPlayerController 0)))
      (bind _output_get (Variables|Default|SetNotebookWidget _returnvalue_2))
      (UserInterface|Viewport|AddtoViewport _output_get 0)
      (Widget|SetVisibility (Variables|Default|GetNotebookWidget) "Hidden")
      (bind _returnvalue_3 (UserInterface|CreateWidget "/Game/Blueprints/Source/LevelBlueprints/Widgets/Tips/NotebookTipsWidgetAnimated.NotebookTipsWidgetAnimated_C" (Game|GetPlayerController 0)))
      (UserInterface|Viewport|AddtoViewport _returnvalue_3 0)
      (Utilities|FlowControl|Delay (Variables|Default|GetTipsDuration))
      (Widget|RemovefromParent _returnvalue_3))))

(event EventBeginPlay
  (bind _returnvalue (Game|GetPlayerController 0))
  (Utilities|FlowControl|Sequence
    (:then_0
      ;[1 1 1] Flashlight
      (Rendering|ToggleVisibility (Variables|Default|GetSpotLight) false))
    (:then_1
      ;[1 1 1] Set default player values
      (Input|EnableInput _returnvalue)
      (Variables|/Script/Engine.CharacterMovementComponent|SetMaxWalkSpeed (Variables|Character|GetCharacterMovement) (Variables|Default|GetWalkSpeed)))
    (:then_2
      ;[1 1 1] Pause menu widget
      (bind _returnvalue_2 (UserInterface|CreateWidget "/Game/Blueprints/Source/Character/HUDWidget.HUDWidget_C" _returnvalue))
      (bind _output_get (Variables|Default|SetHUDWidget _returnvalue_2))
      (UserInterface|Viewport|AddtoViewport _output_get 0))))

(event Input|ActionEvents|InputActionPause
  (params (Key :type Key%20Structure :default "None"))
  ;[1 1 1] Pause
  (:Pressed
    (CallFunction|Pause)))

(event Input|ActionEvents|InputActionInteractMode
  (params (Key :type Key%20Structure :default "None"))
  (bind _returnvalue (Game|GetPlayerController 0))
  ;[1 1 1] Set Interactive mode
  (:Pressed
    (bind _isa (Utilities|FlowControl|FlipFlop)
      (:A
        (Input|SetInputModeGameandUI _returnvalue 0 "DoNotLock" false)
        (Class|PlayerController|SetCinematicMode _returnvalue true false false true true))
      (:B
        (Input|SetInputModeGameOnly _returnvalue)
        (Physics|Components|PhysicsHandle|ReleaseComponent (Variables|Default|GetPhysicsHandle))
        (Class|PlayerController|SetCinematicMode _returnvalue false true true true true)))
    (bind _output_get (Variables|/Script/Engine.PlayerController|SetbShowMouseCursor _returnvalue _isa))
    (Variables|Default|SetInteractiveMode _output_get)))

(event Input|ActionEvents|InputActionFire
  (params (Key :type Key%20Structure :default "None"))
  (bind _physicshandle (Variables|Default|GetPhysicsHandle))
  ;[1 1 1] Handle button press
  (:Pressed
    (if (Variables|Default|GetInteractiveMode)
      ;[1 1 1] Grab component interactive mode
      (bind (_success _hitresult) (CallFunction|DoTrace true))
      (if _success
        (Class|ComponentInterface|OnBeginInteract(Message) (.HitActor (Collision|BreakHitResult _hitresult)) self)
        (Utilities|IsValid (.HitActor (Collision|BreakHitResult _hitresult))
          (:Is%20Valid
            (Variables|Default|SetIsInteracting true)
            (if (== (Variables|/Script/Engine.SceneComponent|GetMobility (.HitComponent (Collision|BreakHitResult _hitresult))) (Utilities|Enum|LiteralenumEComponentMobility "Movable"))
              (Class|ComponentInterface|AxisValuesEvent(Message) (.HitActor (Collision|BreakHitResult _hitresult)) (Math|Vector|MakeVector (- (.x (.ImpactPoint (Collision|BreakHitResult _hitresult))) (.x (Transformation|GetWorldLocation (.HitComponent (Collision|BreakHitResult _hitresult))))) (- (.y (.ImpactPoint (Collision|BreakHitResult _hitresult))) (.y (Transformation|GetWorldLocation (.HitComponent (Collision|BreakHitResult _hitresult))))) (- (.z (.ImpactPoint (Collision|BreakHitResult _hitresult))) (.z (Transformation|GetWorldLocation (.HitComponent (Collision|BreakHitResult _hitresult)))))))
              (if (Physics|IsSimulatingPhysics (.HitComponent (Collision|BreakHitResult _hitresult)) "None")
                (Variables|Default|SetOriginalDistanceToObject (.Distance (Collision|BreakHitResult _hitresult)))
                (Variables|Default|SetGrabbedActor (.HitActor (Collision|BreakHitResult _hitresult)))
                (Variables|Default|SetGrabbedComponent (.HitComponent (Collision|BreakHitResult _hitresult)))
                (else
                  (Variables|Default|SetAnalogueActor (.HitActor (Collision|BreakHitResult _hitresult)))))))))
      (else
        ;[1 1 1] Grab component without interactive mode
        (bind (_success_2 _hitresult_2) (CallFunction|DoTrace false))
        (Variables|Default|SetOriginalDistanceToObject (.Distance (Collision|BreakHitResult _hitresult_2)))
        (if _success_2
          (Class|ComponentInterface|OnBeginInteract(Message) (.HitActor (Collision|BreakHitResult _hitresult_2)) self)
          (Utilities|IsValid (.HitActor (Collision|BreakHitResult _hitresult_2))
            (:Is%20Valid
              (Variables|Default|SetIsInteracting true)
              (Class|ComponentInterface|AxisValuesEvent(Message) (.HitActor (Collision|BreakHitResult _hitresult_2)) (Math|Vector|MakeVector (- (.x (.ImpactPoint (Collision|BreakHitResult _hitresult_2))) (.x (Transformation|GetWorldLocation (.HitComponent (Collision|BreakHitResult _hitresult_2))))) (- (.y (.ImpactPoint (Collision|BreakHitResult _hitresult_2))) (.y (Transformation|GetWorldLocation (.HitComponent (Collision|BreakHitResult _hitresult_2))))) (- (.z (.ImpactPoint (Collision|BreakHitResult _hitresult_2))) (.z (Transformation|GetWorldLocation (.HitComponent (Collision|BreakHitResult _hitresult_2)))))))
              (if (Physics|IsSimulatingPhysics (.HitComponent (Collision|BreakHitResult _hitresult_2)) "None")
                (Physics|Components|PhysicsHandle|GrabComponentatLocationwithRotation _physicshandle (.HitComponent (Collision|BreakHitResult _hitresult_2)) "None" (.Location (Collision|BreakHitResult _hitresult_2)) (Variables|/Script/Engine.SceneComponent|GetRelativeRotation (.HitComponent (Collision|BreakHitResult _hitresult_2))))
                (Class|PhysicsHandleComponent|SetAngularDamping _physicshandle 1e+03)
                (else
                  (Variables|Default|SetAnalogueActor (.HitActor (Collision|BreakHitResult _hitresult_2)))))))))))
  (:Released
    (Class|ComponentInterface|OnEndInteract(Message) (Variables|Default|GetAnalogueActor))
    (Variables|Default|SetIsInteracting false)
    (if (Variables|Default|GetInteractiveMode)
      ;[1 1 1] Release object in Interactive Mode
      (Variables|Default|SetGrabbedComponent 0)
      (Variables|Default|SetGrabbedActor 0)
      (Physics|Components|PhysicsHandle|ReleaseComponent (Variables|Default|GetPhysicsHandle))
      (Variables|Default|SetAnalogueActor 0)
      (else
        ;[1 1 1] Release object without Interactive Mode
        (Physics|Components|PhysicsHandle|ReleaseComponent (Variables|Default|GetPhysicsHandle))
        (Variables|Default|SetAnalogueActor 0)))))

(event Input|ActionEvents|InputActionNotebook
  (params (Key :type Key%20Structure :default "None"))
  (bind _notebookwidget (Variables|Default|GetNotebookWidget))
  ;[1 1 1] Notebook
  (:Pressed
    (if (Variables|Default|GetHasNotebook)
      (Utilities|FlowControl|FlipFlop
        (:A
          (Class|FMODBlueprintStatics|PlayEvent2D "/Game/FMOD/Events/SFX/Interaction_SFX/Notebook/Notebook_open.Notebook_open")
          (Widget|SetVisibility _notebookwidget "Visible"))
        (:B
          (Class|FMODBlueprintStatics|PlayEvent2D "/Game/FMOD/Events/SFX/Interaction_SFX/Notebook/Notebook_close.Notebook_close")
          (Widget|SetVisibility _notebookwidget "Hidden")))
      (CallFunction|PauseNotebook))))

(event Input|ActionEvents|InputActionSprint
  (params (Key :type Key%20Structure :default "None"))
  (bind _charactermovement (Variables|Character|GetCharacterMovement))
  ;[1 1 1] Sprint
  (:Pressed
    (Variables|/Script/Engine.CharacterMovementComponent|SetMaxWalkSpeed _charactermovement (Variables|Default|GetRunSpeed)))
  (:Released
    (Variables|/Script/Engine.CharacterMovementComponent|SetMaxWalkSpeed _charactermovement (Variables|Default|GetWalkSpeed))))

(event Input|ActionEvents|InputActionFlashlight
  (params (Key :type Key%20Structure :default "None"))
  (bind _capsulecomponent (Variables|Collision|GetCapsuleComponent))
  ;[1 1 1] Flashlight
  (:Pressed
    (if (Variables|Default|GetHasFlashlight)
      (Utilities|FlowControl|FlipFlop
        (:A
          (Class|FMODBlueprintStatics|PlayEventAttached "/Game/FMOD/Events/SFX/Interaction_SFX/Flashlight/Flashlight_On.Flashlight_On" _capsulecomponent "None" "0, 0, 0" "KeepRelativeOffset"))
        (:B
          (Class|FMODBlueprintStatics|PlayEventAttached "/Game/FMOD/Events/SFX/Interaction_SFX/Flashlight/Flashlight_Off.Flashlight_Off" _capsulecomponent "None" "0, 0, 0" "KeepRelativeOffset")))
      (Rendering|ToggleVisibility (Variables|Default|GetSpotLight) false))))

(event Input|AxisEvents|InputAxisMoveRight
  (params (AxisValue :type Float%20%28single-precision%29))
  ;[1 1 1] Movement
  (if (not (Variables|Default|GetInteractiveMode))
    (Pawn|Input|AddMovementInput (Math|Vector|GetRightVector (Variables|Default|GetFirstPersonCamera)) AxisValue false)))

(event Input|AxisEvents|InputAxisMoveForward
  (params (AxisValue :type Float%20%28single-precision%29))
  ;[1 1 1] Movement
  (if (not (Variables|Default|GetInteractiveMode))
    (Pawn|Input|AddMovementInput (Math|Vector|GetForwardVector (Variables|Default|GetFirstPersonCamera)) AxisValue false)))

(event Input|AxisEvents|InputAxisTurn
  (params (AxisValue :type Float%20%28single-precision%29))
  (bind _firstpersoncamera (Variables|Default|GetFirstPersonCamera))
  (bind _analogueactor (Variables|Default|GetAnalogueActor))
  ;[1 1 1] Rotate object depending on mouse input
  (if (Utilities|IsValid _analogueactor)
    (Class|ComponentInterface|MouseValues(Message) _analogueactor AxisValue (stale Input|AxisEvents|InputAxisLookUp AxisValue))
    (else
      (Pawn|Input|AddControllerYawInput AxisValue)
      (if (not (Variables|Default|GetInteractiveMode))
        (Physics|Components|PhysicsHandle|SetTargetLocation (Variables|Default|GetPhysicsHandle) (+ (* (Math|Vector|GetForwardVector _firstpersoncamera) (- (Variables|Default|GetOriginalDistanceToObject) 1e+01)) (Transformation|GetWorldLocation _firstpersoncamera)))))))

(event Input|AxisEvents|InputAxisLookUp
  (params (AxisValue :type Float%20%28single-precision%29))
  (bind _firstpersoncamera (Variables|Default|GetFirstPersonCamera))
  (bind _analogueactor (Variables|Default|GetAnalogueActor))
  ;[1 1 1] Rotate object depending on mouse input
  (if (Utilities|IsValid _analogueactor)
    (Class|ComponentInterface|MouseValues(Message) _analogueactor (stale Input|AxisEvents|InputAxisTurn AxisValue) AxisValue)
    (else
      (Pawn|Input|AddControllerPitchInput AxisValue)
      (if (not (Variables|Default|GetInteractiveMode))
        (Physics|Components|PhysicsHandle|SetTargetLocation (Variables|Default|GetPhysicsHandle) (+ (* (Math|Vector|GetForwardVector _firstpersoncamera) (- (Variables|Default|GetOriginalDistanceToObject) 1e+01)) (Transformation|GetWorldLocation _firstpersoncamera)))))))

(event Input|MouseEvents|MouseWheelDown
  (params (Key :type Key%20Structure :default "None"))
  ;[1 1 1] Zoom
  (:Pressed
    (Variables|Rendering|SetIsZoomed false)))

(event Input|MouseEvents|MouseWheelUp
  (params (Key :type Key%20Structure :default "None"))
  ;[1 1 1] Zoom
  (:Pressed
    (Variables|Rendering|SetIsZoomed true)))

(fn ConstructionScript)

(fn Pause
  (bind _returnvalue (Game|GetPlayerController 0))
  (if (Game|IsGamePaused)
    (Game|SetGamePaused false)
    (bind _returnvalue_2 (UserInterface|CreateWidget "/Game/Blueprints/Source/Character/HUDWidget.HUDWidget_C" (Game|GetPlayerController 0)))
    (UserInterface|Viewport|AddtoViewport _returnvalue_2 0)
    (Variables|Default|SetHUDWidget _returnvalue_2)
    (else
      (Game|SetGamePaused true)
      (Widget|RemovefromParent (Variables|Default|GetHUDWidget))
      (bind _returnvalue_3 (UserInterface|CreateWidget "/Game/Blueprints/Source/LevelBlueprints/Widgets/PauseMenu.PauseMenu_C" _returnvalue))
      (UserInterface|Viewport|AddtoViewport _returnvalue_3 0)
      (Variables|/Script/Engine.PlayerController|SetbShowMouseCursor _returnvalue true)
      (Input|SetInputModeUIOnly _returnvalue _returnvalue_3 "DoNotLock"))))

(fn DoTrace
  (params (UseCursor :type Boolean))
  (bind _returnvalue (Game|GetPlayerController 0))
  (bind _firstpersoncamera (Variables|Default|GetFirstPersonCamera))
  (bind (_worldlocation _worlddirection) (Game|Player|ConvertMouseLocationToWorldSpace _returnvalue))
  (bind _returnvalue_2 (Transformation|GetWorldLocation _firstpersoncamera))
  (if UseCursor
    (bind (_outhit _returnvalue_3) (Collision|LineTraceByChannel _worldlocation (+ _worldlocation (* _worlddirection (Variables|Default|GetInteractionDistance))) "TraceTypeQuery1" true 0 "None"))
    (return _returnvalue_3 _outhit)
    (else
      (bind (_outhit_2 _returnvalue_4) (Collision|LineTraceByChannel _returnvalue_2 (+ _returnvalue_2 (* (Math|Vector|GetForwardVector _firstpersoncamera) (Variables|Default|GetInteractionDistance))) "TraceTypeQuery1" false 0 "None"))
      (return _returnvalue_4 _outhit_2))))

(fn PauseNotebook
  (bind _returnvalue (Game|GetPlayerController 0))
  (if (Game|IsGamePaused)
    (Game|SetGamePaused false)
    (Input|SetInputModeGameOnly _returnvalue)
    (Variables|/Script/Engine.PlayerController|SetbShowMouseCursor _returnvalue false)
    (else
      (Game|SetGamePaused true)
      (Variables|/Script/Engine.PlayerController|SetbShowMouseCursor _returnvalue true)
      (Input|SetInputModeGameandUI _returnvalue 0 "DoNotLock" true))))