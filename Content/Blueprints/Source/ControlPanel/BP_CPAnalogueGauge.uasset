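; Analogue gauge control panel component that displays a signal value with a sweeping needle.
; UpdatePassive divides the evaluated signal by the summed absolute start and end values, optionally inverts it, and clamps it to a 0–1 target.
; Tick eases toward that target and rotates the needle between yaw limits set at BeginPlay.
; The construction script selects the meter face through a dynamic material parameter driven by the decal index.
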(event EventBeginPlay
  (|CallParentFunction)
  (Variables|Instrument|SetStartRotator (Math|Rotator|MakeRotator 0.0 0.0 (Variables|Instrument|GetSweepStart)))
  (Variables|Instrument|SetGoalRotator (Math|Rotator|MakeRotator 0.0 0.0 (Variables|Instrument|GetSweepEnd))))

(event EventOnHover
  (params (CursorOver :type Boolean)))

(event EventTick
  (params (DeltaSeconds :type Float%20%28single-precision%29))
  (|CallParentFunction DeltaSeconds)
  (bind _output_get (Variables|Instrument|SetCurrent (Math|Interpolation|FInterpTo (Variables|Instrument|GetCurrent) (Variables|Instrument|GetTarget) DeltaSeconds (Variables|Instrument|GetSweepSpeed))))
  (Transformation|SetRelativeRotation (Variables|Default|GetNeedleOffset) (Math|Rotator|Lerp(Rotator) (Variables|Instrument|GetStartRotator) (Variables|Instrument|GetGoalRotator) _output_get) false false))

(event EventUpdatePassive
  (bind _probevalue (CallFunction|EvalSignal))
  (Variables|Instrument|SetTarget (Math|Float|Clamp(Float) (Math|Float|SelectFloat (- 1.0 (/ _probevalue (+ (Math|Float|Absolute(Float) (Variables|Instrument|GetValueStart)) (Math|Float|Absolute(Float) (Variables|Instrument|GetValueEnd))))) (/ _probevalue (+ (Math|Float|Absolute(Float) (Variables|Instrument|GetValueStart)) (Math|Float|Absolute(Float) (Variables|Instrument|GetValueEnd)))) (Variables|Instrument|GetInvertValue)))))

(fn ConstructionScript
  (bind _frame (Variables|Default|GetFrame))
  (|CallParentFunction)
  (bind _returnvalue (Rendering|Material|CreateDynamicMaterialInstance _frame 1 (Rendering|Material|GetMaterial _frame 1) "None" :!class /Script/Engine.PrimitiveComponent))
  (Rendering|Material|SetScalarParameterValue _returnvalue "Meter" (Math|Conversions|ToFloat(Integer) (Variables|Default|GetDecalIndex)) :!class /Script/Engine.MaterialInstanceDynamic))