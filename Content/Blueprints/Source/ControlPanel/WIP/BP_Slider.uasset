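; BP_Slider is a physics-driven three-position slider for a control panel, with two indicator lights.
; Each tick it compares the slider's world Y offset from its BeginPlay position against a threshold either side of center.
; Crossing a threshold toggles that side's point light and sets the physics constraint's linear target toward that end.
; While the slider stays within the center band, the target returns to zero, creating a detent effect.
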(event EventTick
  (params (DeltaSeconds :type Float%20%28single-precision%29))
  (bind _startvalue (Variables|Default|GetStartValue))
  (bind _slider (Variables|Default|GetSlider))
  (bind _returnvalue (Transformation|GetWorldLocation _slider))
  (bind _returnvalue_2 (- (.y _returnvalue) _startvalue))
  (bind _returnvalue_3 (< _returnvalue_2 1e+01))
  (bind _returnvalue_4 (> _returnvalue_2 -1e+01))
  (Utilities|FlowControl|Sequence
    (:then_0
      (if (Math|Boolean|NotEqual(Boolean) (Variables|Default|GetOn) _returnvalue_3)
        (Variables|Default|SetOn _returnvalue_3)
        (Rendering|ToggleVisibility (Variables|Default|GetPointLight) false)
        (Class|PhysicsConstraintComponent|SetLinearPositionTarget (Variables|Default|GetPhysicsConstraint) (Math|Vector|MakeVector 0.0 22.0 0.0))
        (else
          (if (Math|Boolean|Equal(Boolean) _returnvalue_3 _returnvalue_4) :!label _label
            (Class|PhysicsConstraintComponent|SetLinearPositionTarget (Variables|Default|GetPhysicsConstraint) (Math|Vector|MakeVector 0.0 0.0 0.0))))))
    (:then_1
      (if (Math|Boolean|NotEqual(Boolean) _returnvalue_4 (Variables|Default|GetOn2))
        (Variables|Default|SetOn2 _returnvalue_4)
        (Rendering|ToggleVisibility (Variables|Default|GetPointLight1) false)
        (Class|PhysicsConstraintComponent|SetLinearPositionTarget (Variables|Default|GetPhysicsConstraint) (Math|Vector|MakeVector 0.0 -22.0 0.0))
        (else
          (goto _label))))))

(event EventBeginPlay
  (Variables|Default|SetStartValue (.y (Transformation|GetWorldLocation (Variables|Default|GetSlider)))))

(fn ConstructionScript)