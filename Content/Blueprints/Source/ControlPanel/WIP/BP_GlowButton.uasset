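; BP_GlowButton is a work-in-progress control panel toggle button with a point light that shows its on/off state.
; On BeginPlay the light's visibility is set from the stored state.
; OnInteract flips that state, sends it with a signal to a component through BPI_MCPDelegates' OnButtonPressed, then updates the light.
; If the component fails the interface cast, the interaction does nothing.
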(event EventBeginPlay
  (|CallParentFunction)
  (Rendering|SetVisibility (Variables|Default|GetPointLight) (Variables|Default|GetState_0) false))

(event Collision|EventActorBeginOverlap
  (params (OtherActor :type Actor%20Object%20Reference))
  (|CallParentFunction OtherActor) ; This node is disabled and will not be called.\nDrag off pins to build functionality.
)

(event EventTick
  (params (DeltaSeconds :type Float%20%28single-precision%29))
  (|CallParentFunction DeltaSeconds) ; This node is disabled and will not be called.\nDrag off pins to build functionality.
)

(event EventOnInteract
  (params (Caller :type Actor%20Object%20Reference))
  (bind _asbpi_mcpdelegates (Utilities|Casting|CastToBPI_MCPDelegates (Variables|Default|GetComponent)))
  (bind _output_get (Variables|Default|SetState_0 (not (Variables|Default|GetState_0))))
  (Default|OnButtonPressed _asbpi_mcpdelegates _output_get (Variables|Default|GetActive))
  (Rendering|SetVisibility (Variables|Default|GetPointLight) _output_get false))

(fn ConstructionScript
  (|CallParentFunction))