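; BP_LeverDiscrete is a work-in-progress control panel lever that steps between discrete notches.
; AxisValuesEvent moves it up one notch for positive Z, otherwise down, within NotchMin and NotchMax, ignoring movement while animating.
; A timeline per direction pitches HandleOffset by AngleDifference from CurrentAngle, then stores the new angle and resets.
; Notch states -1, 0 and 1 only print debug strings.
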(event EventBeginPlay
  ;[1 1 1] if no work, member handle offset
  (Transformation|SetRelativeRotation (Variables|Default|GetHandleOffset) (Math|Rotator|MakeRotator 0.0 (Variables|Default|GetStartingAngle) 0.0) false false)
  (Variables|Default|SetCurrentAngle (Variables|Default|GetStartingAngle)))

(event EventAxisValuesEvent
  (params (Values :type Vector :default "0, 0, 0"))
  ;[1 1 1] if no work, member handle offset
  (Utilities|FlowControl|Sequence
    (:then_0
      (if (not (Variables|Default|GetAnimationPlaying))
        (if (> (.z Values) 0.0)
          (if (not (== (Variables|Default|GetCurrentNotch) (Variables|Default|GetNotchMax)))
            (Variables|Default|SetAnimationPlaying true)
            (Variables|Default|SetCurrentNotch (+ (Variables|Default|GetCurrentNotch) 1))
            (Development|PrintString "up")
            (bind _lever_angle_value (Timeline|LeverAnimation2 Play)
              (:Update
                (Transformation|SetRelativeRotation (Variables|Default|GetHandleOffset) (Math|Rotator|MakeRotator 0.0 (+ (Variables|Default|GetCurrentAngle) (* _lever_angle_value (Variables|Default|GetAngleDifference))) 0.0) false false))
              (:Finished
                (bind _output_get (Variables|Default|SetCurrentAngle (+ (Variables|Default|GetCurrentAngle) (* _lever_angle_value (Variables|Default|GetAngleDifference)))))
                (Development|PrintString (Utilities|String|ToString(Float) _output_get))
                (Variables|Default|SetAnimationPlaying false)
                (Timeline|LeverAnimation2 SetNewTime))))
          (elif (not (== (Variables|Default|GetCurrentNotch) (Variables|Default|GetNotchMin)))
            (Variables|Default|SetAnimationPlaying true)
            (Variables|Default|SetCurrentNotch (- (Variables|Default|GetCurrentNotch) 1))
            (Development|PrintString "down")
            (bind _lever_angle_value_2 (Timeline|LeverAnimation Play)
              (:Update
                (Transformation|SetRelativeRotation (Variables|Default|GetHandleOffset) (Math|Rotator|MakeRotator 0.0 (- (Variables|Default|GetCurrentAngle) (* (Variables|Default|GetAngleDifference) _lever_angle_value_2)) 0.0) false false))
              (:Finished
                (bind _output_get_2 (Variables|Default|SetCurrentAngle (- (Variables|Default|GetCurrentAngle) (* (Variables|Default|GetAngleDifference) _lever_angle_value_2))))
                (Development|PrintString (Utilities|String|ToString(Float) _output_get_2))
                (Variables|Default|SetAnimationPlaying false)
                (Timeline|LeverAnimation SetNewTime)))))))
    (:then_1
      (switch int (Variables|Default|GetCurrentNotch)
        (:-1
          (Development|PrintString "Notch -1"))
        (:0
          (Development|PrintString "Notch 0"))
        (:1
          (Development|PrintString "Notch 1"))))))

(fn ConstructionScript)