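; Base Blueprint for control panel indicator lights that switch an emissive material with the alert state.
; Construction passes colors and blink settings to the material; passive updates evaluate the signal, and state changes set the light and notify ExtraLights.
; Linked lights count enable requests, staying lit while any remain, and forward them down the chain.
; SmoothBlink provides a matching clamped-cosine pulse, and an empty hover override suppresses the outline.
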(event Custom|OnStateChanged
  (params (AlertState :type Boolean) (SignalValue :type Float%20%28single-precision%29))
  (CallFunction|SetLightState AlertState)
  (for _array_element (Variables|Instrument|GetExtraLights)
    (CallFunction|RequestLightEnabled _array_element AlertState)))

(event EventBeginPlay
  (|CallParentFunction)
  (EventDispatchers|BindEventtoOnStateChange (delegate Custom|OnStateChanged))
  (Default|CallOnStateChange (Variables|Default|GetAlertState) 0.0))

(event EventUpdatePassive
  (CallFunction|EvalSignal))

(event EventOnHover
  (params (CursorOver :type Boolean)))

(fn ConstructionScript
  (bind _emissivematerial (Variables|Rendering|GetEmissiveMaterial))
  (|CallParentFunction)
  (Rendering|Material|SetVectorParameterValue _emissivematerial "OnColor" (Variables|Instrument|GetOnColor) :!class /Script/Engine.MaterialInstanceDynamic)
  (Rendering|Material|SetVectorParameterValue _emissivematerial "OffColor" (Variables|Instrument|GetOffColor) :!class /Script/Engine.MaterialInstanceDynamic)
  (Rendering|Material|SetScalarParameterValue _emissivematerial "BlinkFrequency" (Variables|Instrument|GetBlinkRate) :!class /Script/Engine.MaterialInstanceDynamic)
  (Rendering|Material|SetScalarParameterValue _emissivematerial "BlinkOffset" (Variables|Instrument|GetBlinkOffset) :!class /Script/Engine.MaterialInstanceDynamic))

(fn SetLightState
  (params (Enabled :type Boolean))
  (bind _emissivematerial (Variables|Rendering|GetEmissiveMaterial))
  (bind _output_get (Variables|Instrument|SetIsLit Enabled))
  (Utilities|FlowControl|Sequence
    (:then_0
      (Utilities|IsValid _emissivematerial
        (:Is%20Valid
          (Rendering|Material|SetScalarParameterValue _emissivematerial "Active" (Math|Conversions|ToFloat(Boolean) _output_get) :!class /Script/Engine.MaterialInstanceDynamic))))))

(fn RequestLightEnabled
  (params (Enabled :type Boolean))
  (Utilities|FlowControl|Sequence
    (:then_0
      (bind _output_get (Variables|Instrument|SetRequestCount (Math|Integer|Max(Integer) (+ (Math|Integer|SelectInt 1 -1 Enabled) (Variables|Instrument|GetRequestCount)))))
      (CallFunction|SetLightState (> _output_get 0)))
    (:then_1
      (for _array_element (Variables|Instrument|GetExtraLights)
        (CallFunction|RequestLightEnabled _array_element Enabled)))))

(fn SmoothBlink
  (return (Math|Float|Clamp(Float) (Math|Trig|Cos(Radians) (* (+ (* (Utilities|Time|GetGameTimeinSeconds) (Variables|Instrument|GetBlinkRate)) (Variables|Instrument|GetBlinkOffset)) (Math|Trig|GetPI) 2.0)))))