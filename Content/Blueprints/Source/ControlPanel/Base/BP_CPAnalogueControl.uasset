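; Base control-panel Blueprint for analogue controls that turn mouse movement into a clamped value while the player interacts.
; Mouse deltas on the chosen axis, scaled by friction and range, update CurrentValue, which is reported to a component.
; A normalised value drives SetControlPosition, an empty hook presumably overridden by children, and triggers click sounds at step changes.
; With AutoReset enabled, ending interaction plays a timeline that eases the value back to ZeroValue.
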(event EventBeginPlay
  (|CallParentFunction)
  (bind _output_get (Variables|Instrument|SetCurrentValue (Math|Float|Clamp(Float) (Variables|Instrument|GetCurrentValue) (Variables|Instrument|GetMinValue) (Variables|Instrument|GetMaxValue))))
  (Class|BPIMCPDelegates|OnAnalogueChanged(Message) (Variables|Default|GetComponent) _output_get (Variables|Default|GetActive))
  (bind _value (CallFunction|GetAnalogueValue (Variables|Instrument|GetInvertValue)))
  (CallFunction|SetControlPosition _value))

(event EventMouseValues
  (params (Mouse%20X :type Float%20%28single-precision%29) (Mouse%20Y :type Float%20%28single-precision%29))
  (bind _usehorizontal (Variables|Instrument|GetUseHorizontal))
  (bind _returnvalue (Math|Float|SelectFloat Mouse%20X Mouse%20Y _usehorizontal))
  (if (Audio|Components|Audio|IsPlaying (Variables|Default|GetResetTimeline))
    (bind _releasedtrack (Timeline|ResetTimeline Stop)
      (:Update
        (bind _output_get (Variables|Instrument|SetCurrentValue (Math|Float|Lerp (Variables|Instrument|GetCurrentValue) (Variables|Instrument|GetZeroValue) _releasedtrack)))
        (Class|BPIMCPDelegates|OnAnalogueChanged(Message) (Variables|Default|GetComponent) _output_get (Variables|Default|GetActive))
        (bind _value (CallFunction|GetAnalogueValue (Variables|Instrument|GetInvertValue)))
        (CallFunction|SetControlPosition _value)))
    (else
      (bind _output_get_2 (Variables|Instrument|SetCurrentValue (Math|Float|Clamp(Float) (+ (* (/ (Math|Float|SelectFloat (* -1 _returnvalue) _returnvalue (Class|KismetMathLibrary|XORBoolean (Variables|Instrument|GetInvertAxis) (not _usehorizontal))) (Variables|Instrument|GetFriction)) (Math|Float|Absolute(Float) (- (Variables|Instrument|GetMaxValue) (Variables|Instrument|GetMinValue)))) (Variables|Instrument|GetCurrentValue)) (Variables|Instrument|GetMinValue) (Variables|Instrument|GetMaxValue))))
      (Class|BPIMCPDelegates|OnAnalogueChanged(Message) (Variables|Default|GetComponent) _output_get_2 (Variables|Default|GetActive))
      (bind _value_2 (CallFunction|GetAnalogueValue (Variables|Instrument|GetInvertValue)))
      (CallFunction|SetControlPosition _value_2)
      (if (not (== (Math|Float|Round (* (Variables|Instrument|GetClickSteps) _value_2)) (Variables|Instrument|GetLastClick)))
        (Variables|Instrument|SetLastClick (Math|Float|Round (* (Variables|Instrument|GetClickSteps) _value_2)))
        (Class|FMODBlueprintStatics|PlayEventAttached (Variables|Instrument|GetClickSound) (Variables|Default|GetSceneRoot) "None" "0, 0, 0" "KeepRelativeOffset")))))

(event EventOnEndInteract
  (if (Variables|Instrument|GetAutoReset)
    (bind _releasedtrack (Timeline|ResetTimeline PlayFromStart)
      (:Update
        (bind _output_get (Variables|Instrument|SetCurrentValue (Math|Float|Lerp (Variables|Instrument|GetCurrentValue) (Variables|Instrument|GetZeroValue) _releasedtrack)))
        (Class|BPIMCPDelegates|OnAnalogueChanged(Message) (Variables|Default|GetComponent) _output_get (Variables|Default|GetActive))
        (bind _value (CallFunction|GetAnalogueValue (Variables|Instrument|GetInvertValue)))
        (CallFunction|SetControlPosition _value)))))

(fn ConstructionScript
  (|CallParentFunction))

(fn SetControlPosition
  (params (Position :type Float%20%28single-precision%29)))

(fn GetAnalogueValue
  (params (Invert :type Boolean))
  (bind _currentvalue (Variables|Instrument|GetCurrentValue))
  (bind _maxvalue (Variables|Instrument|GetMaxValue))
  (bind _minvalue (Variables|Instrument|GetMinValue))
  (bind _returnvalue (Math|Float|Absolute(Float) _maxvalue))
  (bind _returnvalue_2 (Math|Float|Absolute(Float) _minvalue))
  (bind _returnvalue_3 (+ _returnvalue_2 _returnvalue))
  (bind _returnvalue_4 (+ _currentvalue _returnvalue_2))
  (bind _returnvalue_5 (/ _returnvalue_4 _returnvalue_3))
  (if Invert
    (return (- (Variables|Instrument|GetMaxValue) _returnvalue_5))
    (else
      (return _returnvalue_5))))