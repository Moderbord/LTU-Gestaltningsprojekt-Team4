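; Base Blueprint for a control-panel control that steps between integer values within a clamped range.
; Axis input moves the value one step along the chosen axis, with optional inversion, and is ignored while the movement timeline plays.
; The timeline drives SetControlPosition, an empty hook presumably overridden by children, then notifies the component when finished.
; BeginPlay applies and broadcasts the initial value, and GetDiscreteValue returns an offset, optionally inverted value.
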(event EventBeginPlay
  (|CallParentFunction)
  (bind _output_get (Variables|Instrument|SetCurrentValue (Math|Integer|Clamp(Integer) (Variables|Instrument|GetCurrentValue) (Variables|Instrument|GetMinValue) (Variables|Instrument|GetMaxValue))))
  (Class|BPIMCPDelegates|OnDiscreteChanged(Message) (Variables|Default|GetComponent) _output_get (Variables|Default|GetActive))
  (CallFunction|SetControlPosition 0 (Variables|Instrument|GetCurrentValue) 1.0))

(event EventAxisValuesEvent
  (params (Values :type Vector :default "0, 0, 0"))
  (bind _usehorizontal (Variables|Instrument|GetUseHorizontal))
  (bind _returnvalue (Math|Float|SelectFloat (.y Values) (.x Values) _usehorizontal))
  (bind _returnvalue_2 (Math|Float|Sign(Float) _returnvalue))
  (bind _returnvalue_3 (Math|Float|Truncate _returnvalue_2))
  (if (not (Variables|Instrument|GetAnimationPlaying))
    (bind _output_get (Variables|Instrument|SetPreviousValue (Variables|Instrument|GetCurrentValue)))
    (bind _output_get_2 (Variables|Instrument|SetCurrentValue (Math|Integer|Clamp(Integer) (+ (Variables|Instrument|GetCurrentValue) (Math|Integer|SelectInt _returnvalue_3 (* _returnvalue_3 -1) (Class|KismetMathLibrary|XORBoolean (Variables|Instrument|GetInvertAxis) (not _usehorizontal)))) (Variables|Instrument|GetMinValue) (Variables|Instrument|GetMaxValue))))
    (if (!= _output_get _output_get_2)
      (Variables|Instrument|SetAnimationPlaying true)
      (Components|Timeline|SetPlayRate (Variables|Default|GetDiscreteMovement) (Variables|Instrument|GetAnimationSpeed))
      (bind _discretemovement (Timeline|DiscreteMovement PlayFromStart)
        (:Update
          (CallFunction|SetControlPosition (Variables|Instrument|GetPreviousValue) (Variables|Instrument|GetCurrentValue) _discretemovement))
        (:Finished
          (Class|BPIMCPDelegates|OnDiscreteChanged(Message) (Variables|Default|GetComponent) _output_get_2 (Variables|Default|GetActive))
          (Variables|Instrument|SetAnimationPlaying false))))))

(fn ConstructionScript
  (|CallParentFunction))

(fn GetDiscreteValue
  (params (Invert :type Boolean))
  (bind _minvalue (Variables|Instrument|GetMinValue))
  (bind _currentvalue (Variables|Instrument|GetCurrentValue))
  (bind _returnvalue (Math|Integer|Absolute(Integer) _minvalue))
  (bind _returnvalue_2 (+ _currentvalue _returnvalue))
  (return (Math|Integer|SelectInt (- (Variables|Instrument|GetMaxValue) _returnvalue_2) _returnvalue_2 Invert)))

(fn SetControlPosition
  (params (From :type Integer) (To :type Integer) (Alpha :type Float%20%28single-precision%29)))