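; Base Blueprint for control panel elements that monitor a signal, with a configurable text label and a hover outline.
; EvalSignal probes its component, flips the alert state on crossing a threshold (optionally reversed), and broadcasts changes locally and optionally through BP_EventController.
; Chaos contributors also report to the controller's chaos map, scaling their chaos pool between alert thresholds while alerting and reporting zero otherwise.
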(event EventBeginPlay
  (bind _returnvalue (Actor|GetActorOfClass "/Game/Blueprints/Source/EventController/BP_EventController.BP_EventController_C"))
  (Variables|Signaling|SetEventController _returnvalue))

(event EventOnHover
  (params (CursorOver :type Boolean))
  (CallFunction|SetOutline self CursorOver "NewEnumerator0"))

(fn ConstructionScript
  (bind _label (Variables|Default|GetLabel))
  (Rendering|Components|TextRender|SetText _label (Variables|Default|GetLabelText))
  (Rendering|Components|TextRender|SetWorldSize _label (Variables|Default|GetLabelSize)))

(fn GetComponentChaos
  (params (Current :type Float%20%28single-precision%29))
  (if (Math|Float|NearlyEqual(Float) (Variables|Events|GetAlertMaxThreshold) (Variables|Events|GetAlertMinThreshold) 0.01)
    (return (Variables|Events|GetChaosPool))
    (else
      (bind _out (Events|ChaosPoolWeight Current))
      (return _out))))

(fn ChaosPoolWeight
  (params (Amount :type Float%20%28single-precision%29))
  (return (* (Math|Float|Clamp(Float) (/ (Math|Float|Absolute(Float) (- Amount (Variables|Events|GetAlertMinThreshold))) (Math|Float|Absolute(Float) (- (Variables|Events|GetAlertMaxThreshold) (Variables|Events|GetAlertMinThreshold))))) (Variables|Events|GetChaosPool))))

(fn EvalSignal
  (bind _alertstate (Variables|Events|GetAlertState))
  (bind _value (Default|Probe (Variables|Signaling|GetComponent) (Variables|Signaling|GetPassive)))
  (LocalVariables|SetSignalValue _value)
  (Utilities|FlowControl|Sequence
    (:then_0
      (if (Variables|Events|GetMonitorState)
        (if (Variables|Events|GetReverseThresholdCheck)
          (Events|EvalAlertState (< (LocalVariables|GetSignalValue) (Variables|Events|GetAlertMinThreshold)) _alertstate (LocalVariables|GetSignalValue))
          (else
            (Events|EvalAlertState (> (LocalVariables|GetSignalValue) (Variables|Events|GetAlertMinThreshold)) _alertstate (LocalVariables|GetSignalValue))))))
    (:then_1
      (if (Variables|Events|GetChaosContributor)
        (Events|EvalChaos (LocalVariables|GetSignalValue))))))

(fn EvalChaos
  (params (SignalValue :type Float%20%28single-precision%29))
  (bind _self self)
  (bind _eventcontroller (Variables|Signaling|GetEventController))
  (if (Variables|Events|GetAlertState)
    (bind _out (Events|GetComponentChaos SignalValue))
    (Default|AddtoChaosMap _eventcontroller _self _out)
    (else
      (Default|AddtoChaosMap _eventcontroller _self 0.0))))

(fn EvalAlertState
  (params (ShouldAlert :type Boolean) (IsAlerting :type Boolean) (SignalValue :type Float%20%28single-precision%29))
  (if (Math|Boolean|NotEqual(Boolean) ShouldAlert IsAlerting)
    (bind _output_get (Variables|Events|SetAlertState (not (Variables|Events|GetAlertState))))
    (Default|CallOnStateChange _output_get SignalValue)
    (if (Variables|Events|GetEventContributor)
      (Default|CallOnCPAlertStateChange (Variables|Signaling|GetEventController) (Variables|Signaling|GetPassive) (Variables|Events|GetAlertState)))))