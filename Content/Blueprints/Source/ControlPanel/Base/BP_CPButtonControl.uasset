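; Base control panel button that animates on interaction and reports its state through a component message, with optional inversion.
; BeginPlay broadcasts the initial state and sets the control position.
; Interaction flips Pressed and plays or reverses a timeline that drives SetControlPosition, an empty hook presumably left for child Blueprints.
; When the timeline finishes it sends the state, and non-toggle buttons reverse the animation.
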(event EventOnInteract
  (params (Caller :type Actor%20Object%20Reference))
  (if (not (Variables|Instrument|GetAnimationPlaying))
    (Components|Timeline|SetPlayRate (Variables|Default|GetButtonAnim) (Variables|Instrument|GetAnimationSpeed))
    (bind _output_get (Variables|Instrument|SetPressed (not (Variables|Instrument|GetPressed))))
    (if _output_get
      (bind _buttonanimtrack (Timeline|ButtonAnim PlayFromStart)
        (:Update
          (CallFunction|SetControlPosition _output_get _buttonanimtrack))
        (:Finished
          (Class|BPIMCPDelegates|OnButtonPressed(Message) (Variables|Default|GetComponent) (Class|KismetMathLibrary|XORBoolean (Variables|Instrument|GetPressed) (Variables|Instrument|GetInvertValue)) (Variables|Default|GetActive))
          (if (Variables|Instrument|GetIsToggle)
            (Variables|Instrument|SetAnimationPlaying false)
            (else
              (Timeline|ButtonAnim Reverse)))))
      (else
        (Timeline|ButtonAnim ReverseFromEnd)))))

(event EventBeginPlay
  (bind _pressed (Variables|Instrument|GetPressed))
  (Class|BPIMCPDelegates|OnButtonPressed(Message) (Variables|Default|GetComponent) (Class|KismetMathLibrary|XORBoolean (Variables|Instrument|GetInvertValue) _pressed) (Variables|Default|GetActive))
  (CallFunction|SetControlPosition _pressed 1.0))

(fn ConstructionScript
  (|CallParentFunction))

(fn SetControlPosition
  (params (NewState :type Boolean) (Alpha :type Float%20%28single-precision%29)))