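; BP_Button2 is an interactable control panel button that toggles a Pressed state and rocks between two roll angles.
; Interact flips the state and plays or reverses ButtonTimeline, which lerps the rotation of ButtonOffset.
; When the timeline finishes, it sends the Pressed and Active values to Component through OnButtonPressedMessage.
; BeginPlay sends the same message and snaps the button to match its starting state.
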(event EventBeginPlay
  (bind _pressed (Variables|Default|GetPressed))
  (Class|BPIMCPDelegates|OnButtonPressed(Message) (Variables|Default|GetComponent) _pressed (Variables|Default|GetActive))
  (Transformation|SetRelativeRotation (Variables|Default|GetButtonOffset) (Math|Rotator|MakeRotator (Math|Float|SelectFloat 2e+01 -3e+01 _pressed) 0.0 0.0) false false))

(event EventInteract
  (params (Caller :type Actor%20Object%20Reference))
  (if (Variables|Default|GetPressed)
    (Variables|Default|SetPressed false)
    (bind _location_value (Timeline|ButtonTimeline Reverse)
      (:Update
        (Transformation|SetRelativeRotation (Variables|Default|GetButtonOffset) (Math|Rotator|MakeRotator (Math|Float|Lerp -3e+01 2e+01 _location_value) 0.0 0.0) false false))
      (:Finished
        (Class|BPIMCPDelegates|OnButtonPressed(Message) (Variables|Default|GetComponent) (Variables|Default|GetPressed) (Variables|Default|GetActive))))
    (else
      (Variables|Default|SetPressed true)
      (Timeline|ButtonTimeline Play))))

(fn ConstructionScript)