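; Analogue gauge actor for a control panel that swings an arrow to show a value probed from its Component.
; BeginPlay builds start and goal rotators from the sweep's start and end yaw.
; Each Tick reads a passive probe as the target and calls EvalSignal.
; It then eases the current value toward that target, caps it at one, and uses it to lerp the arrow's relative rotation.
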(event EventBeginPlay
  (|CallParentFunction)
  (Variables|Default|SetStartRotator (Math|Rotator|MakeRotator 0.0 0.0 (Variables|Default|GetSweepStart)))
  (Variables|Default|SetGoalRotator (Math|Rotator|MakeRotator 0.0 0.0 (Variables|Default|GetSweepEnd))))

(event Collision|EventActorBeginOverlap
  (params (OtherActor :type Actor%20Object%20Reference))
  (|CallParentFunction OtherActor) ; This node is disabled and will not be called.\nDrag off pins to build functionality.
)

(event EventTick
  (params (DeltaSeconds :type Float%20%28single-precision%29))
  (|CallParentFunction DeltaSeconds)
  (Utilities|FlowControl|Sequence
    (:then_0
      (bind _value (Default|Probe (Variables|Default|GetComponent) (Variables|Default|GetPassive)))
      (Variables|Default|SetTarget _value)
      (CallFunction|EvalSignal))
    (:then_1
      (bind _output_get (Variables|Default|SetCurrent (Math|Float|Min(Float) (Math|Interpolation|FInterpTo (Variables|Default|GetCurrent) (Variables|Default|GetTarget) DeltaSeconds (Variables|Default|GetInterpSpeed)) 1.0)))
      (Transformation|SetRelativeRotation (Variables|Default|GetArrow) (Math|Rotator|Lerp(Rotator) (Variables|Default|GetStartRotator) (Variables|Default|GetGoalRotator) _output_get) false false))))

(fn ConstructionScript
  (|CallParentFunction))