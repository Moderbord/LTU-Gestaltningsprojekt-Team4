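; BP_CPSwitch is a control panel routing node that reduces the values of several components to their minimum or maximum, depending on its Mode.
; Probe forwards a key to each component's ProbeMessage, seeds the result from the first reply, then keeps the smaller or larger value.
; The text render shows the mode name at construction and switches to the selected value on each probe, which is also returned.
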(fn ConstructionScript
  (Rendering|Components|TextRender|SetText (Variables|Default|GetTextRender) (Utilities|Text|ToText(String) (Utilities|String|EnumtoString (Variables|Default|GetMode)))))

(fn Probe
  (params (Key :type Signal%20Key%20Structure))
  (for (_array_element _array_index) (Variables|Default|GetComponents)
    (bind _value (Class|BPIProbable|Probe(Message) _array_element Key))
    (if (== _array_index 0)
      (LocalVariables|SetMaxVal _value)
      (else
        (switch Utilities|FlowControl|Switch|SwitchonESwitchModes (Variables|Default|GetMode)
          (:NewEnumerator0
            (if (< _value (LocalVariables|GetMaxVal))
              (LocalVariables|SetMaxVal _value :!label _label)))
          (:NewEnumerator1
            (if (> _value (LocalVariables|GetMaxVal))
              (goto _label)))))))
  (Rendering|Components|TextRender|SetText (Variables|Default|GetTextRender) (Utilities|Text|ToText(Float) (LocalVariables|GetMaxVal) "HalfToEven"))
  (return (LocalVariables|GetMaxVal)))