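; Physics-driven three-position lever for a control panel, with an indicator light for each of its two thresholds.
; Tick reads the Handle's pitch relative to the actor, toggling the matching light whenever it crosses either threshold.
; The PhysicsConstraint's angular target acts as a detent, switching to a tilted position on crossings and back to center while the handle sits in the middle band.
; A separate axis-values event only prints its input.
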(event EventAxisValuesEvent
  (params (Values :type Vector :default "0, 0, 0"))
  (Development|PrintString (Utilities|String|ToString(Vector) Values)))

(event EventTick
  (params (DeltaSeconds :type Float%20%28single-precision%29))
  (bind _returnvalue (Transformation|GetActorTransform))
  (bind _handle (Variables|Default|GetHandle))
  (bind _returnvalue_2 (Transformation|GetWorldRotation _handle))
  (bind _returnvalue_3 (Math|Transform|InverseTransformRotation _returnvalue _returnvalue_2))
  (bind _pitch (Math|Rotator|BreakRotator _returnvalue_3))
  (bind _returnvalue_4 (< _pitch 2e+01))
  (bind _returnvalue_5 (> _pitch -2e+01))
  (Utilities|FlowControl|Sequence
    (:then_0
      (if (Math|Boolean|NotEqual(Boolean) (Variables|Default|GetOn) _returnvalue_4)
        (Variables|Default|SetOn _returnvalue_4)
        (Rendering|ToggleVisibility (Variables|Default|GetPointLight) false)
        (Class|PhysicsConstraintComponent|SetAngularOrientationTarget (Variables|Default|GetPhysicsConstraint) (Math|Rotator|MakeRotator 0.0 45.0 0.0))
        (else
          (if (Math|Boolean|Equal(Boolean) _returnvalue_4 _returnvalue_5) :!label _label
            (Class|PhysicsConstraintComponent|SetAngularOrientationTarget (Variables|Default|GetPhysicsConstraint) (Math|Rotator|MakeRotator 0.0 0.0 0.0))))))
    (:then_1
      (if (Math|Boolean|NotEqual(Boolean) _returnvalue_5 (Variables|Default|GetOn2))
        (Variables|Default|SetOn2 _returnvalue_5)
        (Rendering|ToggleVisibility (Variables|Default|GetPointLight1) false)
        (Class|PhysicsConstraintComponent|SetAngularOrientationTarget (Variables|Default|GetPhysicsConstraint) (Math|Rotator|MakeRotator 0.0 -45.0 0.0))
        (else
          (goto _label))))))

(fn ConstructionScript)