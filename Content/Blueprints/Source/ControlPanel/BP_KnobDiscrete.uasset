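; BP_KnobDiscrete is a control-panel knob that rotates between discrete notches in response to axis input.
; Y input's sign picks one of two timelines that step the yaw by AngleDifference, ignoring movement while animating or past the notch limits.
; CurrentNotch updates when the animation finishes.
; A zero-based value goes to Component at BeginPlay, and inverted on each axis event, without waiting for the animation.
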(event EventBeginPlay
  (Transformation|SetRelativeRotation (Variables|Default|GetBaseOffset) (Math|Rotator|MakeRotator 0.0 0.0 (Variables|Default|GetStartAngle)) false false)
  (Variables|Default|SetCurrentAngle (Variables|Default|GetStartAngle))
  (bind _returnvalue (CallFunction|GetDiscreteValue false))
  (Class|BPIMCPDelegates|OnDiscreteChanged(Message) (Variables|Default|GetComponent) _returnvalue (Variables|Default|GetActive)))

(event EventAxisValuesEvent
  (params (Values :type Vector :default "0, 0, 0"))
  (bind _baseoffset (Variables|Default|GetBaseOffset))
  (Utilities|FlowControl|Sequence
    (:then_0
      (if (not (Variables|Default|GetAnimationPlaying))
        (if (> (.y Values) 0.0)
          (if (not (== (Variables|Default|GetCurrentNotch) (Variables|Default|GetNotchMin)))
            (Variables|Default|SetAnimationPlaying true)
            (bind _wheelrotationfloat (Timeline|WheelAnimation2 Play)
              (:Update
                (Transformation|SetRelativeRotation _baseoffset (Math|Rotator|MakeRotator 0.0 0.0 (- (Variables|Default|GetCurrentAngle) (* _wheelrotationfloat (Variables|Default|GetAngleDifference)))) false false))
              (:Finished
                (Variables|Default|SetCurrentAngle (- (Variables|Default|GetCurrentAngle) (* _wheelrotationfloat (Variables|Default|GetAngleDifference))))
                (Variables|Default|SetAnimationPlaying false)
                (Variables|Default|SetCurrentNotch (- (Variables|Default|GetCurrentNotch) 1))
                (Timeline|WheelAnimation2 SetNewTime))))
          (elif (not (== (Variables|Default|GetCurrentNotch) (Variables|Default|GetNotchMax)))
            (Variables|Default|SetAnimationPlaying true)
            (bind _wheelrotationfloat_2 (Timeline|WheelAnimation Play)
              (:Update
                (Transformation|SetRelativeRotation _baseoffset (Math|Rotator|MakeRotator 0.0 0.0 (+ (Variables|Default|GetCurrentAngle) (* _wheelrotationfloat_2 (Variables|Default|GetAngleDifference)))) false false))
              (:Finished
                (Variables|Default|SetCurrentAngle (+ (Variables|Default|GetCurrentAngle) (* _wheelrotationfloat_2 (Variables|Default|GetAngleDifference))))
                (Variables|Default|SetAnimationPlaying false)
                (Variables|Default|SetCurrentNotch (+ (Variables|Default|GetCurrentNotch) 1))
                (Timeline|WheelAnimation SetNewTime)))))))
    (:then_1
      (bind _returnvalue (CallFunction|GetDiscreteValue true))
      (Class|BPIMCPDelegates|OnDiscreteChanged(Message) (Variables|Default|GetComponent) _returnvalue (Variables|Default|GetActive)))))

(fn ConstructionScript)

(fn GetDiscreteValue
  (params (Invert :type Boolean))
  (bind _currentnotch (Variables|Default|GetCurrentNotch))
  (bind _notchmin (Variables|Default|GetNotchMin))
  (bind _returnvalue (Math|Integer|Absolute(Integer) _notchmin))
  (bind _returnvalue_2 (+ _currentnotch _returnvalue))
  (return (Math|Integer|SelectInt (- (Variables|Default|GetNotchMax) _returnvalue_2) _returnvalue_2 Invert)))