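; BP_WheelFree is a control panel wheel actor that switches two point lights according to the rotation of its Base component.
; Each tick it reads the yaw of Base in actor space and compares it against symmetric thresholds either side of zero.
; Each threshold has a cached boolean, so its light's visibility toggles only when the yaw crosses that limit.
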(event EventTick
  (params (DeltaSeconds :type Float%20%28single-precision%29))
  (bind _returnvalue (Transformation|GetActorTransform))
  (bind _base (Variables|Default|GetBase))
  (bind _returnvalue_2 (Transformation|GetWorldRotation _base))
  (bind _returnvalue_3 (Math|Transform|InverseTransformRotation _returnvalue _returnvalue_2))
  (bind _yaw (Math|Rotator|BreakRotator _returnvalue_3))
  (bind _returnvalue_4 (< _yaw 2e+01))
  (bind _returnvalue_5 (> _yaw -2e+01))
  (Utilities|FlowControl|Sequence
    (:then_0
      (if (Math|Boolean|NotEqual(Boolean) (Variables|Default|GetOn) _returnvalue_4)
        (Variables|Default|SetOn _returnvalue_4)
        (Rendering|ToggleVisibility (Variables|Default|GetPointLight) false)))
    (:then_1
      (if (Math|Boolean|NotEqual(Boolean) _returnvalue_5 (Variables|Default|GetOn2))
        (Variables|Default|SetOn2 _returnvalue_5)
        (Rendering|ToggleVisibility (Variables|Default|GetPointLight1) false)))))

(fn ConstructionScript)