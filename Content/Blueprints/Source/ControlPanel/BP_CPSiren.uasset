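; BP_CPSiren is a control panel siren that plays a configurable sound event through its Speaker component.
; The event is assigned at construction and starts paused on BeginPlay.
; RequestSetEnabled keeps a counter of enable and disable requests, so the sound plays while the count is above zero, and reapplies the volume.
; Each request is also forwarded to every entry in its Speakers array.
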(event EventBeginPlay
  (|CallParentFunction)
  (Class|FMODAudioComponent|SetPaused (Variables|Default|GetSpeaker) true))

(fn ConstructionScript
  (|CallParentFunction)
  (Class|FMODAudioComponent|SetEvent (Variables|Default|GetSpeaker) (Variables|Default|GetSound)))

(fn RequestSetEnabled
  (params (Enabled :type Boolean))
  (bind _speaker (Variables|Default|GetSpeaker))
  (bind _output_get (Variables|Default|SetSoundCount (+ (Math|Integer|SelectInt 1 -1 Enabled) (Variables|Default|GetSoundCount))))
  (Class|FMODAudioComponent|SetPaused _speaker (<= _output_get 0))
  (Class|FMODAudioComponent|SetVolume _speaker (Variables|Default|GetVolume))
  (for _array_element (Variables|Default|GetSpeakers)
    (CallFunction|RequestSetEnabled _array_element Enabled)))