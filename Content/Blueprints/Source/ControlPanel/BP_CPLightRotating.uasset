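; A control panel light that works as a rotating beacon with two spotlights.
; Construction applies the on color to both spots and caches the brighter one's intensity as the base level.
; While lit, Tick spins the mount in yaw and modulates both spots with a smooth blink.
; SetLightState sets the lit flag and spot visibility, and that flag zeroes rotation and intensity when off.
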(event EventTick
  (params (DeltaSeconds :type Float%20%28single-precision%29))
  (bind _islit (Variables|Default|GetIsLit))
  (bind _returnvalue (Math|Conversions|ToFloat(Boolean) _islit))
  (Transformation|AddRelativeRotation (Variables|Default|GetMount) (Math|Rotator|MakeRotator 0.0 0.0 (* DeltaSeconds (Variables|Instrument|GetRotationSpeed) _returnvalue)) false false)
  (bind _value (CallFunction|SmoothBlink))
  (Rendering|Components|Light|SetIntensity (Variables|Default|GetSpotL) (* _value (Variables|Instrument|GetIntensity) _returnvalue)))

(fn ConstructionScript
  (Variables|Instrument|SetIntensity (Math|Float|Max(Float) (Variables|/Script/Engine.LightComponentBase|GetIntensity (Variables|Default|GetSpotL)) (Variables|/Script/Engine.LightComponentBase|GetIntensity (Variables|Default|GetSpotR))))
  (Rendering|Components|Light|SetLightColor (Variables|Default|GetSpotL) (Variables|Default|GetOnColor) true))

(fn SetLightState
  (params (Enabled :type Boolean))
  (bind _output_get (Variables|Default|SetIsLit Enabled))
  (Rendering|SetVisibility (Variables|Default|GetSpotL) _output_get false))