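; Vertical analogue slider for a control panel that moves its Slider component along relative Y in response to mouse input.
; BeginPlay places the slider at StartValue, without updating CurrentLocation.
; MouseValues adds a quarter of MouseY to CurrentLocation, ignoring any step that would pass MinLocation or MaxLocation.
; Each call also prints a position ratio derived from those limits; the value is only printed, never stored or sent on.
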(event EventBeginPlay
  (Transformation|SetRelativeLocation (Variables|Default|GetSlider) (Math|Vector|MakeVector 0.0 (Variables|Default|GetStartValue) 0.0) false false))

(event EventMouseValues
  (params (Mouse%20X :type Float%20%28single-precision%29) (Mouse%20Y :type Float%20%28single-precision%29))
  (bind _returnvalue (/ Mouse%20Y 4.0))
  (Utilities|FlowControl|Sequence
    (:then_0
      (if (> _returnvalue 0.0)
        (if (not (> (+ _returnvalue (Variables|Default|GetCurrentLocation)) (Variables|Default|GetMaxLocation)))
          (bind _output_get (Variables|Default|SetCurrentLocation (+ _returnvalue (Variables|Default|GetCurrentLocation)) :!label _label))
          (Transformation|SetRelativeLocation (Variables|Default|GetSlider) (Math|Vector|MakeVector 0.0 _output_get 0.0) false false))
        (elif (not (< (+ _returnvalue (Variables|Default|GetCurrentLocation)) (Variables|Default|GetMinLocation)))
          (goto _label))))
    (:then_1
      (Development|PrintString (Utilities|String|ToString(Float) (Math|Float|Absolute(Float) (- (/ (+ (Variables|Default|GetMaxLocation) (Variables|Default|GetCurrentLocation)) (+ (Math|Float|Absolute(Float) (Variables|Default|GetMaxLocation)) (Math|Float|Absolute(Float) (Variables|Default|GetMinLocation)))) 1.0)))))))

(fn ConstructionScript)