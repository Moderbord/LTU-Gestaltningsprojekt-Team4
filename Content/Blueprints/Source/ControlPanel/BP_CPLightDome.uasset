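; BP_CPLightDome is a control panel dome light with a blinking point light.
; Its construction script creates a dynamic material instance on the Lamp as EmissiveMaterial, runs the parent script, then caches the point light's starting intensity.
; Each tick scales that intensity by SmoothBlink and the IsLit flag, so the point light pulses when lit and is dark otherwise.
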(event EventTick
  (params (DeltaSeconds :type Float%20%28single-precision%29))
  (bind _value (CallFunction|SmoothBlink))
  (Rendering|Components|Light|SetIntensity (Variables|Default|GetPointLight) (* _value (Variables|Rendering|GetIntensity) (Math|Conversions|ToFloat(Boolean) (Variables|Default|GetIsLit)))))

(fn ConstructionScript
  (bind _lamp (Variables|Default|GetLamp))
  (bind _returnvalue (Rendering|Material|CreateDynamicMaterialInstance _lamp 0 (Rendering|Material|GetMaterial _lamp 0) "None" :!class /Script/Engine.PrimitiveComponent))
  (Variables|Default|SetEmissiveMaterial _returnvalue)
  (|CallParentFunction)
  (Variables|Rendering|SetIntensity (Variables|/Script/Engine.LightComponentBase|GetIntensity (Variables|Default|GetPointLight))))