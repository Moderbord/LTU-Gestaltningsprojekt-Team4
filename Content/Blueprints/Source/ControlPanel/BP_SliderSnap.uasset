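; BP_SliderSnap is a control panel slider meant to step between discrete notches on axis input.
; When no animation is playing, AxisValuesEvent moves CurrentNotch and CurrentAngle one step up or down within NotchMin and NotchMax, printing the direction.
; The logic looks unfinished: the direction test compares constant zeros, so only the down branch runs, and the Slider's relative location is always set to zero.
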(event EventAxisValuesEvent
  (params (Values :type Vector :default "0, 0, 0"))
  (if (not (Variables|Default|GetAnimationPlaying))
    (if (> 0.0 0.0)
      (if (not (== (Variables|Default|GetCurrentNotch) (Variables|Default|GetNotchMax)))
        (Development|PrintString "up")
        (Variables|Default|SetCurrentAngle (+ (Variables|Default|GetCurrentAngle) (Variables|Default|GetAngleDifference)))
        (Variables|Default|SetCurrentNotch (+ (Variables|Default|GetCurrentNotch) 1))
        (Transformation|SetRelativeLocation (Variables|Default|GetSlider) "0, 0, 0" false false))
      (elif (not (== (Variables|Default|GetCurrentNotch) (Variables|Default|GetNotchMin)))
        (Development|PrintString "down")
        (Variables|Default|SetCurrentAngle (- (Variables|Default|GetCurrentAngle) (Variables|Default|GetAngleDifference)))
        (Variables|Default|SetCurrentNotch (- (Variables|Default|GetCurrentNotch) 1))
        (Transformation|SetRelativeLocation (Variables|Default|GetSlider) "0, 0, 0" false false)))))

(fn ConstructionScript)