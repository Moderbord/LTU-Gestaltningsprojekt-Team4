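; Ceiling light Blueprint for the control panel set that blinks its point light while lit.
; Each tick drives intensity from a clamped cosine of game time, shaped by blink rate and offset and gated by IsLit, so it stays dark half of each cycle.
; The construction script caches the light's intensity as the peak and creates a dynamic lamp material, which this graph never animates.
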(event EventTick
  (params (DeltaSeconds :type Float%20%28single-precision%29))
  (Rendering|Components|Light|SetIntensity (Variables|Default|GetPointLight) (* (Math|Float|Clamp(Float) (Math|Trig|Cos(Radians) (* (+ (* (Utilities|Time|GetGameTimeinSeconds) (Variables|Default|GetBlinkRate)) (Variables|Default|GetBlinkOffset)) (Math|Trig|GetPI) 2.0))) (Variables|Rendering|GetIntensity) (Math|Conversions|ToFloat(Boolean) (Variables|Default|GetIsLit)))))

(fn ConstructionScript
  (bind _lamp (Variables|Default|GetLamp))
  (bind _returnvalue (Rendering|Material|CreateDynamicMaterialInstance _lamp 0 (Rendering|Material|GetMaterial _lamp 0) "None" :!class /Script/Engine.PrimitiveComponent))
  (Variables|Default|SetEmissiveMaterial _returnvalue)
  (|CallParentFunction)
  (Variables|Rendering|SetIntensity (Variables|/Script/Engine.LightComponentBase|GetIntensity (Variables|Default|GetPointLight))))