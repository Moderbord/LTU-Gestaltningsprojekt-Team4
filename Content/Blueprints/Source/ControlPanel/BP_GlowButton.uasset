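; BP_GlowButton is an interactable control panel button with a point light that glows in response to signals.
; Interacting toggles its State and reports it, with the button's signal Type, to its Component through the BPI_MCPDelegates interface.
; The light starts hidden and is driven separately by ReceiveSignal, showing only while the received value exceeds LightThreshold, so it follows incoming signals rather than the toggle.
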(event EventBeginPlay
  (|CallParentFunction)
  (Rendering|SetVisibility (Variables|Default|GetPointLight) false false))

(event Collision|EventActorBeginOverlap
  (params (OtherActor :type Actor%20Object%20Reference))
  (|CallParentFunction OtherActor) ; This node is disabled and will not be called.\nDrag off pins to build functionality.
)

(event EventTick
  (params (DeltaSeconds :type Float%20%28single-precision%29))
  (|CallParentFunction DeltaSeconds) ; This node is disabled and will not be called.\nDrag off pins to build functionality.
)

(event EventOnInteract
  (params (Caller :type Actor%20Object%20Reference))
  (Signaling|Interact))

(fn ConstructionScript
  (|CallParentFunction))

(fn ReceiveSignal
  (params (Value :type Float%20%28single-precision%29))
  (|CallParentFunction Value)
  (Rendering|SetVisibility (Variables|Default|GetPointLight) (> Value (Variables|Settings|GetLightThreshold)) false))

(fn Interact
  (bind _asbpi_mcpdelegates (Utilities|Casting|CastToBPI_MCPDelegates (Variables|Default|GetComponent)))
  (bind _output_get (Variables|Default|SetState (not (Variables|Default|GetState))))
  (Default|ButtonPressed _asbpi_mcpdelegates _output_get (Variables|Default|GetType)))