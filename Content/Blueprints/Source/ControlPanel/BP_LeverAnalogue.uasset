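; Analogue lever for a control panel, with a handle that pitches between a minimum and maximum angle as the mouse moves vertically.
; BeginPlay sets the handle to its starting angle.
; MouseValues inverts and halves mouse Y, then applies it to the angle, rejecting rather than clamping any step that would pass a limit.
; The normalised position, which assumes symmetric limits, is only printed.
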(event EventBeginPlay
  (bind _startingangle (Variables|Default|GetStartingAngle))
  (Transformation|SetRelativeRotation (Variables|Default|GetHandleOffset) (Math|Rotator|MakeRotator 0.0 _startingangle 0.0) false false)
  (Variables|Default|SetCurrentAngle _startingangle))

(event EventMouseValues
  (params (Mouse%20X :type Float%20%28single-precision%29) (Mouse%20Y :type Float%20%28single-precision%29))
  (bind _returnvalue (* -1 Mouse%20Y))
  (bind _returnvalue_2 (/ _returnvalue 2.0))
  (Utilities|FlowControl|Sequence
    (:then_0
      (if (> _returnvalue_2 0.0)
        (if (not (> (+ _returnvalue_2 (Variables|Default|GetCurrentAngle)) (Variables|Default|GetAngleMax)))
          (bind _output_get (Variables|Default|SetCurrentAngle (+ _returnvalue_2 (Variables|Default|GetCurrentAngle)) :!label _label))
          (Transformation|SetRelativeRotation (Variables|Default|GetHandleOffset) (Math|Rotator|MakeRotator 0.0 _output_get 0.0) false false))
        (elif (not (< (+ _returnvalue_2 (Variables|Default|GetCurrentAngle)) (Variables|Default|GetAngleMin)))
          (goto _label))))
    (:then_1
      (Development|PrintString (Utilities|String|ToString(Float) (/ (+ (Variables|Default|GetAngleMax) (Variables|Default|GetCurrentAngle)) (+ (Math|Float|Absolute(Float) (Variables|Default|GetAngleMax)) (Math|Float|Absolute(Float) (Variables|Default|GetAngleMin)))))))))

(fn ConstructionScript)