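; BP_WheelSnap is a control panel wheel that snaps between notches, rotating its Base in yaw one step per move.
; AxisValuesEvent picks the direction from the Y value: positive steps down toward NotchMin, anything else, including zero, steps up toward NotchMax.
; A timeline per direction animates the turn by AngleDifference, blocks input while playing, then updates the stored angle and notch and resets its time.
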(event EventAxisValuesEvent
  (params (Values :type Vector :default "0, 0, 0"))
  (bind _base (Variables|Default|GetBase))
  (if (not (Variables|Default|GetAnimationPlaying))
    (if (> (.y Values) 0.0)
      (if (not (== (Variables|Default|GetCurrentNotch) (Variables|Default|GetNotchMin)))
        (Development|PrintString "spin left")
        (Variables|Default|SetAnimationPlaying true)
        (bind _wheelrotationfloat (Timeline|WheelAnimation2 Play)
          (:Update
            (Transformation|SetRelativeRotation _base (Math|Rotator|MakeRotator 0.0 0.0 (- (Variables|Default|GetCurrentAngle) (* _wheelrotationfloat (Variables|Default|GetAngleDifference)))) false false))
          (:Finished
            (Variables|Default|SetCurrentAngle (- (Variables|Default|GetCurrentAngle) (* _wheelrotationfloat (Variables|Default|GetAngleDifference))))
            (Variables|Default|SetAnimationPlaying false)
            (Variables|Default|SetCurrentNotch (- (Variables|Default|GetCurrentNotch) 1))
            (Timeline|WheelAnimation2 SetNewTime))))
      (elif (not (== (Variables|Default|GetCurrentNotch) (Variables|Default|GetNotchMax)))
        (Development|PrintString "spin right")
        (Variables|Default|SetAnimationPlaying true)
        (bind _wheelrotationfloat_2 (Timeline|WheelAnimation Play)
          (:Update
            (Transformation|SetRelativeRotation _base (Math|Rotator|MakeRotator 0.0 0.0 (+ (Variables|Default|GetCurrentAngle) (* _wheelrotationfloat_2 (Variables|Default|GetAngleDifference)))) false false))
          (:Finished
            (Variables|Default|SetCurrentAngle (+ (Variables|Default|GetCurrentAngle) (* _wheelrotationfloat_2 (Variables|Default|GetAngleDifference))))
            (Variables|Default|SetAnimationPlaying false)
            (Variables|Default|SetCurrentNotch (+ (Variables|Default|GetCurrentNotch) 1))
            (Timeline|WheelAnimation SetNewTime)))))))

(fn ConstructionScript)