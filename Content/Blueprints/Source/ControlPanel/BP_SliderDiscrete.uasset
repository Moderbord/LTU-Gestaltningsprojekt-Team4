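; Control panel slider that moves between discrete notches along its local X axis, starting at StartValue.
; AxisValuesEvent uses the sign of the Y input to pick a direction, unless AnimationPlaying is set or the notch limit is reached.
; One timeline per direction slides the component by LocationDifference, then updates the stored location and notch and resets its time.
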(event EventBeginPlay
  (Transformation|SetRelativeLocation (Variables|Default|GetSlider) (Math|Vector|MakeVector (Variables|Default|GetStartValue) 0.0 0.0) false false)
  (Variables|Default|SetCurrentLocation (Variables|Default|GetStartValue)))

(event EventAxisValuesEvent
  (params (Values :type Vector :default "0, 0, 0"))
  (Utilities|FlowControl|Sequence
    (:then_0
      (if (not (Variables|Default|GetAnimationPlaying))
        (if (> (.y Values) 0.0)
          (if (not (== (Variables|Default|GetCurrentNotch) (Variables|Default|GetNotchMin)))
            (Development|PrintString "left")
            (bind _location_value (Timeline|SliderAnimation Play)
              (:Update
                (Transformation|SetRelativeLocation (Variables|Default|GetSlider) (Math|Vector|MakeVector (- (Variables|Default|GetCurrentLocation) (* _location_value (Variables|Default|GetLocationDifference))) 0.0 0.0) false false))
              (:Finished
                (Variables|Default|SetCurrentLocation (- (Variables|Default|GetCurrentLocation) (* _location_value (Variables|Default|GetLocationDifference))))
                (Variables|Default|SetCurrentNotch (- (Variables|Default|GetCurrentNotch) 1))
                (Timeline|SliderAnimation SetNewTime))))
          (elif (not (== (Variables|Default|GetCurrentNotch) (Variables|Default|GetNotchMax)))
            (Development|PrintString "right")
            (bind _location_value_2 (Timeline|SliderAnimation2 Play)
              (:Update
                (Transformation|SetRelativeLocation (Variables|Default|GetSlider) (Math|Vector|MakeVector (+ (Variables|Default|GetCurrentLocation) (* _location_value_2 (Variables|Default|GetLocationDifference))) 0.0 0.0) false false))
              (:Finished
                (Variables|Default|SetCurrentLocation (+ (Variables|Default|GetCurrentLocation) (* _location_value_2 (Variables|Default|GetLocationDifference))))
                (Variables|Default|SetCurrentNotch (+ (Variables|Default|GetCurrentNotch) 1))
                (Timeline|SliderAnimation2 SetNewTime)))))))
    (:then_1
      (switch int 0))))

(fn ConstructionScript)