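; Interactive control panel button that works as either a momentary or a latching switch, depending on Rebound.
; On BeginPlay it sets the button height from Pressed and reports that state to Component.
; On Interact, timelines slide the button along Z; latching mode toggles Pressed, while rebound mode reverses the motion after pressing.
; When a timeline finishes, it sends OnButtonPressedMessage to Component with the state and Active signal.
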(event EventBeginPlay
  (bind _pressed (Variables|Default|GetPressed))
  (|CallParentFunction)
  (Class|BPIMCPDelegates|OnButtonPressed(Message) (Variables|Default|GetComponent) _pressed (Variables|Default|GetActive))
  (Transformation|SetRelativeLocation (Variables|Default|GetButton) (Math|Vector|MakeVector 0.0 0.0 (Math|Float|SelectFloat -1.0 0.0 _pressed)) false false))

(event EventInteract
  (params (Caller :type Actor%20Object%20Reference))
  (if (Variables|Default|GetRebound)
    (bind _button_value (Timeline|ButtonTimeline2 Play)
      (:Update
        (Transformation|SetRelativeLocation (Variables|Default|GetButton) (Math|Vector|MakeVector 0.0 0.0 (* -1 _button_value)) false false))
      (:Finished
        (Class|BPIMCPDelegates|OnButtonPressed(Message) (Variables|Default|GetComponent) true (Variables|Default|GetActive))
        (Timeline|ButtonTimeline2 Reverse)))
    (elif (Variables|Default|GetPressed)
      (Variables|Default|SetPressed false)
      (bind _location_value (Timeline|ButtonTimeline Reverse)
        (:Update
          (Transformation|SetRelativeLocation (Variables|Default|GetButton) (Math|Vector|MakeVector 0.0 0.0 (* -1 _location_value)) false false))
        (:Finished
          (Class|BPIMCPDelegates|OnButtonPressed(Message) (Variables|Default|GetComponent) (Variables|Default|GetPressed) (Variables|Default|GetActive))))
      (else
        (Variables|Default|SetPressed true)
        (Timeline|ButtonTimeline Play)))))

(fn ConstructionScript)