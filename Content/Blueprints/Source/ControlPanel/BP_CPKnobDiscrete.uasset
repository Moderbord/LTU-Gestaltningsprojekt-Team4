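; Discrete knob for a control panel that rotates between stepped positions.
; SetControlPosition blends the BaseOffset component's relative yaw between the From and To step indices by Alpha.
; Each yaw angle is the index times StepSize plus Offset, interpolated with a rotator lerp.
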(fn ConstructionScript)

(fn SetControlPosition
  (params (From :type Integer) (To :type Integer) (Alpha :type Float%20%28single-precision%29))
  (bind _stepsize (Variables|Default|GetStepSize))
  (bind _offset (Variables|Default|GetOffset))
  (Transformation|SetRelativeRotation (Variables|Default|GetBaseOffset) (Math|Rotator|Lerp(Rotator) (Math|Rotator|MakeRotator 0.0 0.0 (+ (* From _stepsize) _offset)) (Math|Rotator|MakeRotator 0.0 0.0 (+ (* To _stepsize) _offset)) Alpha) false false))