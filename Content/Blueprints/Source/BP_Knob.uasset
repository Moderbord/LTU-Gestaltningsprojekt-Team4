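; BP_Knob is an interactable knob actor that turns in fixed steps when used.
; On interact it adds SetAngle to the stored Angle, prints the new value, and applies it as the yaw of the Base component's relative rotation.
; Two point light visibility toggles remain in the graph but are not connected to any event.
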(event EventOnInteract
  (params (Caller :type Actor%20Object%20Reference))
  (Development|PrintString (Utilities|String|ToString(Float) (+ (Variables|Default|GetAngle) (Variables|Default|GetSetAngle))))
  (Variables|Default|SetAngle (+ (Variables|Default|GetAngle) (Variables|Default|GetSetAngle)))
  (Transformation|SetRelativeRotation (Variables|Default|GetBase) (Math|Rotator|MakeRotator 0.0 0.0 (Variables|Default|GetAngle)) false false))

(fn ConstructionScript)