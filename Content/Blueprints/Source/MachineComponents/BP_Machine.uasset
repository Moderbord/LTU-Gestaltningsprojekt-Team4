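; BP_Machine is a manager that drives the ticking of machine components in the level.
; On BeginPlay it finds every BP_MachineComponentBase actor in the world and sorts it into an Active, SemiPassive or Passive array by its TickGroup.
; Each frame it manually calls Tick on those components group by group, in that order, passing along delta time, which gives a controlled update order.
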(event EventBeginPlay
  (bind _outactors (Actor|GetAllActorsOfClass "/Game/Blueprints/Source/MachineComponents/BP_MachineComponentBase.BP_MachineComponentBase_C")) ; idgaf fight me
  (for _array_element _outactors
    (CallFunction|RegisterComponent (Variables|/Game/Blueprints/Source/MachineComponents/BP_MachineComponentBase.BP_MachineComponentBase_C|GetTick%20Group _array_element) _array_element)))

(event Collision|EventActorBeginOverlap
  (params (OtherActor :type Actor%20Object%20Reference)))

(event EventTick
  (params (DeltaSeconds :type Float%20%28single-precision%29))
  (for _array_element (Variables|Default|GetActive)
    (Default|Tick _array_element DeltaSeconds))
  (for _array_element_2 (Variables|Default|GetSemiPassive)
    (Default|Tick _array_element DeltaSeconds))
  (for _array_element_3 (Variables|Default|GetPassive)
    (Default|Tick _array_element DeltaSeconds)))

(fn ConstructionScript)

(fn RegisterComponent
  (params (Group :type EComponentTickGroup%20Enum :default "NewEnumerator0") (Component :type BP%20Machine%20Component%20Base%20Object%20Reference%20%28by%20ref%29))
  (switch Utilities|FlowControl|Switch|SwitchonEComponentTickGroup Group
    (:NewEnumerator0
      (Utilities|Array|Add (Variables|Default|GetActive) Component))
    (:NewEnumerator1
      (Utilities|Array|Add (Variables|Default|GetSemiPassive) Component))
    (:NewEnumerator2
      (Utilities|Array|Add (Variables|Default|GetPassive) Component))))