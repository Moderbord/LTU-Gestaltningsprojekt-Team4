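; BP_MCBrake is a brake machine component that passes on part of a resource and turns the rest into heat.
; Each Tick pushes the buffered amount scaled by Efficiency, then subtracts the Push result from the initial amount.
; That difference, as a fraction of buffer capacity times MaxHeatPerFullBuffer, is added to Temperature.
; The buffer is then emptied, so nothing carries over between ticks.
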(event EventBeginPlay
  (|CallParentFunction) ; This node is disabled and will not be called.\nDrag off pins to build functionality.
)

(event Collision|EventActorBeginOverlap
  (params (OtherActor :type Actor%20Object%20Reference))
  (|CallParentFunction OtherActor) ; This node is disabled and will not be called.\nDrag off pins to build functionality.
)

(event EventTick
  (params (DeltaSeconds :type Float%20%28single-precision%29))
  (|CallParentFunction DeltaSeconds) ; This node is disabled and will not be called.\nDrag off pins to build functionality.
)

(fn ConstructionScript
  (|CallParentFunction))

(fn Tick
  (params (Delta%20Seconds :type Float%20%28single-precision%29))
  (|CallParentFunction Delta%20Seconds)
  (bind (_current _capacity _maximum) (CallFunction|GetBuffer (Variables|Default|GetResource)))
  (bind _output_get (LocalVariables|SetInitial _current))
  (bind _accepted (CallFunction|Push (Variables|Default|GetResource) (* _output_get (Variables|Default|GetEfficiency))))
  (Variables|Default|SetTemperature (+ (* (Variables|Default|GetMaxHeatPerFullBuffer) (/ (- (LocalVariables|GetInitial) _accepted) _maximum)) (Variables|Default|GetTemperature)))
  (CallFunction|SetBuffer (Variables|Default|GetResource) 0.0))