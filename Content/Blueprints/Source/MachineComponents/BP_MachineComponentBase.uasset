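; Base actor for machine components that store resources in capacity-limited buffers and transfer them between linked Inputs and Outputs.
; Push offers stored amounts to Outputs and Pull requests free space's worth from Inputs, each stopping once the relevant amount is within EmptyMargin.
; Both use SendResource, which deducts what the receiver's ReceiveResource accepts after clamping to capacity.
; An editor tick draws colored debug arrows showing the input and output links.
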(event EventBeginPlay)

(event Collision|EventActorBeginOverlap
  (params (OtherActor :type Actor%20Object%20Reference)))

(event EventTick
  (params (DeltaSeconds :type Float%20%28single-precision%29)))

(event EventEditorTick
  (CallFunction|DrawReferences))

(fn ConstructionScript
  (AddComponent|AddChildActorComponent false))

(fn Push
  (params (Resource :type EResources%20Enum :default "NewEnumerator0"))
  (bind _array_element (Utilities|Array|ForEachLoopwithBreak (Variables|Default|GetOutputs) :!label _label)
    (:LoopBody
      (bind _filled (CallFunction|GetBufferFilled Resource))
      (if (> _filled (LocalVariables|GetEmptyMargin))
        (CallFunction|SendResource _array_element Resource _filled)
        (else
          (goto _label Break))))))

(fn Pull
  (params (Resource :type EResources%20Enum :default "NewEnumerator0"))
  (bind _array_element (Utilities|Array|ForEachLoopwithBreak (Variables|Default|GetInputs) :!label _label)
    (:LoopBody
      (bind _amount (CallFunction|GetBufferFree Resource))
      (if (> _amount (LocalVariables|GetEmpty%20Margin))
        (CallFunction|SendResource _array_element self Resource _amount)
        (else
          (goto _label Break))))))

(fn GetBufferFree
  (params (Resource :type EResources%20Enum :default "NewEnumerator0"))
  (bind _buffers (Variables|Default|GetBuffers))
  (bind (_value _returnvalue) (Utilities|Map|Find _buffers Resource))
  (bind (_capacity _current) (Utilities|Struct|BreakResourceBuffer _value))
  (if _returnvalue
    (return (- _capacity _current) _value)
    (else
      (return 0.0 _value))))

(fn GetBufferFilled
  (params (Resource :type EResources%20Enum :default "NewEnumerator0"))
  (bind _buffers (Variables|Default|GetBuffers))
  (bind (_value _returnvalue) (Utilities|Map|Find _buffers Resource))
  (if _returnvalue
    (return (.Current (Utilities|Struct|BreakResourceBuffer _value)) _value)
    (else
      (return 0.0 _value))))

(fn SendResource
  (params (Send%20To :type BP%20Machine%20Component%20Base%20Object%20Reference) (Resource :type EResources%20Enum :default "NewEnumerator0") (Amount :type Float%20%28single-precision%29))
  (bind (_filled _buffer) (CallFunction|GetBufferFilled Resource))
  (bind _accepted (CallFunction|ReceiveResource Send%20To Resource (Math|Float|Min(Float) _filled Amount)))
  (Utilities|Struct|SetmembersinResourceBuffer _buffer (- _filled _accepted)) ; Check for errors?
  (return (- Amount _accepted)))

(fn ReceiveResource
  (params (Resource :type EResources%20Enum :default "NewEnumerator0") (Amount :type Float%20%28single-precision%29))
  (bind _buffers (Variables|Default|GetBuffers))
  (bind (_value _returnvalue) (Utilities|Map|Find _buffers Resource))
  (bind (_capacity _current) (Utilities|Struct|BreakResourceBuffer _value))
  (bind (_free _total _has_overflowed) (|CalculateOverflow Amount _capacity _current))
  (if _returnvalue
    (if _has_overflowed ; Has overflowed?
      (Utilities|Struct|SetmembersinResourceBuffer _value _capacity)
      (return _free)
      (else
        (Utilities|Struct|SetmembersinResourceBuffer _value _total)
        (return Amount)))
    (else
      (return 0.0))))

(fn DrawReferences
  (for _array_element (Variables|Default|GetInputs)
    (bind (_result _out) (CallFunction|IsValidReference _array_element))
    (if _result
      (CallFunction|DrawLine _out self "(R=0.050070,G=1.000000,B=0.000000,A=1.000000)")))
  (for _array_element_2 (Variables|Default|GetOutputs)
    (bind (_result_2 _out_2) (CallFunction|IsValidReference _array_element_2))
    (if _result_2
      (CallFunction|DrawLine _out_2 "(R=1.000000,G=0.000000,B=0.015400,A=1.000000)"))))

(fn IsValidReference
  (params (Object :type BP%20Machine%20Component%20Base%20Object%20Reference))
  (if (Utilities|IsValid Object)
    (return true Object)
    (else
      (return false 0))))

(fn DrawLine
  (params (Destination :type BP%20Machine%20Component%20Base%20Object%20Reference) (Line%20Color :type Linear%20Color%20Structure))
  (Rendering|Debug|DrawDebugArrow (+ (Transformation|GetWorldLocation (Variables|Default|GetDefaultSceneRoot)) (Variables|Default|GetReferencePoint)) (+ (Transformation|GetWorldLocation (Variables|BP_MachineComponentBase_C|GetDefaultSceneRoot Destination)) (Variables|BP_MachineComponentBase_C|GetReferencePoint Destination)) 5e+02 Line%20Color 0.0 7.0))

(fn Tick
  (params (Delta%20Seconds :type Float%20%28single-precision%29)))