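; BP_MCBattery is a battery machine component that acts as a resource source.
; Each tick it pushes an amount of its resource scaled by delta time, Output and Efficiency.
; It then signals the pushed amount as a fraction of Output for that resource.
; BeginPlay and Tick defer to the parent component first, and the construction script is empty.
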(event EventBeginPlay
  (|CallParentFunction))

(event Collision|EventActorBeginOverlap
  (params (OtherActor :type Actor%20Object%20Reference)))

(event EventTick
  (params (DeltaSeconds :type Float%20%28single-precision%29)))

(fn ConstructionScript)

(fn Tick
  (params (Delta%20Seconds :type Float%20%28single-precision%29))
  (|CallParentFunction Delta%20Seconds)
  (bind _accepted (CallFunction|Push (Variables|Default|GetResource) (* Delta%20Seconds (Variables|Flow|GetOutput) (Variables|Default|GetEfficiency))))
  (CallFunction|SignalValue "NewEnumerator9" (Variables|Default|GetResource) (/ _accepted (Variables|Flow|GetOutput))))