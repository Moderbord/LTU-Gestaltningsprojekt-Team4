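; BP_MCCondenser is a machine component that cools its inputs and converts coolant into a second resource, likely steam.
; Each tick it pulls heat from every input, scaled by efficiency and temperature above a 22-degree baseline, into its own temperature.
; It draws coolant proportional to that heat and outputs product by the fraction supplied.
; It then sheds heat regardless of coolant received, without scaling by delta time.
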(fn ConstructionScript
  (|CallParentFunction))

(fn Tick
  (params (Delta%20Seconds :type Float%20%28single-precision%29))
  (bind _inputs (Variables|Default|GetInputs))
  (|CallParentFunction Delta%20Seconds)
  (for _array_element _inputs
    (Variables|/Game/Blueprints/Source/MachineComponents/Base/BP_MCBase.BP_MCBase_C|SetTemperature _array_element (- (Variables|/Game/Blueprints/Source/MachineComponents/Base/BP_MCBase.BP_MCBase_C|GetTemperature _array_element) (* (/ (Variables|Default|GetHeatTransportPerCycle) (Math|Conversions|ToFloat(Integer) (Utilities|Array|Length _inputs))) (/ (- (Variables|/Game/Blueprints/Source/MachineComponents/Base/BP_MCBase.BP_MCBase_C|GetTemperature _array_element) 22.0) (Variables|Default|GetTargetTemp)) (Variables|Default|GetEfficiency))))
    (Variables|Default|SetTemperature (+ (* (/ (Variables|Default|GetHeatTransportPerCycle) (Math|Conversions|ToFloat(Integer) (Utilities|Array|Length _inputs))) (/ (- (Variables|/Game/Blueprints/Source/MachineComponents/Base/BP_MCBase.BP_MCBase_C|GetTemperature _array_element) 22.0) (Variables|Default|GetTargetTemp)) (Variables|Default|GetEfficiency)) (Variables|Default|GetTemperature))))
  (bind _percentofrequested (CallFunction|TakefromBuffer "NewEnumerator0" (* (Math|Float|Min(Float) (* (/ (Variables|Default|GetTemperature) (Variables|Default|GetTargetTemp)) (Variables|Default|GetEfficiency)) 1.0) (Variables|Default|GetCoolantPerCycle))))
  (CallFunction|ChangeBuffer "NewEnumerator9" (* _percentofrequested (Variables|Default|GetCoolantToSteamRatio)))
  (Variables|Default|SetTemperature (- (Variables|Default|GetTemperature) (* (Math|Float|Min(Float) (* (/ (Variables|Default|GetTemperature) (Variables|Default|GetTargetTemp)) (Variables|Default|GetEfficiency)) 1.0) (Variables|Default|GetHeatTransportPerCycle)))))