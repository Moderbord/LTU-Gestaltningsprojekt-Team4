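; Alternator machine component that converts buffered torque into power.
; Each Tick takes an efficiency-based share of the torque buffer, adds power scaled by PowerPerCycle, then flushes the power buffer and signals the flushed fraction of capacity.
; PostTick drains torque by a loss proportional to load and signals the torque ratio.
; That ratio also drives an eased rotor spin and emissive glow.
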(event EventTick
  (params (DeltaSeconds :type Float%20%28single-precision%29))
  (bind _output_get (Variables|Rendering|SetRotationInertia (Math|Interpolation|FInterptoConstant (Variables|Rendering|GetRotationInertia) (* (Variables|Status|GetActualTorque) (Variables|Rendering|GetRotationMult)) DeltaSeconds (Variables|Rendering|GetRotationDelta))))
  (Transformation|AddRelativeRotation (Variables|Default|GetSM_Generator_polySurface119) (Math|Rotator|MakeRotator 0.0 0.0 _output_get) false false)
  (Rendering|Material|SetScalarParameterValue (Variables|Default|GetMaterial) "Emissive" _output_get :!class /Script/Engine.MaterialInstanceDynamic))

(fn ConstructionScript
  (|CallParentFunction))

(fn Tick
  (params (Delta%20Seconds :type Float%20%28single-precision%29))
  (|CallParentFunction Delta%20Seconds)
  (bind (_current _capacity) (CallFunction|GetBuffer "NewEnumerator2"))
  (Variables|Status|SetActualTorque (/ _current _capacity))
  (bind _percentofcapacity (CallFunction|TakeAllfromBuffer "NewEnumerator2" (Variables|Default|GetEfficiency)))
  (CallFunction|ChangeBuffer "NewEnumerator1" (* _percentofcapacity (Variables|Default|GetPowerPerCycle)))
  (bind _capacity_2 (CallFunction|GetBuffer "NewEnumerator1"))
  (bind _accepted (CallFunction|Flush "NewEnumerator1"))
  (CallFunction|SignalValue "NewEnumerator9" "NewEnumerator1" (/ _accepted _capacity_2)))

(fn PostTick
  (params (DeltaTime :type Float%20%28single-precision%29))
  (bind _actualtorque (Variables|Status|GetActualTorque))
  (|CallParentFunction DeltaTime)
  (CallFunction|ChangeBuffer "NewEnumerator2" (* DeltaTime (Variables|Default|GetLossPerCycle) _actualtorque -1.0))
  (CallFunction|SignalValue "NewEnumerator4" "NewEnumerator2" _actualtorque))