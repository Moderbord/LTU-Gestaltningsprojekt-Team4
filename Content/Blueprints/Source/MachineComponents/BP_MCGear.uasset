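; Gear machine component that relays a resource through the machine and glows according to how much it moves.
; Its Tick function calls the parent, then pulls and pushes the resource at Throughput scaled by Efficiency and delta time.
; The accepted amount divided by Throughput becomes ActualThroughput, which is broadcast through SignalValue.
; The event graph eases the material's Emissive parameter toward that value times EmissionStrength.
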(event EventTick
  (params (DeltaSeconds :type Float%20%28single-precision%29))
  (bind _output_get (Variables|Rendering|SetEmissionCurrent (Math|Interpolation|FInterpTo (Variables|Rendering|GetEmissionCurrent) (* (Variables|Signaling|GetActualThroughput) (Variables|Rendering|GetEmissionStrength)) DeltaSeconds (Variables|Rendering|GetEmissionDelta))))
  (Rendering|Material|SetScalarParameterValue (Variables|Default|GetMaterial) "Emissive" _output_get :!class /Script/Engine.MaterialInstanceDynamic))

(fn ConstructionScript)

(fn Tick
  (params (Delta%20Seconds :type Float%20%28single-precision%29))
  (bind _efficiency (Variables|Default|GetEfficiency))
  (bind _throughput (Variables|Flow|GetThroughput))
  (bind _resource (Variables|Default|GetResource))
  (bind _returnvalue (* _throughput _efficiency Delta%20Seconds))
  (|CallParentFunction Delta%20Seconds)
  (Utilities|FlowControl|Sequence
    (:then_0
      (bind _current (CallFunction|GetBuffer (Variables|Default|GetResource)))
      (LocalVariables|SetInitial _current)
      (bind _received (CallFunction|Pull _resource _returnvalue))
      (LocalVariables|SetTotalReceived _received)
      (bind _accepted (CallFunction|Push _resource _returnvalue))
      (LocalVariables|SetTotalAccepted _accepted))
    (:then_1
      (bind _output_get (Variables|Signaling|SetActualThroughput (/ (LocalVariables|GetTotalAccepted) (Variables|Flow|GetThroughput))))
      (CallFunction|SignalValue "NewEnumerator9" (Variables|Default|GetResource) _output_get))))