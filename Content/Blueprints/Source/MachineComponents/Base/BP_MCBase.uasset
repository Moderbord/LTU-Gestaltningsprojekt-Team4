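; Base Blueprint for machine components that store resources in per-type buffers and exchange them with linked Input and Output components.
; Analogue and button signals set power and throttle, which Tick combines with an optional fuse check into actual throttle and efficiency.
; PostTick cools temperature and publishes state and buffer fill ratios to an OutSignals map, readable through Probe.
; Editor ticks draw colored debug arrows along component links.
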(event EventBeginPlay
  (bind _returnvalue (Actor|GetComponentbyClass "/Script/Engine.StaticMeshComponent"))
  (bind _returnvalue_2 (Rendering|Material|CreateDynamicMaterialInstance _returnvalue 0 (Rendering|Material|GetMaterial _returnvalue 0) "None" :!class /Script/Engine.PrimitiveComponent))
  (Variables|Rendering|SetMaterial _returnvalue_2))

(event EventEditorTick
  (Rendering|DrawReferences))

(event EventOnAnalogueChanged
  (params (New%20Value :type Float%20%28single-precision%29) (Signal :type EActiveSignals%20Enum :default "NewEnumerator0"))
  (switch Utilities|FlowControl|Switch|SwitchonEActiveSignals Signal
    (:NewEnumerator1
      (Variables|Status|SetRunning (Math|Conversions|ToBoolean(Integer) (Math|Float|Truncate New%20Value))))
    (:NewEnumerator2
      (Variables|Status|SetThrottle New%20Value))
    (:NewEnumerator5
      (Variables|Status|SetThrottle (Math|Float|Clamp(Float) (+ New%20Value (Variables|Status|GetThrottle)) (Variables|Status|GetMinThrottle) (Variables|Status|GetMaxThrottle))))))

(event EventOnButtonStateChanged
  (params (State :type Boolean) (Signal :type EActiveSignals%20Enum :default "NewEnumerator0"))
  (switch Utilities|FlowControl|Switch|SwitchonEActiveSignals Signal
    (:NewEnumerator1
      (Variables|Status|SetRunning State))
    (:NewEnumerator2
      (Variables|Status|SetThrottle (Math|Conversions|ToFloat(Boolean) State)))
    (:NewEnumerator6
      (if State
        (Variables|Status|SetRunning (not (Variables|Status|GetRunning)))))
    (:NewEnumerator4
      (Variables|Status|SetRunning false :!label _label))
    (:NewEnumerator7
      (Variables|Status|SetThrottle 0.0)
      (goto _label))
    (:NewEnumerator8
      (Variables|Status|SetRunning true :!label _label_2))
    (:NewEnumerator9
      (Variables|Status|SetThrottle 1.0)
      (goto _label_2))))

(fn ConstructionScript
  (AddComponent|AddChildActorComponent false))

(fn Push
  (params (Resource :type EResources%20Enum :default "NewEnumerator0") (Amount :type Float%20%28single-precision%29))
  (bind _returnvalue (< Amount 0.0))
  (bind _inputs (Variables|Flow|GetInputs))
  (bind _outputs (Variables|Flow|GetOutputs))
  (bind _returnvalue_2 (select _returnvalue _inputs _outputs))
  (bind _array_element (Utilities|Array|ForEachLoopwithBreak _returnvalue_2 :!label _label)
    (:LoopBody
      (bind _current (Flow|GetBuffer Resource))
      (if (> (+ (LocalVariables|GetOverflow) (/ (Math|Float|Min(Float) (Math|Float|Absolute(Float) Amount) _current) (Math|Conversions|ToFloat(Integer) (Utilities|Array|Length _returnvalue_2)))) (LocalVariables|GetEmptyMargin))
        (bind _accepted (Flow|SendResource _array_element Resource (+ (LocalVariables|GetOverflow) (/ (Math|Float|Min(Float) (Math|Float|Absolute(Float) Amount) _current) (Math|Conversions|ToFloat(Integer) (Utilities|Array|Length _returnvalue_2))))))
        (LocalVariables|SetOverflow (- (+ (LocalVariables|GetOverflow) (/ (Math|Float|Min(Float) (Math|Float|Absolute(Float) Amount) _current) (Math|Conversions|ToFloat(Integer) (Utilities|Array|Length _returnvalue_2)))) _accepted))
        (LocalVariables|SetTotalAccepted (+ _accepted (LocalVariables|GetTotalAccepted)))
        (else
          (goto _label Break))))
    (:Completed
      (return (LocalVariables|GetTotalAccepted)))))

(fn Pull
  (params (Resource :type EResources%20Enum :default "NewEnumerator0") (Amount :type Float%20%28single-precision%29))
  (bind _array_element (Utilities|Array|ForEachLoopwithBreak (select (< Amount 0.0) (Variables|Flow|GetOutputs) (Variables|Flow|GetInputs)) :!label _label)
    (:LoopBody
      (bind _capacity (Flow|GetBuffer Resource))
      (if (> (Math|Float|Min(Float) (Math|Float|Absolute(Float) Amount) _capacity) (LocalVariables|GetEmptyMargin))
        (bind _accepted (Flow|SendResource _array_element self Resource (Math|Float|Min(Float) (Math|Float|Absolute(Float) Amount) _capacity)))
        (LocalVariables|SetTotalReceived (+ _accepted (LocalVariables|GetTotalReceived)))
        (else
          (goto _label Break))))
    (:Completed
      (return (LocalVariables|GetTotalReceived)))))

(fn Flush
  (params (Resource :type EResources%20Enum :default "NewEnumerator5"))
  (bind _current (Flow|GetBuffer Resource))
  (bind _accepted (Flow|Push Resource _current))
  (return _accepted))

(fn SetBuffer
  (params (Resource :type EResources%20Enum :default "NewEnumerator0") (Amount :type Float%20%28single-precision%29))
  (bind _buffers (Variables|Flow|GetBuffers))
  (bind _structout (Utilities|Struct|SetmembersinResourceBuffer (.Value (Utilities|Map|Find _buffers Resource)) Amount))
  (Utilities|Map|Add _buffers Resource _structout))

(fn GetBuffer
  (params (Resource :type EResources%20Enum :default "NewEnumerator0"))
  (bind _buffers (Variables|Flow|GetBuffers))
  (bind (_value _returnvalue) (Utilities|Map|Find _buffers Resource))
  (bind (_current _capacity _maximum) (Utilities|Struct|BreakResourceBuffer _value))
  (if _returnvalue
    (return _current _capacity _maximum (- _maximum _current))
    (else
      (return 0.0 0.0 0.0 0.0))))

(fn ChangeBuffer
  (params (Resource :type EResources%20Enum :default "NewEnumerator5") (Amount :type Float%20%28single-precision%29))
  (bind _buffers (Variables|Flow|GetBuffers))
  (bind _value (Utilities|Map|Find _buffers Resource))
  (bind (_current _maximum) (Utilities|Struct|BreakResourceBuffer _value))
  (bind _structout (Utilities|Struct|SetmembersinResourceBuffer _value (Math|Float|Clamp(Float) (+ _current Amount) 0.0 _maximum)))
  (Utilities|Map|Add _buffers Resource _structout))

(fn TakefromBuffer
  (params (Resource :type EResources%20Enum :default "NewEnumerator5") (Amount :type Float%20%28single-precision%29))
  (bind (_current _capacity _maximum) (Flow|GetBuffer Resource))
  (bind _result (Math|Float|NegateFloat (Math|Float|Min(Float) _current Amount))
    (:%20%20
      (Flow|ChangeBuffer Resource _result)
      (return (Math|Float|Min(Float) _current Amount) (/ (Math|Float|Min(Float) _current Amount) _capacity) (/ (Math|Float|Min(Float) _current Amount) _maximum) (/ (Math|Float|Min(Float) _current Amount) Amount)))))

(fn TakeAllfromBuffer
  (params (Resource :type EResources%20Enum :default "NewEnumerator5") (Percentage :type Float%20%28single-precision%29))
  (bind (_current _capacity _maximum) (Flow|GetBuffer Resource))
  (bind _result (Math|Float|NegateFloat (Math|Float|Min(Float) _current (* _capacity Percentage)))
    (:%20%20
      (Flow|ChangeBuffer Resource _result)
      (return (Math|Float|Min(Float) _current (* _capacity Percentage)) (/ (Math|Float|Min(Float) _current (* _capacity Percentage)) _capacity) (/ (Math|Float|Min(Float) _current (* _capacity Percentage)) _maximum)))))

(fn EditBufferInternal
  (params (Resource :type EResources%20Enum :default "NewEnumerator5") (Current :type Float%20%28single-precision%29) (Capacity :type Float%20%28single-precision%29) (Maximum :type Float%20%28single-precision%29))
  (bind (_current _capacity _maximum) (Flow|GetBuffer Resource))
  (Utilities|Map|Add (Variables|Flow|GetBuffers) Resource (Utilities|Struct|MakeResourceBuffer (Math|Float|SelectFloat _current Current (< Current 0.0)) (Math|Float|SelectFloat _capacity Capacity (< Capacity 0.0)) (Math|Float|SelectFloat _maximum Maximum (< Maximum 0.0)) true)))

(fn SendResource
  (params (Send%20To :type BP%20MC%20Base%20Object%20Reference) (Resource :type EResources%20Enum :default "NewEnumerator0") (Amount :type Float%20%28single-precision%29))
  (bind _current (Flow|GetBuffer Resource))
  (bind _accepted (Flow|ReceiveResource Send%20To Resource (Math|Float|Min(Float) _current Amount)))
  (Flow|SetBuffer Resource (- _current _accepted))
  (return _accepted))

(fn ReceiveResource
  (params (Resource :type EResources%20Enum :default "NewEnumerator0") (Amount :type Float%20%28single-precision%29))
  (bind _free (Flow|GetBuffer Resource))
  (Flow|ChangeBuffer Resource (Math|Float|Min(Float) Amount _free))
  (return (Math|Float|Min(Float) Amount _free)))

(fn SignalValue
  (params (Type :type EPassiveSignals%20Enum :default "NewEnumerator2") (Data :type EResources%20Enum :default "NewEnumerator5") (Value :type Float%20%28single-precision%29))
  (Utilities|Map|Add (Variables|Signaling|GetOut%20Signals) (Utilities|Struct|MakeSignalKey Type Data) Value))

(fn DrawReferences
  (for _array_element (Variables|Flow|GetInputs)
    (bind (_result _out) (Rendering|IsValidReference _array_element))
    (if _result
      (Rendering|DrawLine _out self "(R=0.050070,G=1.000000,B=0.000000,A=1.000000)")))
  (for _array_element_2 (Variables|Flow|GetOutputs)
    (bind (_result_2 _out_2) (Rendering|IsValidReference _array_element_2))
    (if _result_2
      (Rendering|DrawLine _out_2 "(R=1.000000,G=0.000000,B=0.015400,A=1.000000)"))))

(fn IsValidReference
  (params (Object :type BP%20MC%20Base%20Object%20Reference))
  (if (Utilities|IsValid Object)
    (return true Object)
    (else
      (return false 0))))

(fn DrawLine
  (params (Destination :type BP%20MC%20Base%20Object%20Reference) (Line%20Color :type Linear%20Color%20Structure))
  (Rendering|Debug|DrawDebugArrow (+ (Transformation|GetWorldLocation (Variables|Default|GetDefaultSceneRoot)) (Variables|Rendering|GetReferencePoint)) (+ (Transformation|GetWorldLocation (Variables|BP_MCBase_C|GetDefaultSceneRoot Destination)) (Variables|BP_MCBase_C|GetReferencePoint Destination)) 5e+02 Line%20Color 0.0 7.0))

(fn Tick
  (params (Delta%20Seconds :type Float%20%28single-precision%29))
  (bind _working (Flow|TestFuse))
  (bind _output_get (Variables|Status|SetActualThrottle (* (Math|Conversions|ToFloat(Boolean) _working) (Variables|Status|GetThrottle) (Math|Conversions|ToFloat(Boolean) (Variables|Status|GetRunning)))))
  (Variables|Status|SetEfficiency (* Delta%20Seconds _output_get)))

(fn PostTick
  (params (DeltaTime :type Float%20%28single-precision%29))
  (if false
    (|WidgetUpdate))
  (Variables|Status|SetTemperature (Math|Float|Max(Float) (- (Variables|Status|GetTemperature) (* DeltaTime (Variables|Status|GetCoolingRate))) 22.0))
  (Signaling|SignalBuffers)
  (Signaling|SignalValue "NewEnumerator0" "NewEnumerator5" (Variables|Status|GetTemperature))
  (Signaling|SignalValue "NewEnumerator5" "NewEnumerator5" (Variables|Status|GetThrottle))
  (Signaling|SignalValue "NewEnumerator7" "NewEnumerator5" (Math|Conversions|ToFloat(Boolean) (Variables|Status|GetRunning)))
  (Signaling|SignalValue "NewEnumerator6" "NewEnumerator5" (Variables|Status|GetActualThrottle))
  (Signaling|SignalValue "NewEnumerator10" "NewEnumerator5" (Variables|Status|GetEfficiency)))

(fn SignalBuffers
  (bind _keys (Utilities|Map|Keys (Variables|Flow|GetBuffers)))
  (for _array_element _keys
    (bind (_current _capacity) (Flow|GetBuffer _array_element))
    (Utilities|Map|Add (Variables|Signaling|GetOut%20Signals) (Utilities|Struct|MakeSignalKey "NewEnumerator4" _array_element) (/ _current _capacity))))

(fn Probe
  (params (Query :type Signal%20Key%20Structure))
  (return (.Value (Utilities|Map|Find (Variables|Signaling|GetOut%20Signals) Query))))

(fn TestFuse
  (bind _fuse (Variables|Status|GetFuse))
  (Utilities|IsValid _fuse
    (:Is%20Valid
      (bind _working (Default|GetFuse _fuse))
      (return _working))
    (:Is%20Not%20Valid
      (return true))))