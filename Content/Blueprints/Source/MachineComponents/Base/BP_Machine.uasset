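; BP_Machine is the central updater for machine components, driving every BP_MCBase actor in the level.
; On BeginPlay, RegisterAll gathers them with GetAllActorsOfClass, buckets them by TickGroup, then builds one Components list ordered Active, Semi Passive, Passive.
; Each frame it runs two passes over that list, Tick on every component and then PostTick, giving a controlled update order.
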(event EventBeginPlay
  (CallFunction|RegisterAll))

(event Collision|EventActorBeginOverlap
  (params (OtherActor :type Actor%20Object%20Reference)))

(event EventTick
  (params (DeltaSeconds :type Float%20%28single-precision%29))
  (bind _components (Variables|Default|GetComponents))
  (for _array_element _components
    (Default|Tick _array_element DeltaSeconds))
  (for _array_element_2 _components
    (Default|PostTick _array_element_2)))

(fn ConstructionScript)

(fn RegisterAll
  (bind _components (Variables|Default|GetComponents))
  (Utilities|FlowControl|Sequence
    (:then_0
      (bind _outactors (Actor|GetAllActorsOfClass "/Game/Blueprints/Source/MachineComponents/Base/BP_MCBase.BP_MCBase_C")) ; idgaf fight me
      (for _array_element _outactors
        (switch Utilities|FlowControl|Switch|SwitchonEComponentTickGroup (Variables|/Game/Blueprints/Source/MachineComponents/Base/BP_MCBase.BP_MCBase_C|GetTick%20Group _array_element)
          (:NewEnumerator0
            (Utilities|Array|Add (LocalVariables|GetActive) _array_element))
          (:NewEnumerator1
            (Utilities|Array|Add (LocalVariables|GetSemi-passive) _array_element))
          (:NewEnumerator2
            (Utilities|Array|Add (LocalVariables|GetPassive) _array_element)))))
    (:then_1
      (for _array_element_2 (LocalVariables|GetActive)
        (Utilities|Array|Add _components _array_element_2)))
    (:then_2
      (for _array_element_3 (LocalVariables|GetSemi-passive)
        (Utilities|Array|Add _components _array_element_3)))
    (:then_3
      (for _array_element_4 (LocalVariables|GetPassive)
        (Utilities|Array|Add _components _array_element_4)))))