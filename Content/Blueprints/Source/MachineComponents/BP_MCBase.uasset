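; Base Blueprint for machine components that exchange resources and signals, with empty Tick and PostTick functions.
; Each component keeps per-resource buffers, and Push and Pull move amounts along its Outputs and Inputs through SendResource and ReceiveResource, which clamps at the buffer's Maximum.
; SignalValue forwards values to the receiver mapped to each signal type in OutSignals.
; Editor tick draws coloured debug arrows for the input and output links.
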(event EventBeginPlay)

(event Collision|EventActorBeginOverlap
  (params (OtherActor :type Actor%20Object%20Reference)))

(event EventTick
  (params (DeltaSeconds :type Float%20%28single-precision%29)))

(event EventEditorTick
  (Rendering|DrawReferences))

(fn ConstructionScript
  (AddComponent|AddChildActorComponent false))

(fn Push
  (params (Resource :type EResources%20Enum :default "NewEnumerator0") (Amount :type Float%20%28single-precision%29))
  (bind _array_element (Utilities|Array|ForEachLoopwithBreak (Variables|Flow|GetOutputs) :!label _label)
    (:LoopBody
      (bind _current (Flow|GetBuffer Resource))
      (if (> (Math|Float|Min(Float) Amount _current) (LocalVariables|GetEmptyMargin))
        (Flow|SendResource _array_element Resource (Math|Float|Min(Float) Amount _current))
        (else
          (goto _label Break))))))

(fn Pull
  (params (Resource :type EResources%20Enum :default "NewEnumerator0") (Amount :type Float%20%28single-precision%29))
  (bind _array_element (Utilities|Array|ForEachLoopwithBreak (Variables|Flow|GetInputs) :!label _label)
    (:LoopBody
      (bind _capacity (Flow|GetBuffer Resource))
      (if (> (Math|Float|Min(Float) Amount _capacity) (LocalVariables|GetEmpty%20Margin))
        (Flow|SendResource _array_element self Resource (Math|Float|Min(Float) Amount _capacity))
        (else
          (goto _label Break))))))

(fn SetBuffer
  (params (Resource :type EResources%20Enum :default "NewEnumerator0") (Amount :type Float%20%28single-precision%29))
  (bind _buffers (Variables|Flow|GetBuffers))
  (bind _structout (Utilities|Struct|SetmembersinFResourceBuffer (.Value (Utilities|Map|Find _buffers Resource)) Amount))
  (Utilities|Map|Add _buffers Resource _structout))

(fn GetBuffer
  (params (Resource :type EResources%20Enum :default "NewEnumerator0"))
  (bind _buffers (Variables|Flow|GetBuffers))
  (bind (_value _returnvalue) (Utilities|Map|Find _buffers Resource))
  (bind (_current _capacity _maximum) (Utilities|Struct|BreakFResourceBuffer _value))
  (if _returnvalue
    (return _current _capacity _maximum (- _capacity _current))
    (else
      (return 0.0 0.0 0.0 0.0))))

(fn SendResource
  (params (Send%20To :type BP%20MC%20Base%20Object%20Reference) (Resource :type EResources%20Enum :default "NewEnumerator0") (Amount :type Float%20%28single-precision%29))
  (bind _current (Flow|GetBuffer Resource))
  (bind _accepted (Flow|ReceiveResource Send%20To Resource (Math|Float|Min(Float) _current Amount)))
  (Flow|SetBuffer Resource (- _current _accepted))
  (return (- Amount _accepted)))

(fn ReceiveResource
  (params (Resource :type EResources%20Enum :default "NewEnumerator0") (Amount :type Float%20%28single-precision%29))
  (bind (_current _capacity _maximum) (Flow|GetBuffer Resource))
  (if (.Has%20Overflowed (|CalculateOverflow Amount _current _maximum)) ; Has overflowed?
    (Flow|SetBuffer Resource _maximum)
    (return (.Free (|CalculateOverflow Amount _current _maximum)))
    (else
      (Flow|SetBuffer Resource (.Total (|CalculateOverflow Amount _current _maximum)))
      (return Amount))))

(fn SignalValue
  (params (Signal%20Type :type ESignals%20Enum :default "NewEnumerator0") (Value :type Float%20%28single-precision%29))
  (bind _out_signals (Variables|Signaling|GetOut%20Signals))
  (bind (_value _returnvalue) (Utilities|Map|Find _out_signals Signal%20Type))
  (if _returnvalue
    (Utilities|IsValid _value
      (:Is%20Valid
        (Default|ReceiveSignal _value Value)))))

(fn DrawReferences
  (for _array_element (Variables|Flow|GetInputs)
    (bind (_result _out) (Rendering|IsValidReference _array_element))
    (if _result
      (Rendering|DrawLine _out self "(R=0.050070,G=1.000000,B=0.000000,A=1.000000)")))
  (for _array_element_2 (Variables|Flow|GetOutputs)
    (bind (_result_2 _out_2) (Rendering|IsValidReference _array_element_2))
    (if _result_2
      (Rendering|DrawLine _out_2 "(R=1.000000,G=0.000000,B=0.015400,A=1.000000)"))))

(fn IsValidReference
  (params (Object :type BP%20MC%20Base%20Object%20Reference))
  (if (Utilities|IsValid Object)
    (return true Object)
    (else
      (return false 0))))

(fn DrawLine
  (params (Destination :type BP%20MC%20Base%20Object%20Reference) (Line%20Color :type Linear%20Color%20Structure))
  (Rendering|Debug|DrawDebugArrow (+ (Transformation|GetWorldLocation (Variables|Default|GetDefaultSceneRoot)) (Variables|Rendering|GetReferencePoint)) (+ (Transformation|GetWorldLocation (Variables|BP_MCBase_C|GetDefaultSceneRoot Destination)) (Variables|BP_MCBase_C|GetReferencePoint Destination)) 5e+02 Line%20Color 0.0 7.0))

(fn Tick
  (params (Delta%20Seconds :type Float%20%28single-precision%29)))

(fn PostTick)