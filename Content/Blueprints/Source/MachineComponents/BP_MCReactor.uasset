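; BP_MCReactor is a reactor machine component that changes resource buffers and generates heat.
; Each Tick changes one buffer by a Radiak rate scaled by efficiency and by 0.7 minus another buffer's fill ratio, turning negative above 70%.
; Tick also adds efficiency-scaled heat to Temperature, without using delta time.
; PostTick drains that second buffer by the vacuum loss rate times delta time.
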(event EventBeginPlay
  (|CallParentFunction) ; This node is disabled and will not be called.\nDrag off pins to build functionality.
)

(event Collision|EventActorBeginOverlap
  (params (OtherActor :type Actor%20Object%20Reference))
  (|CallParentFunction OtherActor) ; This node is disabled and will not be called.\nDrag off pins to build functionality.
)

(event EventTick
  (params (DeltaSeconds :type Float%20%28single-precision%29))
  (|CallParentFunction DeltaSeconds) ; This node is disabled and will not be called.\nDrag off pins to build functionality.
)

(fn ConstructionScript
  (|CallParentFunction))

(fn Tick
  (params (Delta%20Seconds :type Float%20%28single-precision%29))
  (bind _efficiency (Variables|Default|GetEfficiency))
  (|CallParentFunction Delta%20Seconds)
  (bind (_current _capacity _maximum) (CallFunction|GetBuffer "NewEnumerator7"))
  (CallFunction|ChangeBuffer "NewEnumerator8" (* (Variables|Default|GetRadiakPerDirtyCycle) (* (- 0.7 (/ _current _maximum)) _efficiency)))
  (Variables|Default|SetTemperature (+ (* _efficiency (Variables|Default|GetHeatPerUnit)) (Variables|Default|GetTemperature))))

(fn PostTick
  (params (DeltaTime :type Float%20%28single-precision%29))
  (|CallParentFunction DeltaTime)
  (CallFunction|ChangeBuffer "NewEnumerator7" (* DeltaTime (Variables|Default|GetVacuumLossPerCycle) -1.0)))