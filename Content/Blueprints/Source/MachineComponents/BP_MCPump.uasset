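; Machine component pump that moves a resource through its buffers, registering a buffer for its configured resource on BeginPlay.
; Each tick, for every buffered resource, it pulls Throughput scaled by Throttle and power buffer fill, then pushes up to Throughput onward.
; The pulled amount times PowerPerTick adjusts the power buffer.
; A Toggle Power button signal switches Throttle between full and off.
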(event EventBeginPlay
  (Utilities|Map|Add (Variables|Default|GetBuffers) (Variables|Flow|GetResource) (Variables|Flow|GetBuffer)))

(event Collision|EventActorBeginOverlap
  (params (OtherActor :type Actor%20Object%20Reference)))

(event EventTick
  (params (DeltaSeconds :type Float%20%28single-precision%29)))

(event EventButtonPressed
  (params (State :type Boolean) (Signal :type EActiveSignals%20Enum :default "NewEnumerator0"))
  (switch Utilities|FlowControl|Switch|SwitchonEActiveSignals Signal
    (:NewEnumerator1
      (if State
        (Variables|Default|SetThrottle 1.0)
        (else
          (Variables|Default|SetThrottle 0.0))))))

(fn ConstructionScript)

(fn Tick
  (params (Delta%20Seconds :type Float%20%28single-precision%29))
  (|CallParentFunction Delta%20Seconds)
  (bind _keys (Utilities|Map|Keys (Variables|Default|GetBuffers)))
  (for _array_element _keys
    ;[1 1 1] Get power and calculate efficiency
    (bind (_current _capacity) (CallFunction|GetBuffer "NewEnumerator1"))
    (bind _received (CallFunction|Pull _array_element (* (/ _current _capacity) (Variables|Flow|GetThroughput) (Variables|Default|GetThrottle))))
    (CallFunction|ChangeBuffer "NewEnumerator1" (* _received (Variables|Status|GetPowerPerTick)))
    (CallFunction|Push _array_element (Variables|Flow|GetThroughput))))

(fn PostTick
  (|CallParentFunction)
  (Utilities|FlowControl|Sequence))