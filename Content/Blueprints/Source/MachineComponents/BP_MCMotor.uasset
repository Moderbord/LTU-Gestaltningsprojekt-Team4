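; BP_MCMotor is a motor machine component that converts one buffered resource into another, apparently torque, while generating heat.
; Tick draws input by Efficiency, adds output scaled by the draw's capacity percentage and the input buffer's unfilled fraction, then flushes it.
; Temperature rises in proportion to the same draw.
; PostTick adjusts the output buffer by a time-scaled torque falloff, capped at its current amount.
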(event EventBeginPlay)

(event Collision|EventActorBeginOverlap
  (params (OtherActor :type Actor%20Object%20Reference)))

(event EventTick
  (params (DeltaSeconds :type Float%20%28single-precision%29)))

(fn ConstructionScript)

(fn Tick
  (params (Delta%20Seconds :type Float%20%28single-precision%29))
  (|CallParentFunction Delta%20Seconds)
  (bind _percentofcapacity (CallFunction|TakeAllfromBuffer "NewEnumerator3" (Variables|Default|GetEfficiency)))
  (bind (_current _capacity _maximum) (CallFunction|GetBuffer "NewEnumerator3"))
  (CallFunction|ChangeBuffer "NewEnumerator2" (* (- 1.0 (/ _current _maximum)) (Variables|Default|GetTorquePerCycle) _percentofcapacity))
  (Variables|Default|SetTemperature (+ (Variables|Default|GetTemperature) (* (Variables|Default|GetHeatPerCycle) _percentofcapacity)))
  (CallFunction|Flush "NewEnumerator2"))

(fn PostTick
  (params (DeltaTime :type Float%20%28single-precision%29))
  (|CallParentFunction DeltaTime)
  (bind _current (CallFunction|GetBuffer "NewEnumerator2"))
  (bind _result (Math|Float|NegateFloat (Math|Float|Min(Float) _current (* DeltaTime (Variables|Default|GetTorqueFalloffPerCycle))))
    (:%20%20
      (CallFunction|ChangeBuffer "NewEnumerator2" _result))))