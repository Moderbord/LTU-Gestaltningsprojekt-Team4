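; BP_MachineComponent is an actor for a machine part that references other components through Inputs and Outputs arrays.
; On editor tick, it draws debug arrows between each component's reference point: green from valid inputs into itself, red from itself to valid outputs.
; Its construction script adds a child actor component.
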(event EventBeginPlay)

(event Collision|EventActorBeginOverlap
  (params (OtherActor :type Actor%20Object%20Reference)))

(event EventTick
  (params (DeltaSeconds :type Float%20%28single-precision%29)))

(event EventEditorTick
  (CallFunction|DrawReferences))

(fn ConstructionScript
  (AddComponent|AddChildActorComponent false))

(fn DrawReferences
  (for _array_element (Variables|Default|GetInputs)
    (bind (_result _out) (CallFunction|ValidCheck _array_element))
    (if _result
      (CallFunction|DrawLine _out self "(R=0.087762,G=1.000000,B=0.000000,A=1.000000)")))
  (for _array_element_2 (Variables|Default|GetOutputs)
    (bind (_result_2 _out_2) (CallFunction|ValidCheck _array_element_2))
    (if _result_2
      (CallFunction|DrawLine _out_2 "(R=1.000000,G=0.000000,B=0.019289,A=1.000000)"))))

(fn DrawLine
  (params (Destination :type BP%20Machine%20Component%20Object%20Reference) (Line%20Color :type Linear%20Color%20Structure))
  (Rendering|Debug|DrawDebugArrow (+ (Transformation|GetWorldLocation (Variables|Default|GetDefaultSceneRoot)) (Variables|Default|GetReferencePoint)) (+ (Transformation|GetWorldLocation (Variables|BP_MachineComponent_C|GetDefaultSceneRoot Destination)) (Variables|BP_MachineComponent_C|GetReferencePoint Destination)) 5e+02 Line%20Color 0.0 7.0))

(fn ValidCheck
  (params (object :type BP%20Machine%20Component%20Object%20Reference))
  (if (Utilities|IsValid object)
    (return true object)
    (else
      (return false 0))))