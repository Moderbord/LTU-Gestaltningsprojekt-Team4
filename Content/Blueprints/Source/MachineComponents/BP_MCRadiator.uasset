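; BP_MCRadiator is a radiator machine component that draws heat out of its connected inputs and dissipates it.
; Each tick it moves heat from every input into itself, scaled by input temperature and buffer fill, consuming water per heat unit.
; It then sheds heat by draining a second resource buffer in proportion to its temperature.
; Temperature also drives an interpolated emissive glow and toggles heat distortion effects above a threshold.
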(event EventBeginPlay
  (|CallParentFunction))

(event EventTick
  (params (DeltaSeconds :type Float%20%28single-precision%29))
  (|CallParentFunction DeltaSeconds)
  (bind _output_get (Variables|Rendering|SetEmissiveCurrent (Math|Interpolation|FInterpTo (Variables|Rendering|GetEmissiveCurrent) (* (- (Variables|Default|GetTemperature) 22.0) (Variables|Rendering|GetEmissiveMult)) DeltaSeconds (Variables|Rendering|GetEmissiveDelta))))
  (Rendering|Material|SetScalarParameterValue (Variables|Default|GetMaterial) "Emissive" _output_get :!class /Script/Engine.MaterialInstanceDynamic))

(fn ConstructionScript
  (|CallParentFunction))

(fn Tick
  (params (Delta%20Seconds :type Float%20%28single-precision%29))
  (bind _inputs (Variables|Default|GetInputs))
  (bind _efficiency (Variables|Default|GetEfficiency))
  (bind _returnvalue (* Delta%20Seconds _efficiency))
  (|CallParentFunction Delta%20Seconds)
  (bind (_current _capacity) (CallFunction|GetBuffer "NewEnumerator0"))
  (for _array_element _inputs
    (Variables|/Game/Blueprints/Source/MachineComponents/Base/BP_MCBase.BP_MCBase_C|SetTemperature _array_element (- (Variables|/Game/Blueprints/Source/MachineComponents/Base/BP_MCBase.BP_MCBase_C|GetTemperature _array_element) (* (/ (Variables|/Game/Blueprints/Source/MachineComponents/Base/BP_MCBase.BP_MCBase_C|GetTemperature _array_element) (Variables|Default|GetTargetTemp)) (/ (Variables|Default|GetHeatTransportPerCycle) (Math|Conversions|ToFloat(Integer) (Utilities|Array|Length _inputs))) (/ _current _capacity) _returnvalue)))
    (Variables|Default|SetTemperature (+ (* (/ (Variables|/Game/Blueprints/Source/MachineComponents/Base/BP_MCBase.BP_MCBase_C|GetTemperature _array_element) (Variables|Default|GetTargetTemp)) (/ (Variables|Default|GetHeatTransportPerCycle) (Math|Conversions|ToFloat(Integer) (Utilities|Array|Length _inputs))) (/ _current _capacity) _returnvalue) (Variables|Default|GetTemperature)))
    (CallFunction|ChangeBuffer "NewEnumerator0" (* (* (/ (Variables|/Game/Blueprints/Source/MachineComponents/Base/BP_MCBase.BP_MCBase_C|GetTemperature _array_element) (Variables|Default|GetTargetTemp)) (/ (Variables|Default|GetHeatTransportPerCycle) (Math|Conversions|ToFloat(Integer) (Utilities|Array|Length _inputs))) (/ _current _capacity) _returnvalue) (Variables|Default|GetWaterPerHeatUnit) -1.0)))
  (bind _percentofcapacity (CallFunction|TakeAllfromBuffer "NewEnumerator1" (* _returnvalue (/ (Variables|Default|GetTemperature) (Variables|Default|GetTargetTemp)))))
  (bind _output_get (Variables|Default|SetTemperature (- (Variables|Default|GetTemperature) (* _percentofcapacity (Variables|Default|GetHeatTransportPerCycle)))))
  (Components|Activation|SetActive (Variables|Default|GetDistortions) (> _output_get (Variables|Default|GetDistortionTreshold)) false))