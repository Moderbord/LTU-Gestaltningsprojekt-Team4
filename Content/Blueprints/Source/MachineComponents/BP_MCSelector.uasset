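; BP_MCSelector is a machine component that acts as a switch, routing resource buffer access to one of several inputs.
; A Change State discrete signal sets the selected input index, clamped to the bounds of the Inputs array.
; GetBuffer and SetBuffer forward each call to the selected input when it is valid, so the selector passes that input's buffer values through.
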(event EventOnDiscreteChanged
  (params (New%20Value :type Integer) (Signal :type EActiveSignals%20Enum :default "NewEnumerator0"))
  (switch Utilities|FlowControl|Switch|SwitchonEActiveSignals Signal
    (:NewEnumerator3
      (Variables|Default|SetSelectedInput (Math|Integer|Clamp(Integer) New%20Value 0 (- (Utilities|Array|Length (Variables|Default|GetInputs)) 1))))))

(fn ConstructionScript
  (|CallParentFunction))

(fn GetBuffer
  (params (Resource :type EResources%20Enum :default "NewEnumerator5"))
  (bind _inputs (Variables|Default|GetInputs))
  (bind _selectedinput (Variables|Default|GetSelectedInput))
  (bind _output (Utilities|Array|Get(acopy) _inputs _selectedinput))
  (Utilities|IsValid _output
    (:Is%20Valid
      (bind (_current _capacity _maximum _free) (CallFunction|GetBuffer _output Resource))
      (return _current _capacity _maximum _free))))

(fn SetBuffer
  (params (Resource :type EResources%20Enum :default "NewEnumerator5") (Amount :type Float%20%28single-precision%29))
  (bind _inputs (Variables|Default|GetInputs))
  (bind _selectedinput (Variables|Default|GetSelectedInput))
  (bind _output (Utilities|Array|Get(acopy) _inputs _selectedinput))
  (Utilities|IsValid _output
    (:Is%20Valid
      (CallFunction|SetBuffer _output Resource Amount))))