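; BP_LeverSnap is a lever that snaps between notches in response to axis input.
; Positive Z steps one notch down and any other Z value one notch up, within the notch limits.
; Each step shifts the stored angle, then sets the physics constraint's pitch target one further increment beyond it.
; The AnimationPlaying guard is set and cleared within the same step, with debug prints for direction.
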(event EventAxisValuesEvent
  (params (Values :type Vector :default "0, 0, 0"))
  (bind _physicsconstraint (Variables|Default|GetPhysicsConstraint))
  (if (not (Variables|Default|GetAnimationPlaying))
    (if (> (.z Values) 0.0)
      (if (not (== (Variables|Default|GetCurrentNotch) (Variables|Default|GetNotchMin)))
        (Development|PrintString "spin left")
        (Variables|Default|SetAnimationPlaying true)
        (Variables|Default|SetCurrentAngle (- (Variables|Default|GetCurrentAngle) (Variables|Default|GetAngleDifference)))
        (Variables|Default|SetAnimationPlaying false)
        (Variables|Default|SetCurrentNotch (- (Variables|Default|GetCurrentNotch) 1))
        (Class|PhysicsConstraintComponent|SetAngularOrientationTarget _physicsconstraint (Math|Rotator|MakeRotator 0.0 (- (Variables|Default|GetCurrentAngle) (Variables|Default|GetAngleDifference)) 0.0)))
      (elif (not (== (Variables|Default|GetCurrentNotch) (Variables|Default|GetNotchMax)))
        (Development|PrintString "spin right")
        (Variables|Default|SetAnimationPlaying true)
        (Variables|Default|SetCurrentAngle (+ (Variables|Default|GetCurrentAngle) (Variables|Default|GetAngleDifference)))
        (Variables|Default|SetAnimationPlaying false)
        (Variables|Default|SetCurrentNotch (+ (Variables|Default|GetCurrentNotch) 1))
        (Class|PhysicsConstraintComponent|SetAngularOrientationTarget _physicsconstraint (Math|Rotator|MakeRotator 0.0 (+ (Variables|Default|GetCurrentAngle) (Variables|Default|GetAngleDifference)) 0.0))))))

(fn ConstructionScript)